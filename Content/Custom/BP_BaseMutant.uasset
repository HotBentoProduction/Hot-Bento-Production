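; Base mutant enemy for the turn-based RPG battle, whose AI turn moves it one spot on a four-wide grid, then ends the turn.
; MoveFromPosition randomly picks an orthogonal neighbour from the game instance's EnemySpotMap, discarding invalid or blocked spots and retrying.
; It can enter spots held by an unbroken pan part, breaking it; TryBreakingPan currently always succeeds.
; An attack sequence against the player exists but is unconnected.
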(event EventBeginPlay
  (|CallParentFunction))

(event Collision|EventActorBeginOverlap
  (params (OtherActor :type Actor%20Object%20Reference))
  (|CallParentFunction OtherActor) ; This node is disabled and will not be called.\nDrag off pins to build functionality.
)

(event EventTick
  (params (DeltaSeconds :type Float%20%28single-precision%29))
  (|CallParentFunction DeltaSeconds) ; This node is disabled and will not be called.\nDrag off pins to build functionality.
)

(event EventPerformActionbyAI
  (CallFunction|MovefromPosition)
  (Utilities|FlowControl|Delay 0.5)
  (Default|EndCharacterTurn (Variables|Default|GetBattleManagerReferences)))

(fn ConstructionScript
  (|CallParentFunction))

(fn MovefromPosition
  (bind _possibleindexes (CallFunction|CreatePointArray))
  (bind _output_get (LocalVariables|SetPossibleIndexMoves _possibleindexes))
  (bind _selectedspot (CallFunction|GetRandomPoint _output_get :!label _label))
  (if (== _selectedspot -99)
    (Development|PrintString "No moves available")
    (return)
    (else
      (LocalVariables|SetSelectedSpotToMove _selectedspot)
      (bind _asgi_rpg (Utilities|Casting|CastToGI_RPG (Game|GetGameInstance)))
      (if (.ReturnValue (Utilities|Map|Find (Variables|/Game/Custom/GI_RPG.GI_RPG_C|GetEnemySpotMap _asgi_rpg) (LocalVariables|GetSelectedSpotToMove)))
        (if (Variables|/Game/Custom/BP_EnemySpot.BP_EnemySpot_C|GetisOccupied (.Value (Utilities|Map|Find (Variables|/Game/Custom/GI_RPG.GI_RPG_C|GetEnemySpotMap _asgi_rpg) (LocalVariables|GetSelectedSpotToMove))))
          (if (and (Variables|/Game/Custom/BP_EnemySpot.BP_EnemySpot_C|GetisOccupiedByPan (.Value (Utilities|Map|Find (Variables|/Game/Custom/GI_RPG.GI_RPG_C|GetEnemySpotMap _asgi_rpg) (LocalVariables|GetSelectedSpotToMove)))) (not (Variables|/Game/Custom/BP_EnemySpot.BP_EnemySpot_C|GetHasPanPartBeenBroken (.Value (Utilities|Map|Find (Variables|/Game/Custom/GI_RPG.GI_RPG_C|GetEnemySpotMap _asgi_rpg) (LocalVariables|GetSelectedSpotToMove))))))
            (bind _success (CallFunction|TryBreakingPan (.Value (Utilities|Map|Find (Variables|/Game/Custom/GI_RPG.GI_RPG_C|GetEnemySpotMap _asgi_rpg) (LocalVariables|GetSelectedSpotToMove)))))
            (if _success
              (Transformation|SetActorLocation (Math|Vector|MakeVector (.X (Math|Vector|BreakVector (.location (Transformation|GetActorTransform (.Value (Utilities|Map|Find (Variables|/Game/Custom/GI_RPG.GI_RPG_C|GetEnemySpotMap _asgi_rpg) (LocalVariables|GetSelectedSpotToMove))))))) (.Y (Math|Vector|BreakVector (.location (Transformation|GetActorTransform (.Value (Utilities|Map|Find (Variables|/Game/Custom/GI_RPG.GI_RPG_C|GetEnemySpotMap _asgi_rpg) (LocalVariables|GetSelectedSpotToMove))))))) (.z (Transformation|GetActorLocation))) false false)
              (Variables|/Game/Custom/BP_EnemySpot.BP_EnemySpot_C|SetisOccupied (.Value (Utilities|Map|Find (Variables|/Game/Custom/GI_RPG.GI_RPG_C|GetEnemySpotMap _asgi_rpg) (LocalVariables|GetSelectedSpotToMove))) true)
              (Default|StartShowing (.Value (Utilities|Map|Find (Variables|/Game/Custom/GI_RPG.GI_RPG_C|GetEnemySpotMap _asgi_rpg) (LocalVariables|GetSelectedSpotToMove))))
              (Variables|/Game/Custom/BP_EnemySpot.BP_EnemySpot_C|SetisOccupied (.Value (Utilities|Map|Find (Variables|/Game/Custom/GI_RPG.GI_RPG_C|GetEnemySpotMap _asgi_rpg) (Variables|Default|GetCurrentIndex))) false)
              (Default|StopShowing (.Value (Utilities|Map|Find (Variables|/Game/Custom/GI_RPG.GI_RPG_C|GetEnemySpotMap _asgi_rpg) (Variables|Default|GetCurrentIndex))))
              (Variables|Default|SetCurrentIndex (LocalVariables|GetSelectedSpotToMove))
              (Variables|/Game/Custom/BP_EnemySpot.BP_EnemySpot_C|SetisOccupiedByPan (.Value (Utilities|Map|Find (Variables|/Game/Custom/GI_RPG.GI_RPG_C|GetEnemySpotMap _asgi_rpg) (LocalVariables|GetSelectedSpotToMove))) false)
              (Default|PanPartBroken (.Value (Utilities|Map|Find (Variables|/Game/Custom/GI_RPG.GI_RPG_C|GetEnemySpotMap _asgi_rpg) (LocalVariables|GetSelectedSpotToMove))))
              (else
                (Utilities|Array|RemoveItem (LocalVariables|GetPossibleIndexMoves) (LocalVariables|GetSelectedSpotToMove) :!label _label_2)
                (goto _label)))
            (else
              (goto _label_2)))
          (else
            (Transformation|SetActorLocation (Math|Vector|MakeVector (.X (Math|Vector|BreakVector (.location (Transformation|GetActorTransform (.Value (Utilities|Map|Find (Variables|/Game/Custom/GI_RPG.GI_RPG_C|GetEnemySpotMap _asgi_rpg) (LocalVariables|GetSelectedSpotToMove))))))) (.Y (Math|Vector|BreakVector (.location (Transformation|GetActorTransform (.Value (Utilities|Map|Find (Variables|/Game/Custom/GI_RPG.GI_RPG_C|GetEnemySpotMap _asgi_rpg) (LocalVariables|GetSelectedSpotToMove))))))) (.z (Transformation|GetActorLocation))) false false)
            (Variables|/Game/Custom/BP_EnemySpot.BP_EnemySpot_C|SetisOccupied (.Value (Utilities|Map|Find (Variables|/Game/Custom/GI_RPG.GI_RPG_C|GetEnemySpotMap _asgi_rpg) (LocalVariables|GetSelectedSpotToMove))) true)
            (Variables|/Game/Custom/BP_EnemySpot.BP_EnemySpot_C|SetisOccupied (.Value (Utilities|Map|Find (Variables|/Game/Custom/GI_RPG.GI_RPG_C|GetEnemySpotMap _asgi_rpg) (Variables|Default|GetCurrentIndex))) false)
            (Default|StopShowing (.Value (Utilities|Map|Find (Variables|/Game/Custom/GI_RPG.GI_RPG_C|GetEnemySpotMap _asgi_rpg) (LocalVariables|GetSelectedSpotToMove))))
            (Default|StopShowing (.Value (Utilities|Map|Find (Variables|/Game/Custom/GI_RPG.GI_RPG_C|GetEnemySpotMap _asgi_rpg) (Variables|Default|GetCurrentIndex))))
            (Variables|Default|SetCurrentIndex (LocalVariables|GetSelectedSpotToMove))))
        (else
          (goto _label_2))))))

(fn GetRandomPoint
  (params (Array :type Array%20of%20Integers))
  (if (== (Utilities|Array|Length Array) 0)
    (return -99)
    (else
      (bind _array_element (Utilities|Array|ForEachLoopwithBreak Array :!label _label)
        (:LoopBody
          (if (Math|Random|RandomBool)
            (return _array_element)))
        (:Completed
          (if true
            (goto _label)))))))

(fn CreatePointArray
  (bind _currentindex (Variables|Default|GetCurrentIndex))
  (bind _currentindex_2 (Variables|Default|GetCurrentIndex))
  (bind _currentindex_3 (Variables|Default|GetCurrentIndex))
  (bind _returnvalue (+ _currentindex_3 1))
  (bind _returnvalue_2 (- _currentindex 1))
  (bind _output_get (LocalVariables|SetCurrentArray (Utilities|Array|MakeArray (+ _currentindex_2 4) (+ _currentindex_2 -4))))
  (if (Math|Boolean|ANDBoolean (!= _returnvalue 5) (!= (+ _currentindex_3 1) 9) (!= (+ _currentindex_3 1) 13))
    (Utilities|Array|Add _output_get _returnvalue))
  (if (Math|Boolean|ANDBoolean (!= _returnvalue_2 4) (!= (- _currentindex 1) 8) (!= (- _currentindex 1) 12))
    (Utilities|Array|Add (LocalVariables|GetCurrentArray) _returnvalue_2)
    (Utilities|Array|Shuffle (LocalVariables|GetCurrentArray)))
  (return (LocalVariables|GetCurrentArray)))

(fn TryBreakingPan
  (params (PointReference :type BP%20Enemy%20Spot%20Object%20Reference))
  (if (Math|Random|RandomBool)
    _
    (else
      _))
  (return true))