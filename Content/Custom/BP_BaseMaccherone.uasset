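; Turn-based battle enemy "BaseMaccherone", a child Blueprint tuned by its DT_Enemies row, that moves across a spot grid and attacks the player.
; Movement steps back five indices per step through GI_RPG's EnemySpotMap, carrying occupancy and soiled state, with a simulation pass checking for blocked moves.
; Cook time counts down toward death and regenerates, eventually lowering the sauce bar and clearing soiling.
; Attacks also soil the board; pan breaking is a coin flip.
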(event EventBeginPlay
  (|CallParentFunction)
  (bind _returnvalue (Utilities|GetDataTableRow "/Game/Custom/DataTables/DT_Enemies.DT_Enemies" "BaseMaccherone")
    (:then
      (Variables|Default|SetcookTimeRegen (.CookingTimeRegen (Utilities|Struct|BreakS_Enemy _returnvalue)))
      (Variables|Default|SetcookTime (.CookingTime (Utilities|Struct|BreakS_Enemy _returnvalue))))))

(event Collision|EventActorBeginOverlap
  (params (OtherActor :type Actor%20Object%20Reference))
  (|CallParentFunction OtherActor) ; This node is disabled and will not be called.\nDrag off pins to build functionality.
)

(event EventTick
  (params (DeltaSeconds :type Float%20%28single-precision%29))
  (|CallParentFunction DeltaSeconds) ; This node is disabled and will not be called.\nDrag off pins to build functionality.
)

(event EventUpdateCookTime
  (Rendering|Components|TextRender|SetText (Variables|/Game/Custom/Widgets/BattleWidgets/Widget_BattleCharacterSlot.Widget_BattleCharacterSlot_C|GetTextBlock_MP (Variables|/Game/Custom/Components/AC_CharacterBattleStats.AC_CharacterBattleStats_C|GetCharacterBattleSlotReference (Variables|Default|GetAC_CharacterBattleStats))) (Utilities|Text|ToText(String) (Utilities|String|Append "CookTime:" (Utilities|String|ToString(Integer) (Variables|Default|GetcookTime))))))

(event EventOnSoiled
  (Variables|Default|SetisSoiled true)
  (bind _asgi_rpg (Utilities|Casting|CastToGI_RPG (Game|GetGameInstance)))
  (Variables|/Game/Custom/BP_EnemySpot.BP_EnemySpot_C|SetisEnemySoiled (.Value (Utilities|Map|Find (Variables|/Game/Custom/GI_RPG.GI_RPG_C|GetEnemySpotMap _asgi_rpg) (Variables|Default|GetcurrentIndex))) true))

(fn ConstructionScript
  (|CallParentFunction))

(fn TryBreakingPan
  (params (PointReference :type BP%20Enemy%20Spot%20Object%20Reference))
  (|CallParentFunction PointReference)
  (if (Math|Random|RandomBool)
    (return true)
    (else
      (return false))))

(fn RecoverSauceBar
  (bind _ac_characterbattlestats (Variables|Default|GetAC_CharacterBattleStats))
  (bind _returnvalue (Utilities|GetDataTableRow "/Game/Custom/DataTables/DT_Enemies.DT_Enemies" "BaseMaccherone")
    (:then
      (Variables|/Game/Custom/Components/AC_CharacterBattleStats.AC_CharacterBattleStats_C|SetCurrentHP _ac_characterbattlestats (Math|Float|Clamp(Float) (- (Variables|/Game/Custom/Components/AC_CharacterBattleStats.AC_CharacterBattleStats_C|GetCurrentHP _ac_characterbattlestats) (.SauceBarRegen (Utilities|Struct|BreakS_Enemy _returnvalue))) 0.0 (.Value (Utilities|Map|Find (Variables|/Game/Custom/Components/AC_CharacterBattleStats.AC_CharacterBattleStats_C|GetCharacterStats (Variables|Default|GetAC_CharacterBattleStats)) "NewEnumerator1"))))
      (Default|RefreshHP _ac_characterbattlestats))))

(fn StartRegeneration
  (bind _returnvalue (Utilities|GetDataTableRow "/Game/Custom/DataTables/DT_Enemies.DT_Enemies" "BaseMaccherone")
    (:then
      (Variables|Default|SetcookTime (Math|Integer|Clamp(Integer) (+ (Variables|Default|GetcookTime) (Variables|Default|GetcookTimeRegen)) 0 (.CookingTime (Utilities|Struct|BreakS_Enemy _returnvalue))))
      (CallFunction|UpdateCookTime)
      (if (Variables|Default|GetStartRegen)
        (if (== (Variables|Default|GetcookTime) (.CookingTime (Utilities|Struct|BreakS_Enemy _returnvalue)))
          (CallFunction|RecoverSauceBar)
          (if (Variables|Default|GetisSoiled)
            (Variables|Default|SetisSoiled false)
            (bind _asgi_rpg (Utilities|Casting|CastToGI_RPG (Game|GetGameInstance)))
            (Variables|/Game/Custom/BP_EnemySpot.BP_EnemySpot_C|SetisEnemySoiled (.Value (Utilities|Map|Find (Variables|/Game/Custom/GI_RPG.GI_RPG_C|GetEnemySpotMap _asgi_rpg) (Variables|Default|GetcurrentIndex))) false)))
        (elif (Variables|Default|GetwasHitLastTurn)
          (Variables|Default|SetwasHitLastTurn false)
          (else
            (Variables|Default|SetStartRegen true)))))))

(fn IsGettingCookedFunction
  (bind _output_get (Variables|Default|SetcookTime (- (Variables|Default|GetcookTime) 1)))
  (Development|PrintString (Utilities|String|Append "Turn before death for" (Utilities|GetDisplayName self) ": " (Utilities|String|ToString(Integer) _output_get)))
  (CallFunction|UpdateCookTime)
  (if (<= _output_get 0)
    (return true)
    (else
      (return false))))

(fn MoveFunction
  (Variables|MoveFunction|SetFirstWasASuccess false)
  (Variables|MoveFunction|SetsecondWasASuccess false)
  (bind _returnvalue (Utilities|GetDataTableRow "/Game/Custom/DataTables/DT_Enemies.DT_Enemies" "BaseMaccherone")
    (:then
      (for _index (range 1 (- (.MovementValue (Utilities|Struct|BreakS_Enemy _returnvalue)) (Math|Random|RandomIntegerinRange 0 1)))
        (CallFunction|CreatePointArray)
        (Variables|MoveFunction|SetSelectedSpotToMove (Utilities|Array|Get(acopy) (Variables|MoveFunction|GetMovePointArray)))
        (bind _asgi_rpg (Utilities|Casting|CastToGI_RPG (Game|GetGameInstance)))
        (if (.ReturnValue (Utilities|Map|Find (Variables|/Game/Custom/GI_RPG.GI_RPG_C|GetEnemySpotMap _asgi_rpg) (Variables|MoveFunction|GetSelectedSpotToMove)))
          (if (not (and (Variables|/Game/Custom/BP_EnemySpot.BP_EnemySpot_C|GetisOccupiedByPan (.Value (Utilities|Map|Find (Variables|/Game/Custom/GI_RPG.GI_RPG_C|GetEnemySpotMap _asgi_rpg) (Variables|MoveFunction|GetSelectedSpotToMove)))) (not (Variables|/Game/Custom/BP_EnemySpot.BP_EnemySpot_C|GetHasPanPartBeenBroken (.Value (Utilities|Map|Find (Variables|/Game/Custom/GI_RPG.GI_RPG_C|GetEnemySpotMap _asgi_rpg) (Variables|MoveFunction|GetSelectedSpotToMove)))))))
            (if (not (Variables|/Game/Custom/BP_EnemySpot.BP_EnemySpot_C|GetisOccupied (.Value (Utilities|Map|Find (Variables|/Game/Custom/GI_RPG.GI_RPG_C|GetEnemySpotMap _asgi_rpg) (Variables|MoveFunction|GetSelectedSpotToMove)))))
              (Transformation|SetActorLocation (Math|Vector|MakeVector (.X (Math|Vector|BreakVector (.location (Transformation|GetActorTransform (.Value (Utilities|Map|Find (Variables|/Game/Custom/GI_RPG.GI_RPG_C|GetEnemySpotMap _asgi_rpg) (Variables|MoveFunction|GetSelectedSpotToMove))))))) (.Y (Math|Vector|BreakVector (.location (Transformation|GetActorTransform (.Value (Utilities|Map|Find (Variables|/Game/Custom/GI_RPG.GI_RPG_C|GetEnemySpotMap _asgi_rpg) (Variables|MoveFunction|GetSelectedSpotToMove))))))) (.z (Transformation|GetActorLocation))) false false)
              (Variables|/Game/Custom/BP_EnemySpot.BP_EnemySpot_C|SetisOccupied (.Value (Utilities|Map|Find (Variables|/Game/Custom/GI_RPG.GI_RPG_C|GetEnemySpotMap _asgi_rpg) (Variables|MoveFunction|GetSelectedSpotToMove))) true)
              (Variables|/Game/Custom/BP_EnemySpot.BP_EnemySpot_C|SetisOccupied (.Value (Utilities|Map|Find (Variables|/Game/Custom/GI_RPG.GI_RPG_C|GetEnemySpotMap _asgi_rpg) (Variables|Default|GetCurrentIndex))) false)
              (Default|StopShowing (.Value (Utilities|Map|Find (Variables|/Game/Custom/GI_RPG.GI_RPG_C|GetEnemySpotMap _asgi_rpg) (Variables|Default|GetCurrentIndex))))
              (Variables|/Game/Custom/BP_EnemySpot.BP_EnemySpot_C|SetenemyReference (.Value (Utilities|Map|Find (Variables|/Game/Custom/GI_RPG.GI_RPG_C|GetEnemySpotMap _asgi_rpg) (Variables|Default|GetCurrentIndex))) 0)
              (Variables|/Game/Custom/BP_EnemySpot.BP_EnemySpot_C|SetisEnemySoiled (.Value (Utilities|Map|Find (Variables|/Game/Custom/GI_RPG.GI_RPG_C|GetEnemySpotMap _asgi_rpg) (Variables|Default|GetCurrentIndex))) false)
              (Variables|/Game/Custom/BP_EnemySpot.BP_EnemySpot_C|SetenemyReference (.Value (Utilities|Map|Find (Variables|/Game/Custom/GI_RPG.GI_RPG_C|GetEnemySpotMap _asgi_rpg) (Variables|MoveFunction|GetSelectedSpotToMove))) self)
              (Default|StopShowing (.Value (Utilities|Map|Find (Variables|/Game/Custom/GI_RPG.GI_RPG_C|GetEnemySpotMap _asgi_rpg) (Variables|MoveFunction|GetSelectedSpotToMove))))
              (Variables|/Game/Custom/BP_EnemySpot.BP_EnemySpot_C|SetisEnemySoiled (.Value (Utilities|Map|Find (Variables|/Game/Custom/GI_RPG.GI_RPG_C|GetEnemySpotMap _asgi_rpg) (Variables|MoveFunction|GetSelectedSpotToMove))) (Variables|Default|GetisSoiled))
              (Variables|Default|SetCurrentIndex (Variables|MoveFunction|GetSelectedSpotToMove))
              (if (== _index 1)
                (Variables|MoveFunction|SetFirstWasASuccess true)
                (else
                  (Variables|MoveFunction|SetsecondWasASuccess true)))))))
      (if (or (Variables|MoveFunction|GetFirstWasASuccess) (Variables|MoveFunction|GetsecondWasASuccess))
        _))))

(fn CreatePointArray
  (Variables|MoveFunction|SetMovePointArray (Utilities|Array|MakeArray (+ (Variables|Default|GetCurrentIndex) -5))))

(fn AttackPlayerFunction
  (bind _ac_characterbattlestats (Variables|Default|GetAC_CharacterBattleStats))
  (bind _battlemanagerreference (Variables|/Game/Custom/Components/AC_CharacterBattleStats.AC_CharacterBattleStats_C|GetBattleManagerReference _ac_characterbattlestats))
  (bind _playercharacter (Variables|/Game/Custom/Components/AC_BattleManager.AC_BattleManager_C|GetPlayerCharacter _battlemanagerreference))
  (LocalVariables|SetAttackValue (.Value (Utilities|Map|Find (Variables|/Game/Custom/Components/AC_CharacterBattleStats.AC_CharacterBattleStats_C|GetCharacterStats _ac_characterbattlestats) "NewEnumerator3")))
  (if (not (>= (Variables|/Game/Custom/Components/AC_CharacterBattleStats.AC_CharacterBattleStats_C|GetCurrentHP (Variables|/Game/Custom/BP_BaseRPGCharacter.BP_BaseRPGCharacter_C|GetAC_CharacterBattleStats _playercharacter)) 1e+02))
    (bind _returnvalue (Utilities|GetDataTableRow "/Game/Custom/DataTables/DT_Enemies.DT_Enemies" "BaseMaccherone")
      (:then
        (Default|ReceiveDamage (Variables|/Game/Custom/BP_BaseRPGCharacter.BP_BaseRPGCharacter_C|GetAC_CharacterBattleStats _playercharacter) (LocalVariables|GetAttackValue) 0.0 0.0 "NewEnumerator17")
        (Default|BoardSoiledState _battlemanagerreference false (LocalVariables|GetAttackValue))))))

(fn SelectActionfortheTurn
  (|CallParentFunction))

(fn SimulateMove
  (CallFunction|CreatePointArray)
  (Variables|MoveFunction|SetFirstWasASuccess false)
  (Variables|MoveFunction|SetsecondWasASuccess false)
  (bind _returnvalue (Utilities|GetDataTableRow "/Game/Custom/DataTables/DT_Enemies.DT_Enemies" "BaseMaccherone")
    (:then
      (for _index (range 1 (.MovementValue (Utilities|Struct|BreakS_Enemy _returnvalue)))
        (Variables|MoveFunction|SetSelectedSpotToMove (Utilities|Array|Get(acopy) (Variables|MoveFunction|GetMovePointArray)))
        (bind _asgi_rpg (Utilities|Casting|CastToGI_RPG (Game|GetGameInstance)))
        (if (.ReturnValue (Utilities|Map|Find (Variables|/Game/Custom/GI_RPG.GI_RPG_C|GetEnemySpotMap _asgi_rpg) (Variables|MoveFunction|GetSelectedSpotToMove)))
          (if (not (or (and (Variables|/Game/Custom/BP_EnemySpot.BP_EnemySpot_C|GetisOccupiedByPan (.Value (Utilities|Map|Find (Variables|/Game/Custom/GI_RPG.GI_RPG_C|GetEnemySpotMap _asgi_rpg) (Variables|MoveFunction|GetSelectedSpotToMove)))) (not (Variables|/Game/Custom/BP_EnemySpot.BP_EnemySpot_C|GetHasPanPartBeenBroken (.Value (Utilities|Map|Find (Variables|/Game/Custom/GI_RPG.GI_RPG_C|GetEnemySpotMap _asgi_rpg) (Variables|MoveFunction|GetSelectedSpotToMove)))))) (Variables|/Game/Custom/BP_EnemySpot.BP_EnemySpot_C|GetisOccupied (.Value (Utilities|Map|Find (Variables|/Game/Custom/GI_RPG.GI_RPG_C|GetEnemySpotMap _asgi_rpg) (Variables|MoveFunction|GetSelectedSpotToMove))))))
            (if (== _index 1)
              (Variables|MoveFunction|SetFirstWasASuccess true)
              (else
                (Variables|MoveFunction|SetsecondWasASuccess true))))))
      (if (not (or (Variables|MoveFunction|GetFirstWasASuccess) (Variables|MoveFunction|GetsecondWasASuccess)))
        (Development|PrintString (Utilities|String|Append (Utilities|GetDisplayName self) " " "Cannot move"))
        (CallFunction|GotoRightTurnArray)))))