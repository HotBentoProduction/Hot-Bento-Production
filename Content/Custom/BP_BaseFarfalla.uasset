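; BP_BaseFarfalla is the Farfalla enemy in a cooking-themed turn-based battle, configured from its DT_Enemies row.
; It steps along the EnemySpotMap grid and can fly over a blocked spot unless soiled, with SimulateMove dry-running the same rules.
; It queues random-ingredient attacks through the battle manager, counts down CookTime while cooked, and regenerates it to recover the sauce bar and clear soiling.
; The EventGraph's sleep and turn logic is disconnected.
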(event EventBeginPlay
  (|CallParentFunction)
  (bind _returnvalue (Utilities|GetDataTableRow "/Game/Custom/DataTables/DT_Enemies.DT_Enemies" "BaseFarfalla")
    (:then
      (Variables|Default|SetcookTimeRegen (.CookingTimeRegen (Utilities|Struct|BreakS_Enemy _returnvalue)))
      (Variables|Default|SetcookTime (.CookingTime (Utilities|Struct|BreakS_Enemy _returnvalue)))
      (Variables|Default|SetWhatEnemyAmI (.EnemyHardcodedName (Utilities|Struct|BreakS_Enemy _returnvalue))))))

(event Collision|EventActorBeginOverlap
  (params (OtherActor :type Actor%20Object%20Reference))
  (|CallParentFunction OtherActor) ; This node is disabled and will not be called.\nDrag off pins to build functionality.
)

(event EventTick
  (params (DeltaSeconds :type Float%20%28single-precision%29))
  (|CallParentFunction DeltaSeconds) ; This node is disabled and will not be called.\nDrag off pins to build functionality.
)

(event EventUpdateSleepTime
  (Rendering|Components|TextRender|SetText (Variables|/Game/Custom/Widgets/BattleWidgets/Widget_BattleCharacterSlot.Widget_BattleCharacterSlot_C|GetTextBlock_Sleep (Variables|/Game/Custom/Components/AC_CharacterBattleStats.AC_CharacterBattleStats_C|GetCharacterBattleSlotReference (Variables|Default|GetAC_CharacterBattleStats))) (Utilities|Text|ToText(String) (Utilities|String|Append "Sleep:" (Utilities|String|ToString(Integer) (Variables|Default|GetsleepCounter))))))

(event EventUpdateCookTime
  (Rendering|Components|TextRender|SetText (Variables|/Game/Custom/Widgets/BattleWidgets/Widget_BattleCharacterSlot.Widget_BattleCharacterSlot_C|GetTextBlock_MP (Variables|/Game/Custom/Components/AC_CharacterBattleStats.AC_CharacterBattleStats_C|GetCharacterBattleSlotReference (Variables|Default|GetAC_CharacterBattleStats))) (Utilities|Text|ToText(String) (Utilities|String|Append "CookTime:" (Utilities|String|ToString(Integer) (Variables|Default|GetcookTime))))))

(event EventOnSoiled
  (Variables|Default|SetisSoiled true)
  (bind _asgi_rpg (Utilities|Casting|CastToGI_RPG (Game|GetGameInstance)))
  (Variables|/Game/Custom/BP_EnemySpot.BP_EnemySpot_C|SetisEnemySoiled (.Value (Utilities|Map|Find (Variables|/Game/Custom/GI_RPG.GI_RPG_C|GetEnemySpotMap _asgi_rpg) (Variables|Default|GetcurrentIndex))) true))

(fn ConstructionScript
  (|CallParentFunction))

(fn TryBreakingPan
  (params (PointReference :type BP%20Enemy%20Spot%20Object%20Reference))
  (return true))

(fn RecoverSauceBar
  (bind _ac_characterbattlestats (Variables|Default|GetAC_CharacterBattleStats))
  (bind _returnvalue (Utilities|GetDataTableRow "/Game/Custom/DataTables/DT_Enemies.DT_Enemies" "BaseFarfalla")
    (:then
      (Variables|/Game/Custom/Components/AC_CharacterBattleStats.AC_CharacterBattleStats_C|SetCurrentHP _ac_characterbattlestats (Math|Float|Clamp(Float) (- (Variables|/Game/Custom/Components/AC_CharacterBattleStats.AC_CharacterBattleStats_C|GetCurrentHP _ac_characterbattlestats) (.SauceBarRegen (Utilities|Struct|BreakS_Enemy _returnvalue))) 0.0 (.Value (Utilities|Map|Find (Variables|/Game/Custom/Components/AC_CharacterBattleStats.AC_CharacterBattleStats_C|GetCharacterStats (Variables|Default|GetAC_CharacterBattleStats)) "NewEnumerator1"))))
      (Default|RefreshHP _ac_characterbattlestats))))

(fn StartRegeneration
  (bind _returnvalue (Utilities|GetDataTableRow "/Game/Custom/DataTables/DT_Enemies.DT_Enemies" "BaseFarfalla")
    (:then
      (Variables|Default|SetcookTime (Math|Integer|Clamp(Integer) (+ (Variables|Default|GetcookTime) (Variables|Default|GetcookTimeRegen)) 0 (.CookingTime (Utilities|Struct|BreakS_Enemy _returnvalue))))
      (CallFunction|UpdateCookTime)
      (if (Variables|Default|GetStartRegen)
        (if (== (Variables|Default|GetcookTime) (.CookingTime (Utilities|Struct|BreakS_Enemy _returnvalue)))
          (CallFunction|RecoverSauceBar)
          (if (Variables|Default|GetisSoiled)
            (Variables|Default|SetisSoiled false)
            (bind _asgi_rpg (Utilities|Casting|CastToGI_RPG (Game|GetGameInstance)))
            (Variables|/Game/Custom/BP_EnemySpot.BP_EnemySpot_C|SetisEnemySoiled (.Value (Utilities|Map|Find (Variables|/Game/Custom/GI_RPG.GI_RPG_C|GetEnemySpotMap _asgi_rpg) (Variables|Default|GetcurrentIndex))) false)))
        (elif (Variables|Default|GetwasHitLastTurn)
          (Variables|Default|SetwasHitLastTurn false)
          (else
            (Variables|Default|SetStartRegen true)))))))

(fn IsGettingCookedFunction
  (bind _output_get (Variables|Default|SetcookTime (- (Variables|Default|GetcookTime) 1)))
  (Development|PrintString (Utilities|String|Append "Turn before death for" (Utilities|GetDisplayName self) ": " (Utilities|String|ToString(Integer) _output_get)))
  (CallFunction|UpdateCookTime)
  (if (<= _output_get 0)
    (return true)
    (else
      (return false))))

(fn AttackPlayerFunction
  (bind _ac_characterbattlestats (Variables|Default|GetAC_CharacterBattleStats))
  (bind _battlemanagerreference (Variables|/Game/Custom/Components/AC_CharacterBattleStats.AC_CharacterBattleStats_C|GetBattleManagerReference _ac_characterbattlestats))
  (|CallParentFunction)
  (LocalVariables|SetAttackValue (.Value (Utilities|Map|Find (Variables|/Game/Custom/Components/AC_CharacterBattleStats.AC_CharacterBattleStats_C|GetCharacterStats _ac_characterbattlestats) "NewEnumerator3")))
  (if (not (>= (+ (Variables|/Game/Custom/Components/AC_BattleManager.AC_BattleManager_C|GetDamageToPlayer _battlemanagerreference) (Variables|/Game/Custom/Components/AC_CharacterBattleStats.AC_CharacterBattleStats_C|GetCurrentHP (Variables|/Game/Custom/BP_BaseRPGCharacter.BP_BaseRPGCharacter_C|GetAC_CharacterBattleStats (Variables|/Game/Custom/Components/AC_BattleManager.AC_BattleManager_C|GetPlayerCharacter _battlemanagerreference)))) 1e+02))
    (bind _returnvalue (Utilities|GetDataTableRow "/Game/Custom/DataTables/DT_Enemies.DT_Enemies" "BaseFarfalla")
      (:then
        (Development|PrintString (Utilities|String|Append "Attacked with:" (Utilities|String|EnumtoString (Utilities|Array|Get(acopy) (.Ingredients (Utilities|Struct|BreakS_Enemy _returnvalue)) (Math|Random|RandomIntegerinRange 0 (- (Utilities|Array|Length (.Ingredients (Utilities|Struct|BreakS_Enemy _returnvalue))) 1))))))
        (Default|AddEnemyAttack (Variables|Default|GetBattleManagerRef) (LocalVariables|GetAttackValue) (Utilities|Array|Get(acopy) (.Ingredients (Utilities|Struct|BreakS_Enemy _returnvalue)) (Math|Random|RandomIntegerinRange 0 (- (Utilities|Array|Length (.Ingredients (Utilities|Struct|BreakS_Enemy _returnvalue))) 1))) self)))))

(fn MoveFunction
  (Variables|MoveFunction|SetFirstWasASuccess false)
  (Variables|MoveFunction|SetsecondWasASuccess false)
  (bind _returnvalue (Utilities|GetDataTableRow "/Game/Custom/DataTables/DT_Enemies.DT_Enemies" "BaseFarfalla")
    (:then
      (CallFunction|CreatePointArray)
      (bind _index (Utilities|FlowControl|ForLoopwithBreak 0 (- (.MovementValue (Utilities|Struct|BreakS_Enemy _returnvalue)) 1) :!label _label)
        (:LoopBody
          (bind (_didfly_ _didfailfly_) (CallFunction|MovefromPosition _index (Variables|MoveFunction|GetMoveArray)))
          (if (or _didfly_ _didfailfly_)
            (goto _label Break)))
        (:Completed
          (if (or (Variables|MoveFunction|GetFirstWasASuccess) (Variables|MoveFunction|GetsecondWasASuccess))
            _))))))

(fn CreatePointArray
  (bind _currentindex (Variables|Default|GetCurrentIndex))
  (Variables|MoveFunction|SetMoveArray (Utilities|Array|MakeArray (- _currentindex 5) (- _currentindex 10))))

(fn MovefromPosition
  (params (loopIndex :type Integer) (PointArray :type Array%20of%20Integers))
  (LocalVariables|SetPossibleIndexMoves PointArray)
  (bind _asgi_rpg (Utilities|Casting|CastToGI_RPG (Game|GetGameInstance)))
  (LocalVariables|SetlocalSelectedSpot (.Value (Utilities|Map|Find (Variables|/Game/Custom/GI_RPG.GI_RPG_C|GetEnemySpotMap _asgi_rpg) (Utilities|Array|Get(acopy) (LocalVariables|GetPossibleIndexMoves) loopIndex))))
  (LocalVariables|SetcurrentSelectedSpot (.Value (Utilities|Map|Find (Variables|/Game/Custom/GI_RPG.GI_RPG_C|GetEnemySpotMap _asgi_rpg) (Variables|Default|GetcurrentIndex))))
  (if (.ReturnValue (Utilities|Map|Find (Variables|/Game/Custom/GI_RPG.GI_RPG_C|GetEnemySpotMap _asgi_rpg) (Utilities|Array|Get(acopy) (LocalVariables|GetPossibleIndexMoves) loopIndex)))
    (if (or (Variables|/Game/Custom/BP_EnemySpot.BP_EnemySpot_C|GetisOccupied (.Value (Utilities|Map|Find (Variables|/Game/Custom/GI_RPG.GI_RPG_C|GetEnemySpotMap _asgi_rpg) (Utilities|Array|Get(acopy) (LocalVariables|GetPossibleIndexMoves) loopIndex)))) (Variables|/Game/Custom/BP_EnemySpot.BP_EnemySpot_C|GetisOccupiedByPan (.Value (Utilities|Map|Find (Variables|/Game/Custom/GI_RPG.GI_RPG_C|GetEnemySpotMap _asgi_rpg) (Utilities|Array|Get(acopy) (LocalVariables|GetPossibleIndexMoves) loopIndex)))))
      (if (and (== loopIndex 0) (not (Variables|Default|GetisSoiled)))
        (if (.ReturnValue (Utilities|Map|Find (Variables|/Game/Custom/GI_RPG.GI_RPG_C|GetEnemySpotMap _asgi_rpg) (Utilities|Array|Get(acopy) (LocalVariables|GetPossibleIndexMoves) 1)))
          (if (or (not (Variables|/Game/Custom/BP_EnemySpot.BP_EnemySpot_C|GetisOccupied (.Value (Utilities|Map|Find (Variables|/Game/Custom/GI_RPG.GI_RPG_C|GetEnemySpotMap _asgi_rpg) (Utilities|Array|Get(acopy) (LocalVariables|GetPossibleIndexMoves) 1))))) (Variables|/Game/Custom/BP_EnemySpot.BP_EnemySpot_C|GetisOccupiedByPan (.Value (Utilities|Map|Find (Variables|/Game/Custom/GI_RPG.GI_RPG_C|GetEnemySpotMap _asgi_rpg) (Utilities|Array|Get(acopy) (LocalVariables|GetPossibleIndexMoves) 1)))))
            (bind _output_get (LocalVariables|SetlocalFliedToPoint (.Value (Utilities|Map|Find (Variables|/Game/Custom/GI_RPG.GI_RPG_C|GetEnemySpotMap _asgi_rpg) (Utilities|Array|Get(acopy) (LocalVariables|GetPossibleIndexMoves) 1)))))
            (Transformation|SetActorLocation (Math|Vector|MakeVector (.x (Transformation|GetActorLocation _output_get)) (.y (Transformation|GetActorLocation _output_get)) (.z (Transformation|GetActorLocation))) false true)
            (Variables|/Game/Custom/BP_EnemySpot.BP_EnemySpot_C|SetisOccupied (LocalVariables|GetcurrentSelectedSpot) false)
            (Variables|/Game/Custom/BP_EnemySpot.BP_EnemySpot_C|SetenemyReference (LocalVariables|GetcurrentSelectedSpot) 0)
            (Variables|/Game/Custom/BP_EnemySpot.BP_EnemySpot_C|SetisEnemySoiled (LocalVariables|GetcurrentSelectedSpot) false)
            (Default|StopShowing (LocalVariables|GetcurrentSelectedSpot))
            (Variables|/Game/Custom/BP_EnemySpot.BP_EnemySpot_C|SetenemyReference (LocalVariables|GetlocalFliedToPoint) self)
            (Variables|/Game/Custom/BP_EnemySpot.BP_EnemySpot_C|SetisEnemySoiled (LocalVariables|GetlocalFliedToPoint) (Variables|Default|GetisSoiled))
            (Variables|/Game/Custom/BP_EnemySpot.BP_EnemySpot_C|SetisOccupied (LocalVariables|GetlocalFliedToPoint) true)
            (Default|StopShowing (LocalVariables|GetlocalFliedToPoint))
            (Variables|Default|SetcurrentIndex (Variables|/Game/Custom/BP_EnemySpot.BP_EnemySpot_C|GetSlotIndex (LocalVariables|GetlocalFliedToPoint)))
            (Development|PrintString "Flied Over Obstacle")
            (Variables|MoveFunction|SetFirstWasASuccess true)
            (return true false)
            (else
              _)))
        (return false true)
        (elif (and (not (Variables|/Game/Custom/BP_EnemySpot.BP_EnemySpot_C|GetisOccupied (.Value (Utilities|Map|Find (Variables|/Game/Custom/GI_RPG.GI_RPG_C|GetEnemySpotMap _asgi_rpg) (Utilities|Array|Get(acopy) (LocalVariables|GetPossibleIndexMoves) loopIndex))))) (Variables|/Game/Custom/BP_EnemySpot.BP_EnemySpot_C|GetisOccupiedByPan (.Value (Utilities|Map|Find (Variables|/Game/Custom/GI_RPG.GI_RPG_C|GetEnemySpotMap _asgi_rpg) (Utilities|Array|Get(acopy) (LocalVariables|GetPossibleIndexMoves) loopIndex)))))
          _
          (else
            (Development|PrintString "Movement Failed")
            (return false true)))))
    (Transformation|SetActorLocation (Math|Vector|MakeVector (.x (Transformation|GetActorLocation (.Value (Utilities|Map|Find (Variables|/Game/Custom/GI_RPG.GI_RPG_C|GetEnemySpotMap _asgi_rpg) (Utilities|Array|Get(acopy) (LocalVariables|GetPossibleIndexMoves) loopIndex))))) (.y (Transformation|GetActorLocation (.Value (Utilities|Map|Find (Variables|/Game/Custom/GI_RPG.GI_RPG_C|GetEnemySpotMap _asgi_rpg) (Utilities|Array|Get(acopy) (LocalVariables|GetPossibleIndexMoves) loopIndex))))) (.z (Transformation|GetActorLocation))) false true)
    (Variables|/Game/Custom/BP_EnemySpot.BP_EnemySpot_C|SetisOccupied (LocalVariables|GetcurrentSelectedSpot) false)
    (Variables|/Game/Custom/BP_EnemySpot.BP_EnemySpot_C|SetenemyReference (LocalVariables|GetcurrentSelectedSpot) 0)
    (Variables|/Game/Custom/BP_EnemySpot.BP_EnemySpot_C|SetisEnemySoiled (LocalVariables|GetcurrentSelectedSpot) false)
    (Default|StopShowing (LocalVariables|GetcurrentSelectedSpot))
    (Variables|/Game/Custom/BP_EnemySpot.BP_EnemySpot_C|SetenemyReference (LocalVariables|GetlocalSelectedSpot) self)
    (Variables|/Game/Custom/BP_EnemySpot.BP_EnemySpot_C|SetisEnemySoiled (LocalVariables|GetlocalSelectedSpot) (Variables|Default|GetisSoiled))
    (Variables|/Game/Custom/BP_EnemySpot.BP_EnemySpot_C|SetisOccupied (LocalVariables|GetlocalSelectedSpot) true)
    (Default|StopShowing (LocalVariables|GetlocalSelectedSpot))
    (Variables|Default|SetcurrentIndex (Variables|/Game/Custom/BP_EnemySpot.BP_EnemySpot_C|GetSlotIndex (LocalVariables|GetlocalSelectedSpot)))
    (if (== loopIndex 0)
      (Variables|MoveFunction|SetFirstWasASuccess true)
      (else
        (Variables|MoveFunction|SetsecondWasASuccess true)))))

(fn SelectActionfortheTurn
  (Variables|Default|SetselectedAction "NewEnumerator0"))

(fn SimulateMove
  (Variables|MoveFunction|SetFirstWasASuccess false)
  (Variables|MoveFunction|SetsecondWasASuccess false)
  (bind _returnvalue (Utilities|GetDataTableRow "/Game/Custom/DataTables/DT_Enemies.DT_Enemies" "BaseFarfalla")
    (:then
      (CallFunction|CreatePointArray)
      (bind _index (Utilities|FlowControl|ForLoopwithBreak 0 (- (.MovementValue (Utilities|Struct|BreakS_Enemy _returnvalue)) 1) :!label _label)
        (:LoopBody
          (bind (_didfly_ _didfailfly_) (CallFunction|SimulateMoveFunction _index (Variables|MoveFunction|GetMoveArray)))
          (if (or _didfly_ _didfailfly_)
            (goto _label Break)))
        (:Completed
          (if (not (or (Variables|MoveFunction|GetFirstWasASuccess) (Variables|MoveFunction|GetsecondWasASuccess)))
            (Development|PrintString (Utilities|String|Append (Utilities|GetDisplayName self) " " "Cannot move"))
            (CallFunction|GotoRightTurnArray)))))))

(fn SimulateMoveFunction
  (params (loopIndex :type Integer) (PointArray :type Array%20of%20Integers))
  (LocalVariables|SetPossibleIndexMoves PointArray)
  (bind _asgi_rpg (Utilities|Casting|CastToGI_RPG (Game|GetGameInstance)))
  (LocalVariables|SetlocalSelectedSpot (.Value (Utilities|Map|Find (Variables|/Game/Custom/GI_RPG.GI_RPG_C|GetEnemySpotMap _asgi_rpg) (Utilities|Array|Get(acopy) (LocalVariables|GetPossibleIndexMoves) loopIndex))))
  (LocalVariables|SetcurrentSelectedSpot (.Value (Utilities|Map|Find (Variables|/Game/Custom/GI_RPG.GI_RPG_C|GetEnemySpotMap _asgi_rpg) (Variables|Default|GetcurrentIndex))))
  (if (.ReturnValue (Utilities|Map|Find (Variables|/Game/Custom/GI_RPG.GI_RPG_C|GetEnemySpotMap _asgi_rpg) (Utilities|Array|Get(acopy) (LocalVariables|GetPossibleIndexMoves) loopIndex)))
    (if (or (Variables|/Game/Custom/BP_EnemySpot.BP_EnemySpot_C|GetisOccupied (.Value (Utilities|Map|Find (Variables|/Game/Custom/GI_RPG.GI_RPG_C|GetEnemySpotMap _asgi_rpg) (Utilities|Array|Get(acopy) (LocalVariables|GetPossibleIndexMoves) loopIndex)))) (Variables|/Game/Custom/BP_EnemySpot.BP_EnemySpot_C|GetisOccupiedByPan (.Value (Utilities|Map|Find (Variables|/Game/Custom/GI_RPG.GI_RPG_C|GetEnemySpotMap _asgi_rpg) (Utilities|Array|Get(acopy) (LocalVariables|GetPossibleIndexMoves) loopIndex)))))
      (if (and (== loopIndex 0) (not (Variables|Default|GetisSoiled)))
        (if (.ReturnValue (Utilities|Map|Find (Variables|/Game/Custom/GI_RPG.GI_RPG_C|GetEnemySpotMap _asgi_rpg) (Utilities|Array|Get(acopy) (LocalVariables|GetPossibleIndexMoves) 1)))
          (if (or (not (Variables|/Game/Custom/BP_EnemySpot.BP_EnemySpot_C|GetisOccupied (.Value (Utilities|Map|Find (Variables|/Game/Custom/GI_RPG.GI_RPG_C|GetEnemySpotMap _asgi_rpg) (Utilities|Array|Get(acopy) (LocalVariables|GetPossibleIndexMoves) 1))))) (Variables|/Game/Custom/BP_EnemySpot.BP_EnemySpot_C|GetisOccupiedByPan (.Value (Utilities|Map|Find (Variables|/Game/Custom/GI_RPG.GI_RPG_C|GetEnemySpotMap _asgi_rpg) (Utilities|Array|Get(acopy) (LocalVariables|GetPossibleIndexMoves) 1)))))
            (Variables|MoveFunction|SetFirstWasASuccess true)
            (return true false)
            (else
              _)))
        (return false true)
        (elif (and (not (Variables|/Game/Custom/BP_EnemySpot.BP_EnemySpot_C|GetisOccupied (.Value (Utilities|Map|Find (Variables|/Game/Custom/GI_RPG.GI_RPG_C|GetEnemySpotMap _asgi_rpg) (Utilities|Array|Get(acopy) (LocalVariables|GetPossibleIndexMoves) loopIndex))))) (Variables|/Game/Custom/BP_EnemySpot.BP_EnemySpot_C|GetisOccupiedByPan (.Value (Utilities|Map|Find (Variables|/Game/Custom/GI_RPG.GI_RPG_C|GetEnemySpotMap _asgi_rpg) (Utilities|Array|Get(acopy) (LocalVariables|GetPossibleIndexMoves) loopIndex)))))
          _
          (else
            (Development|PrintString "Movement Failed")
            (return false true)))))
    (if (== loopIndex 0)
      (Variables|MoveFunction|SetFirstWasASuccess true)
      (else
        (Variables|MoveFunction|SetsecondWasASuccess true)))))