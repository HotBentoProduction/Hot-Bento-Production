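; Base spaghetto enemy for turn-based RPG battles, with cooking, sleep, soiling and regeneration mechanics, tuned from the BaseMaccherone row of DT_Enemies.
; On its AI turn, cooking counts CookTime down to death; otherwise it regenerates, then sleeps or runs one of two StateTrees chosen by HP.
; CookTime regenerates each uncooked turn; once full, and after a hit-free delay, sauce-bar recovery adjusts HP and clears soiled status in GI_RPG.
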(event EventBeginPlay
  (|CallParentFunction)
  (bind _returnvalue (Utilities|GetDataTableRow "/Game/Custom/DataTables/DT_Enemies.DT_Enemies" "BaseMaccherone")
    (:then
      (Variables|Default|SetcookTimeRegen (.CookingTimeRegen (Utilities|Struct|BreakS_Enemy _returnvalue)))
      (Variables|Default|SetcookTime (.CookingTime (Utilities|Struct|BreakS_Enemy _returnvalue))))))

(event Collision|EventActorBeginOverlap
  (params (OtherActor :type Actor%20Object%20Reference))
  (|CallParentFunction OtherActor) ; This node is disabled and will not be called.\nDrag off pins to build functionality.
)

(event EventPerformActionbyAI
  (bind _ac_characterbattlestats (Variables|Default|GetAC_CharacterBattleStats))
  (Variables|Default|SetwasAsleep? false)
  (if (Variables|Default|GetisGettingCooked)
    (bind _isdead (CallFunction|IsGettingCookedFunction))
    (if _isdead
      (Utilities|FlowControl|Delay 1.0)
      (Default|EndCharacterTurn (Variables|Default|GetBattleManagerReferences))
      (CallFunction|OnDeath)
      (else
        (if (== (Math|Random|RandomIntegerinRange 0 (Variables|Default|GetsleepCounter)) 0) :!label _label
          (Development|PrintString "Sleep was inefective")
          (else
            (Development|PrintString "Target is asleep")))
        (Variables|Default|SetsleepCounter 0)
        (Variables|Default|SetwasAsleep? true)
        (Utilities|FlowControl|Delay 1.0 :!label _label_2)
        (Default|EndCharacterTurn (Variables|Default|GetBattleManagerReferences))))
    (else
      (CallFunction|StartRegeneration)
      (if (> (Variables|Default|GetsleepCounter) 0)
        (goto _label)
        (else
          (Development|PrintString (Utilities|GetDisplayName self))
          (if (< (Variables|/Game/Custom/Components/AC_CharacterBattleStats.AC_CharacterBattleStats_C|GetCurrentHP _ac_characterbattlestats) (* (.Value (Utilities|Map|Find (Variables|/Game/Custom/Components/AC_CharacterBattleStats.AC_CharacterBattleStats_C|GetCharacterStats _ac_characterbattlestats) "NewEnumerator1")) 0.5))
            (AI|Logic|StartLogic (Variables|Default|GetStateTree))
            (goto _label_2)
            (else
              (AI|Logic|StartLogic (Variables|Default|GetStateTreeHalfHP))
              (goto _label_2))))))))

(event EventTick
  (params (DeltaSeconds :type Float%20%28single-precision%29))
  (|CallParentFunction DeltaSeconds) ; This node is disabled and will not be called.\nDrag off pins to build functionality.
)

(event EventOnDamageReceived
  (params (Damage :type Float%20%28double-precision%29) (Critical :type Boolean))
  (Variables|Default|SetwasHitLastTurn true)
  (Variables|Default|SetStartRegen false))

(event EventUpdateCookTime
  (Rendering|Components|TextRender|SetText (Variables|/Game/Custom/Widgets/BattleWidgets/Widget_BattleCharacterSlot.Widget_BattleCharacterSlot_C|GetTextBlock_MP (Variables|/Game/Custom/Components/AC_CharacterBattleStats.AC_CharacterBattleStats_C|GetCharacterBattleSlotReference (Variables|Default|GetAC_CharacterBattleStats))) (Utilities|Text|ToText(String) (Utilities|String|Append "CookTime:" (Utilities|String|ToString(Integer) (Variables|Default|GetcookTime))))))

(event EventOnSoiled
  (Variables|Default|SetisSoiled true)
  (bind _asgi_rpg (Utilities|Casting|CastToGI_RPG (Game|GetGameInstance)))
  (Variables|/Game/Custom/BP_EnemySpot.BP_EnemySpot_C|SetisEnemySoiled (.Value (Utilities|Map|Find (Variables|/Game/Custom/GI_RPG.GI_RPG_C|GetEnemySpotMap _asgi_rpg) (Variables|Default|GetcurrentIndex))) true))

(fn ConstructionScript
  (|CallParentFunction))

(fn TryBreakingPan
  (params (PointReference :type BP%20Enemy%20Spot%20Object%20Reference))
  (return true))

(fn RecoverSauceBar
  (bind _ac_characterbattlestats (Variables|Default|GetAC_CharacterBattleStats))
  (bind _returnvalue (Utilities|GetDataTableRow "/Game/Custom/DataTables/DT_Enemies.DT_Enemies" "BaseMaccherone")
    (:then
      (Variables|/Game/Custom/Components/AC_CharacterBattleStats.AC_CharacterBattleStats_C|SetCurrentHP _ac_characterbattlestats (Math|Float|Clamp(Float) (- (Variables|/Game/Custom/Components/AC_CharacterBattleStats.AC_CharacterBattleStats_C|GetCurrentHP _ac_characterbattlestats) (.SauceBarRegen (Utilities|Struct|BreakS_Enemy _returnvalue))) 0.0 (.Value (Utilities|Map|Find (Variables|/Game/Custom/Components/AC_CharacterBattleStats.AC_CharacterBattleStats_C|GetCharacterStats (Variables|Default|GetAC_CharacterBattleStats)) "NewEnumerator1"))))
      (Default|RefreshHP _ac_characterbattlestats))))

(fn StartRegeneration
  (bind _returnvalue (Utilities|GetDataTableRow "/Game/Custom/DataTables/DT_Enemies.DT_Enemies" "BaseMaccherone")
    (:then
      (Variables|Default|SetcookTime (Math|Integer|Clamp(Integer) (+ (Variables|Default|GetcookTime) (Variables|Default|GetcookTimeRegen)) 0 (.CookingTime (Utilities|Struct|BreakS_Enemy _returnvalue))))
      (CallFunction|UpdateCookTime)
      (if (Variables|Default|GetStartRegen)
        (if (== (Variables|Default|GetcookTime) (.CookingTime (Utilities|Struct|BreakS_Enemy _returnvalue)))
          (CallFunction|RecoverSauceBar)
          (if (Variables|Default|GetisSoiled)
            (Variables|Default|SetisSoiled false)
            (bind _asgi_rpg (Utilities|Casting|CastToGI_RPG (Game|GetGameInstance)))
            (Variables|/Game/Custom/BP_EnemySpot.BP_EnemySpot_C|SetisEnemySoiled (.Value (Utilities|Map|Find (Variables|/Game/Custom/GI_RPG.GI_RPG_C|GetEnemySpotMap _asgi_rpg) (Variables|Default|GetcurrentIndex))) false)))
        (elif (Variables|Default|GetwasHitLastTurn)
          (Variables|Default|SetwasHitLastTurn false)
          (else
            (Variables|Default|SetStartRegen true)))))))

(fn IsGettingCookedFunction
  (bind _output_get (Variables|Default|SetcookTime (- (Variables|Default|GetcookTime) 1)))
  (Development|PrintString (Utilities|String|Append "Turn before death for" (Utilities|GetDisplayName self) ": " (Utilities|String|ToString(Integer) _output_get)))
  (CallFunction|UpdateCookTime)
  (if (<= _output_get 0)
    (return true)
    (else
      (return false))))