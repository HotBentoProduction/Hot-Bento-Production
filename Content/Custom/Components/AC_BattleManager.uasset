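; Turn-based RPG battle manager component that runs fights from encounter map loading to victory or game over.
; It saves world state to GI_RPG, spawns the player and enemies at spot actors, and writes HP/MP back after victory.
; Turns follow descending speed, alternating between AI actions and player menus.
; Menus fill pooled widgets with items, abilities or Pasta, then pass choices to sibling action and targeting components.
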(event EventBeginPlay
  (bind _asgi_rpg (Utilities|Casting|CastToGI_RPG (Game|GetGameInstance) :!label _label)
    (:then
      (Variables|Default|SetGameInstanceReference _asgi_rpg))
    (:CastFailed
      (Utilities|FlowControl|Delay 0.1)
      (goto _label))))

(event Custom|EndBattle
  (BattleEnd|Functionality|GoBacktoWorldMap)
  (Utilities|FlowControl|Delay 2.0)
  (Game|OpenLevel(byName) (Variables|/Game/Custom/GI_RPG.GI_RPG_C|GetMapName (Variables|Default|GetGameInstanceReference))))

(event Custom|GameOver
  (Utilities|FlowControl|Delay 2.0)
  (Game|QuitGame 0 "Quit" false))

(fn SelectAction
  (params (ActionType :type E_ActionType%20Enum :default "NewEnumerator0"))
  (bind _returnvalue (Components|GetOwner))
  (bind _slotindexlocal (LocalVariables|GetslotIndexLocal))
  (bind _currentcharacter (Variables|BattleInProgress|GetCurrentCharacter))
  (bind _returnvalue_2 (Actor|GetComponentbyClass _returnvalue "/Game/Custom/Components/AC_ActionManager.AC_ActionManager_C"))
  (bind _ac_characterbattlestats (Variables|/Game/Custom/BP_BaseRPGCharacter.BP_BaseRPGCharacter_C|GetAC_CharacterBattleStats _currentcharacter))
  (bind _output_get (Variables|BattleInProgress|SetSelectedAction ActionType))
  (switch Utilities|FlowControl|Switch|SwitchonE_ActionType _output_get
    (:NewEnumerator1
      (Utilities|IsValid _returnvalue_2 :!label _label
        (:Is%20Valid
          (Default|SelectAction _returnvalue_2 (Variables|BattleInProgress|GetSelectedAction) "None"))))
    (:NewEnumerator2
      (goto _label))
    (:NewEnumerator3
      (Variables|/Game/Custom/Components/AC_CharacterBattleStats.AC_CharacterBattleStats_C|SetSelectedActionType (Variables|/Game/Custom/BP_BaseRPGCharacter.BP_BaseRPGCharacter_C|GetAC_CharacterBattleStats (Variables|BattleInProgress|GetCurrentCharacter)) (Variables|BattleInProgress|GetSelectedAction))
      (Class|WidgetSwitcher|SetActiveWidgetIndex (Variables|/Game/Custom/Widgets/BattleWidgets/Widget_ActionsPanel.Widget_ActionsPanel_C|GetWidgetSwitcher_Actions (Variables|/Game/Custom/Widgets/BattleWidgets/Widget_BattleInterface.Widget_BattleInterface_C|GetWidget_ActionsPanel (Variables|Widgets|GetBattleInterfaceReference))) 1)
      (for _array_element (Variables|Widgets|GetSecondaryActionsReference)
        (Widget|SetVisibility _array_element "Collapsed")
        (Widget|SetIsEnabled _array_element true))
      (bind _usableitems (BattleInProgress|Functionality|Getters|GetAllItemsUsableinBattle (Variables|/Game/Custom/GI_RPG.GI_RPG_C|GetInventory (Variables|Default|GetGameInstanceReference))))
      (for (_array_element_2 _array_index) _usableitems
        (bind _output (BattleInProgress|Widgets|GetProperSecondaryActionWidget _array_index))
        (Utilities|IsValid _output
          (:Is%20Valid
            (Widget|SetVisibility _output "Visible")
            (Variables|/Game/Custom/Widgets/BattleWidgets/Widget_SecondaryAction.Widget_SecondaryAction_C|SetAssignedSecondaryAction _output (.ItemHardCodedName (Utilities|Struct|BreakS_ItemStaticData (.ItemStaticData (Utilities|Struct|BreakS_ItemDynamicData _array_element_2)))))
            (Rendering|Components|TextRender|SetText (Variables|/Game/Custom/Widgets/BattleWidgets/Widget_SecondaryAction.Widget_SecondaryAction_C|GetTextBlock_Name _output) (.ItemDisplayName (Utilities|Struct|BreakS_ItemStaticData (.ItemStaticData (Utilities|Struct|BreakS_ItemDynamicData _array_element_2)))))
            (Rendering|Components|TextRender|SetText (Variables|/Game/Custom/Widgets/BattleWidgets/Widget_SecondaryAction.Widget_SecondaryAction_C|GetTextBlock_Info _output) (Utilities|Text|ToText(Integer) (.StackAmount (Utilities|Struct|BreakS_ItemDynamicData _array_element_2))))))))
    (:NewEnumerator4
      (goto _label))
    (:NewEnumerator6
      (Variables|/Game/Custom/Components/AC_CharacterBattleStats.AC_CharacterBattleStats_C|SetSelectedActionType (Variables|/Game/Custom/BP_BaseRPGCharacter.BP_BaseRPGCharacter_C|GetAC_CharacterBattleStats (Variables|BattleInProgress|GetCurrentCharacter)) (Variables|BattleInProgress|GetSelectedAction))
      (Class|WidgetSwitcher|SetActiveWidgetIndex (Variables|/Game/Custom/Widgets/BattleWidgets/Widget_ActionsPanel.Widget_ActionsPanel_C|GetWidgetSwitcher_Actions (Variables|/Game/Custom/Widgets/BattleWidgets/Widget_BattleInterface.Widget_BattleInterface_C|GetWidget_ActionsPanel (Variables|Widgets|GetBattleInterfaceReference))) 1)
      (for _array_element_3 (Variables|Widgets|GetSecondaryActionsReference)
        (Widget|SetVisibility _array_element_3 "Collapsed")
        (Widget|SetIsEnabled _array_element_3 true))
      (bind _keys (Utilities|Map|Keys (.CharacterActions (Utilities|Struct|BreakS_Character (.Value (Utilities|Map|Find (Variables|/Game/Custom/GI_RPG.GI_RPG_C|GetCharacterCollection (Variables|Default|GetGameInstanceReference)) (Variables|/Game/Custom/Components/AC_CharacterBattleStats.AC_CharacterBattleStats_C|GetCharacterHardcodedName (Variables|/Game/Custom/BP_BaseRPGCharacter.BP_BaseRPGCharacter_C|GetAC_CharacterBattleStats (Variables|BattleInProgress|GetCurrentCharacter)))))))))
      (for _array_element_4 _keys
        (bind _returnvalue_3 (Utilities|GetDataTableRow "/Game/Custom/DataTables/DT_Actions.DT_Actions" _array_element_4)
          (:then
            (if (Utilities|Enum|Equal(Enum) (.ActionType (Utilities|Struct|BreakS_Actions _returnvalue_3)) (Variables|BattleInProgress|GetSelectedAction))
              (Math|Integer|IncrementInt _slotindexlocal
                (:%20%20
                  (bind _output_2 (BattleInProgress|Widgets|GetProperSecondaryActionWidget _slotindexlocal))
                  (Utilities|IsValid _output_2
                    (:Is%20Valid
                      (Widget|SetVisibility _output_2 "Visible")
                      (bind _output_get_2 (Variables|/Game/Custom/Widgets/BattleWidgets/Widget_SecondaryAction.Widget_SecondaryAction_C|SetAssignedSecondaryAction _output_2 (.HardCodedName (Utilities|Struct|BreakS_Actions _returnvalue_3))))
                      (Variables|/Script/UMG.TextBlock|SetText (Variables|/Game/Custom/Widgets/BattleWidgets/Widget_SecondaryAction.Widget_SecondaryAction_C|GetTextBlock_Name _output_2) (.DisplayName (Utilities|Struct|BreakS_Actions _returnvalue_3)))
                      (bind (_costhp _costmp) (Default|GetActionCost (Actor|GetComponentbyClass (Components|GetOwner) "/Game/Custom/Components/AC_ActionManager.AC_ActionManager_C") _output_get_2))
                      (Variables|/Script/UMG.TextBlock|SetText (Variables|/Game/Custom/Widgets/BattleWidgets/Widget_SecondaryAction.Widget_SecondaryAction_C|GetTextBlock_Info _output_2) (Utilities|Text|FormatText "{HP cost}{MP cost}" (select (> _costhp 0.0) (Utilities|Text|FormatText "{cost} HP" (Utilities|Text|ToText(Float) _costhp "HalfToEven")) "") (Utilities|Text|FormatText "{cost} MP" (Utilities|Text|ToText(Float) _costmp "HalfToEven"))))
                      (Widget|SetIsEnabled _output_2 (and (>= (Variables|/Game/Custom/Components/AC_CharacterBattleStats.AC_CharacterBattleStats_C|GetCurrentHP _ac_characterbattlestats) _costhp) (>= (Variables|/Game/Custom/Components/AC_CharacterBattleStats.AC_CharacterBattleStats_C|GetCurrentMP _ac_characterbattlestats) _costmp))))))))))))
    (:NewEnumerator8
      ;[0.15 0.15 0.15 0.5] Set targets of Attack
      (Variables|/Game/Custom/Components/AC_CharacterBattleStats.AC_CharacterBattleStats_C|SetSelectedActionType (Variables|/Game/Custom/BP_BaseRPGCharacter.BP_BaseRPGCharacter_C|GetAC_CharacterBattleStats (Variables|BattleInProgress|GetCurrentCharacter)) (Variables|BattleInProgress|GetSelectedAction))
      (Class|WidgetSwitcher|SetActiveWidgetIndex (Variables|/Game/Custom/Widgets/BattleWidgets/Widget_ActionsPanel.Widget_ActionsPanel_C|GetWidgetSwitcher_Actions (Variables|/Game/Custom/Widgets/BattleWidgets/Widget_BattleInterface.Widget_BattleInterface_C|GetWidget_ActionsPanel (Variables|Widgets|GetBattleInterfaceReference))) 1)
      (for _array_element_5 (Variables|Widgets|GetSecondaryActionsReference)
        (Widget|SetVisibility _array_element_5 "Collapsed")
        (Widget|SetIsEnabled _array_element_5 true))
      (bind _values (Utilities|Map|Values (Variables|/Game/Custom/GI_RPG.GI_RPG_C|GetPastaNameDictionary (Variables|Default|GetGameInstanceReference))))
      ;[0.15 0.15 0.15 0.5] For each Pasta check its values
      (for _array_element_6 _values
        (bind _result (Math|Integer|IncrementInt (LocalVariables|GetslotIndexLocal))
          (:%20%20
            (bind _output_3 (BattleInProgress|Widgets|GetProperSecondaryActionWidget _result))
            (Utilities|IsValid _output_3
              (:Is%20Valid
                (Widget|SetVisibility _output_3 "Visible")
                (Variables|/Game/Custom/Widgets/BattleWidgets/Widget_SecondaryAction.Widget_SecondaryAction_C|SetAssignedSecondaryAction _output_3 (.PastaHardCodedName (Utilities|Struct|BreakS_Pasta _array_element_6)))
                (Variables|/Script/UMG.TextBlock|SetText (Variables|/Game/Custom/Widgets/BattleWidgets/Widget_SecondaryAction.Widget_SecondaryAction_C|GetTextBlock_Name _output_3) (Utilities|Text|ToText(String) (.ItemDisplayName (Utilities|Struct|BreakS_Pasta _array_element_6))))
                (Widget|SetIsEnabled _output_3 true)
                (bind _costpasta (Default|GetPastaCost (Actor|GetComponentbyClass (Components|GetOwner) "/Game/Custom/Components/AC_ActionManager.AC_ActionManager_C") (.PastaHardCodedName (Utilities|Struct|BreakS_Pasta _array_element_6))))
                (Variables|/Script/UMG.TextBlock|SetText (Variables|/Game/Custom/Widgets/BattleWidgets/Widget_SecondaryAction.Widget_SecondaryAction_C|GetTextBlock_Info _output_3) (Utilities|Text|FormatText "{PastaCost}/{PastaCurrentAmount}" _costpasta (.PastaStackAmount (Utilities|Struct|BreakS_Pasta _array_element_6))))
                (Widget|SetIsEnabled _output_3 (>= (.PastaStackAmount (Utilities|Struct|BreakS_Pasta _array_element_6)) (.PastaConsumptionCost (Utilities|Struct|BreakS_Pasta _array_element_6))))))))))))

(fn RequestActionExecution
  (params (TargetedCharacter :type Array%20of%20BP%20Base%20RPG%20Character%20Object%20References))
  (bind _selectedaction (Variables|BattleInProgress|GetSelectedAction))
  (bind _selectedsecondaryaction (Variables|BattleInProgress|GetSelectedSecondaryAction))
  (Variables|/Game/Custom/Components/AC_CharacterBattleStats.AC_CharacterBattleStats_C|SetTargetedCharacters (Variables|/Game/Custom/BP_BaseRPGCharacter.BP_BaseRPGCharacter_C|GetAC_CharacterBattleStats (Variables|BattleInProgress|GetCurrentCharacter)) TargetedCharacter)
  (Utilities|FlowControl|Sequence
    (:then_0
      (Default|ActivateActionEvent (Utilities|GetActionManager) _selectedaction _selectedsecondaryaction)
      (Default|ExecuteAction (Variables|BattleInProgress|GetCurrentCharacter) _selectedaction _selectedsecondaryaction))
    (:then_1
      (BattleInProgress|Functionality|ActionSelection|DisableTargetingandInput))))

(fn SelectSecondaryAction
  (params (SelectedSecondaryAction :type Name))
  (bind _returnvalue (Components|GetOwner))
  (bind _returnvalue_2 (Actor|GetComponentbyClass _returnvalue "/Game/Custom/Components/AC_ActionManager.AC_ActionManager_C"))
  (Variables|BattleInProgress|SetSelectedSecondaryAction SelectedSecondaryAction)
  (Utilities|IsValid _returnvalue_2
    (:Is%20Valid
      (Default|SelectAction _returnvalue_2 (Variables|BattleInProgress|GetSelectedAction) (Variables|BattleInProgress|GetSelectedSecondaryAction)))))

(fn DisableTargetingandInput
  (bind _returnvalue (Components|GetOwner))
  (bind _returnvalue_2 (Actor|GetComponentbyClass _returnvalue "/Game/Custom/Components/AC_TargetingManager.AC_TargetingManager_C"))
  (Utilities|IsValid _returnvalue_2
    (:Is%20Valid
      (Default|DisableTargeting _returnvalue_2)
      (Default|HideTargets _returnvalue_2))))

(fn EncounterEnemies
  (params (EncounterName :type Name) (BattleMapName :type Name))
  (bind _returnvalue (Utilities|GetDataTableRow "/Game/Custom/DataTables/DT_EnemyEncounterDataTable.DT_EnemyEncounterDataTable" EncounterName)
    (:then
      (PreBattle|OpenBattleMap BattleMapName (Utilities|Struct|BreakS_EnemyEncounters _returnvalue)))))

(fn OpenBattleMap
  (params (BattleMapName :type Name) (EncounteredEnemies :type Map%20of%20Integers%20to%20Names))
  (bind _returnvalue (Game|Player|GetPlayerPawn 0))
  (Variables|/Game/Custom/GI_RPG.GI_RPG_C|SetEncounteredEnemies (Variables|Default|GetGameInstanceReference) EncounteredEnemies)
  (Variables|/Game/Custom/GI_RPG.GI_RPG_C|SetWorldTransformBeforeBattle (Variables|Default|GetGameInstanceReference) (Transformation|GetActorTransform _returnvalue))
  (Variables|/Game/Custom/GI_RPG.GI_RPG_C|SetCameraWorldRotationBeforeBattle (Variables|Default|GetGameInstanceReference) (Pawn|GetControlRotation _returnvalue :!class /Script/Engine.Pawn))
  (Game|OpenLevel(byName) BattleMapName))

(fn GetProperSpawnPoint
  (params (isEnemy :type Boolean) (Index :type Integer))
  (if isEnemy
    (bind _outactors (Actor|GetAllActorsOfClass "/Game/Custom/BP_EnemySpot.BP_EnemySpot_C"))
    (bind _array_element (Utilities|Array|ForEachLoopwithBreak _outactors :!label _label)
      (:LoopBody
        (if (== (Variables|/Game/Custom/BP_EnemySpot.BP_EnemySpot_C|GetSlotIndex _array_element) Index)
          (LocalVariables|SetbattleSpotTransfromLocal (Math|Transform|MakeTransform (Transformation|GetActorLocation _array_element) (.rotation (Transformation|GetWorldTransform (Variables|/Game/Custom/BP_EnemySpot.BP_EnemySpot_C|GetArrow _array_element))) (.scale (Transformation|GetWorldTransform (Variables|/Game/Custom/BP_EnemySpot.BP_EnemySpot_C|GetArrow _array_element)))))
          (goto _label Break)))
      (:Completed
        (return (LocalVariables|GetbattleSpotTransfromLocal))))
    (else
      (bind _returnvalue (Actor|GetActorOfClass "/Game/Custom/BP_MCSpot.BP_MCSpot_C"))
      (bind _output_get (LocalVariables|SetbattleSpotTransfromLocal (Math|Transform|MakeTransform (Math|Vector|MakeVector (.X (Math|Vector|BreakVector (.location (Transformation|GetWorldTransform (Variables|/Game/Custom/BP_MCSpot.BP_MCSpot_C|GetArrow _returnvalue))))) (.Y (Math|Vector|BreakVector (.location (Transformation|GetWorldTransform (Variables|/Game/Custom/BP_MCSpot.BP_MCSpot_C|GetArrow _returnvalue))))) (.z (Transformation|GetActorLocation _returnvalue))) (.rotation (Transformation|GetWorldTransform (Variables|/Game/Custom/BP_MCSpot.BP_MCSpot_C|GetArrow _returnvalue))) (.scale (Transformation|GetWorldTransform (Variables|/Game/Custom/BP_MCSpot.BP_MCSpot_C|GetArrow _returnvalue))))))
      (return _output_get))))

(fn SpawnPlayerCharacter
  (bind _gameinstancereference (Variables|Default|GetGameInstanceReference))
  (bind _charactercollection (Variables|/Game/Custom/GI_RPG.GI_RPG_C|GetCharacterCollection _gameinstancereference))
  (bind _maincharacter (Variables|/Game/Custom/GI_RPG.GI_RPG_C|GetMainCharacter _gameinstancereference))
  (bind _name (Utilities|Struct|BreakS_CharacterSlot _maincharacter))
  (bind _value (Utilities|Map|Find _charactercollection _name))
  (bind (_characterhardcodedname _characterdisplayname _currentlevel _currentexperience _availableactionpoints _characteractorclass _charactericon _currenthp _currentmp _characterstats) (Utilities|Struct|BreakS_Character _value))
  (bind _returnvalue (Game|SpawnActorfromClass "/Game/Custom/BP_MainCharacter.BP_MainCharacter_C" (BattleInit|Functionality|GetProperSpawnPoint false) "Undefined" "MultiplyWithRoot" 0 self 0))
  (Variables|/Game/Custom/BP_BaseRPGCharacter.BP_BaseRPGCharacter_C|SetTargetingManagerReference _returnvalue (Actor|GetComponentbyClass (Components|GetOwner) "/Game/Custom/Components/AC_TargetingManager.AC_TargetingManager_C"))
  (Variables|/Game/Custom/BP_BaseRPGCharacter.BP_BaseRPGCharacter_C|SetEnemy _returnvalue false)
  (Variables|/Game/Custom/BP_BaseRPGCharacter.BP_BaseRPGCharacter_C|SetControlledByAI _returnvalue false)
  (Default|SetCharacterData (Variables|/Game/Custom/BP_BaseRPGCharacter.BP_BaseRPGCharacter_C|GetAC_CharacterBattleStats _returnvalue) _characterdisplayname _characterstats _currenthp _currentmp)
  (bind _output_get (Variables|BattleInProgress|SetPlayerCharacter _returnvalue))
  (Default|CreateCharacterBattleSlot (Variables|/Game/Custom/BP_BaseRPGCharacter.BP_BaseRPGCharacter_C|GetAC_CharacterBattleStats _returnvalue))
  (Variables|/Game/Custom/Components/AC_CharacterBattleStats.AC_CharacterBattleStats_C|SetBattleManagerReference (Variables|/Game/Custom/BP_BaseRPGCharacter.BP_BaseRPGCharacter_C|GetAC_CharacterBattleStats _returnvalue) self)
  (Utilities|Array|Add (Variables|BattleInProgress|GetAllCharactersInBattle) _output_get))

(fn SpawnEnemies
  (bind _keys (Utilities|Map|Keys (Variables|/Game/Custom/GI_RPG.GI_RPG_C|GetEncounteredEnemies (Variables|Default|GetGameInstanceReference))))
  (for _array_element _keys
    (bind _returnvalue (Utilities|GetDataTableRow "/Game/Custom/DataTables/DT_Enemies.DT_Enemies" (.Value (Utilities|Map|Find (Variables|/Game/Custom/GI_RPG.GI_RPG_C|GetEncounteredEnemies (Variables|Default|GetGameInstanceReference)) _array_element)))
      (:then
        (bind _returnvalue_2 (Game|SpawnActorfromClass (.EnemyActorClass (Utilities|Struct|BreakS_Enemy _returnvalue)) (BattleInit|Functionality|GetProperSpawnPoint true _array_element) "Undefined" "OverrideRootScale" 0 0 0))
        (Variables|/Game/Custom/BP_BaseRPGCharacter.BP_BaseRPGCharacter_C|SetTargetingManagerReference _returnvalue_2 (Actor|GetComponentbyClass (Components|GetOwner) "/Game/Custom/Components/AC_TargetingManager.AC_TargetingManager_C"))
        (Variables|/Game/Custom/BP_BaseRPGCharacter.BP_BaseRPGCharacter_C|SetBattleManagerReferences _returnvalue_2 self)
        (Variables|/Game/Custom/BP_BaseRPGCharacter.BP_BaseRPGCharacter_C|SetControlledByAI _returnvalue_2 true)
        (Variables|/Game/Custom/BP_BaseRPGCharacter.BP_BaseRPGCharacter_C|SetEnemy _returnvalue_2 true)
        (Default|SetCharacterData (Variables|/Game/Custom/BP_BaseRPGCharacter.BP_BaseRPGCharacter_C|GetAC_CharacterBattleStats _returnvalue_2) (.EnemyDisplayName (Utilities|Struct|BreakS_Enemy _returnvalue)) (.EnemyStats (Utilities|Struct|BreakS_Enemy _returnvalue)) (.Value (Utilities|Map|Find (.EnemyStats (Utilities|Struct|BreakS_Enemy _returnvalue)) "NewEnumerator1")) (.Value (Utilities|Map|Find (.EnemyStats (Utilities|Struct|BreakS_Enemy _returnvalue)) "NewEnumerator2")))
        (Utilities|Array|Add (Variables|BattleInProgress|GetAllCharactersInBattle) _returnvalue_2)
        (Utilities|Array|Add (Variables|BattleInProgress|GetEnemies) _returnvalue_2)))))

(fn GetTurnOrder
  (if (not (== (Utilities|Array|Length (Variables|BattleInProgress|GetAllCharactersInBattle)) 1))
    (Variables|BattleInProgress|TurnOrder|SetSpeeds (Utilities|Array|MakeArray))
    (for _array_element (Variables|BattleInProgress|GetAllCharactersInBattle)
      (Utilities|Array|Add (Variables|BattleInProgress|TurnOrder|GetSpeeds) (.Value (Utilities|Map|Find (Variables|/Game/Custom/Components/AC_CharacterBattleStats.AC_CharacterBattleStats_C|GetCharacterStats (Variables|/Game/Custom/BP_BaseRPGCharacter.BP_BaseRPGCharacter_C|GetAC_CharacterBattleStats _array_element)) "NewEnumerator7"))))
    (Class|KismetArrayLibrary|SortFloatArray (Variables|BattleInProgress|TurnOrder|GetSpeeds) false "Descending")
    (for _array_element_2 (Variables|BattleInProgress|TurnOrder|GetSpeeds)
      (for _array_element_3 (Variables|BattleInProgress|GetAllCharactersInBattle)
        (if (== (.Value (Utilities|Map|Find (Variables|/Game/Custom/Components/AC_CharacterBattleStats.AC_CharacterBattleStats_C|GetCharacterStats (Variables|/Game/Custom/BP_BaseRPGCharacter.BP_BaseRPGCharacter_C|GetAC_CharacterBattleStats _array_element_3)) "NewEnumerator7")) _array_element_2)
          (Utilities|Array|AddUnique (Variables|BattleInProgress|TurnOrder|GetTurnOrder) _array_element_3))))
    (BattleInProgress|Functionality|TurnStart|GetNextCharacter)))

(fn GetNextCharacter
  (bind _turnorder (Variables|BattleInProgress|TurnOrder|GetTurnOrder))
  (bind _output (Utilities|Array|Get(acopy) _turnorder))
  (BattleInProgress|Functionality|TurnStart|StartCharacterTurn _output)
  (Utilities|Array|RemoveItem (Variables|BattleInProgress|TurnOrder|GetTurnOrder) _output))

(fn StartCharacterTurn
  (params (Character :type BP%20Base%20RPG%20Character%20Object%20Reference))
  (bind _output_get (Variables|BattleInProgress|SetCurrentCharacter Character))
  (if (not (Variables|/Game/Custom/BP_BaseRPGCharacter.BP_BaseRPGCharacter_C|GetControlledByAI _output_get))
    (Variables|/Game/Custom/Components/AC_CharacterBattleStats.AC_CharacterBattleStats_C|SetDefending (Variables|/Game/Custom/BP_BaseRPGCharacter.BP_BaseRPGCharacter_C|GetAC_CharacterBattleStats (Variables|BattleInProgress|GetCurrentCharacter)) false)
    (bind _characterbattleslotreference (Variables|/Game/Custom/Components/AC_CharacterBattleStats.AC_CharacterBattleStats_C|GetCharacterBattleSlotReference (Variables|/Game/Custom/BP_BaseRPGCharacter.BP_BaseRPGCharacter_C|GetAC_CharacterBattleStats (Variables|BattleInProgress|GetCurrentCharacter)))
      (:then
        (Default|HighlightSlot _characterbattleslotreference)
        (BattleInProgress|Widgets|ShowActionWidget))
      (:else))
    (else
      (Default|PerformActionbyAI (Variables|BattleInProgress|GetCurrentCharacter)))))

(fn ShowActionWidget
  (bind _battleinterfacereference (Variables|Widgets|GetBattleInterfaceReference))
  (bind _widget_actionspanel (Variables|/Game/Custom/Widgets/BattleWidgets/Widget_BattleInterface.Widget_BattleInterface_C|GetWidget_ActionsPanel _battleinterfacereference))
  (Utilities|IsValid (Variables|BattleInProgress|GetCurrentCharacter)
    (:Is%20Valid
      (Variables|/Script/UMG.TextBlock|SetText (Variables|/Game/Custom/Widgets/BattleWidgets/Widget_ActionsPanel.Widget_ActionsPanel_C|GetCharacterName _widget_actionspanel) (Variables|/Game/Custom/Components/AC_CharacterBattleStats.AC_CharacterBattleStats_C|GetCharacterDisplayName (Variables|/Game/Custom/BP_BaseRPGCharacter.BP_BaseRPGCharacter_C|GetAC_CharacterBattleStats (Variables|BattleInProgress|GetCurrentCharacter))))
      (Default|ShowActionSlots _widget_actionspanel (.CharacterActions (Utilities|Struct|BreakS_Character (.Value (Utilities|Map|Find (Variables|/Game/Custom/GI_RPG.GI_RPG_C|GetCharacterCollection (Variables|Default|GetGameInstanceReference)) (Variables|/Game/Custom/Components/AC_CharacterBattleStats.AC_CharacterBattleStats_C|GetCharacterHardcodedName (Variables|/Game/Custom/BP_BaseRPGCharacter.BP_BaseRPGCharacter_C|GetAC_CharacterBattleStats (Variables|BattleInProgress|GetCurrentCharacter))))))))
      (Widget|SetVisibility _widget_actionspanel "Visible"))))

(fn HideActionWidget
  (bind _battleinterfacereference (Variables|Widgets|GetBattleInterfaceReference)
    (:then
      (Widget|SetVisibility (Variables|/Game/Custom/Widgets/BattleWidgets/Widget_BattleInterface.Widget_BattleInterface_C|GetWidget_ActionsPanel _battleinterfacereference) "Hidden"))
    (:else)))

(fn ShowBattleToolTip
  (params (TooltipText :type Text))
  (bind _foundwidgets (Widget|GetAllWidgetsOfClass "/Game/Custom/Widgets/BattleWidgets/Widget_BattleInterface.Widget_BattleInterface_C" false))
  (Utilities|IsValid (Utilities|Array|Get(acopy) _foundwidgets)
    (:Is%20Valid
      (Rendering|Components|TextRender|SetText (Variables|/Game/Custom/Widgets/BattleWidgets/Widget_BattleInterface.Widget_BattleInterface_C|GetToolTipoText (Utilities|Array|Get(acopy) _foundwidgets)) TooltipText))))

(fn GetProperSecondaryActionWidget
  (params (SlotIndex :type Integer))
  (bind _secondaryactionsreference (Variables|Widgets|GetSecondaryActionsReference))
  (if (Utilities|Array|IsValidIndex _secondaryactionsreference SlotIndex)
    (return (Utilities|Array|Get(acopy) _secondaryactionsreference SlotIndex))
    (else
      (bind _returnvalue (UserInterface|CreateWidget "/Game/Custom/Widgets/BattleWidgets/Widget_SecondaryAction.Widget_SecondaryAction_C" 0 0))
      (Variables|/Game/Custom/Widgets/BattleWidgets/Widget_SecondaryAction.Widget_SecondaryAction_C|SetBattleManagerReference _returnvalue self)
      (Utilities|IsValid _returnvalue
        (:Is%20Valid
          (Utilities|Array|Add (Variables|Widgets|GetSecondaryActionsReference) _returnvalue)
          (Widget|Panel|AddChild (Variables|/Game/Custom/Widgets/BattleWidgets/Widget_ActionsPanel.Widget_ActionsPanel_C|GetContainerSecondaryActions (Variables|/Game/Custom/Widgets/BattleWidgets/Widget_BattleInterface.Widget_BattleInterface_C|GetWidget_ActionsPanel (Variables|Widgets|GetBattleInterfaceReference))) _returnvalue)
          (return _returnvalue))))))

(fn OnPlayerKilled
  (CallFunction|GameOver))

(fn OnEnemyKilled
  (params (Enemy :type BP%20Base%20RPG%20Character%20Object%20Reference))
  (bind _output_get (LocalVariables|SetenemyLocal Enemy))
  (Collision|SetCollisionResponsetoChannel (Variables|/Script/Engine.Character|GetCapsuleComponent _output_get) "ECC_Visibility" "ECR_Ignore")
  (Rendering|SetActorHiddenInGame (LocalVariables|GetenemyLocal) true)
  (Utilities|Array|RemoveItem (Variables|BattleInProgress|GetEnemies) (LocalVariables|GetenemyLocal))
  (Utilities|Array|RemoveItem (Variables|BattleInProgress|GetAllCharactersInBattle) (LocalVariables|GetenemyLocal))
  (Utilities|Array|RemoveItem (Variables|BattleInProgress|TurnOrder|GetTurnOrder) (LocalVariables|GetenemyLocal))
  (Utilities|Array|Add (Variables|BattleInProgress|GetDeadEnemies) (LocalVariables|GetenemyLocal))
  (if (== (Utilities|Array|Length (Variables|BattleInProgress|GetEnemies)) 0)
    (CallFunction|EndBattle)))

(fn GetAllItemsUsableinBattle
  (params (Inventory :type Array%20of%20S%20Item%20Dynamic%20Data%20Structures))
  (for _array_element Inventory
    (if (.CanBeUsedInBattle (Utilities|Struct|BreakS_ItemStaticData (.ItemStaticData (Utilities|Struct|BreakS_ItemDynamicData _array_element))))
      (if (not (Utilities|Array|ContainsItem (LocalVariables|GetalreadyAddedItems) (.ItemHardCodedName (Utilities|Struct|BreakS_ItemStaticData (.ItemStaticData (Utilities|Struct|BreakS_ItemDynamicData _array_element))))))
        (Utilities|Array|Add (LocalVariables|GetalreadyAddedItems) (.ItemHardCodedName (Utilities|Struct|BreakS_ItemStaticData (.ItemStaticData (Utilities|Struct|BreakS_ItemDynamicData _array_element)))))
        (bind _totalamountowned (Default|CheckAmountOfIteminInventory (Actor|GetComponentbyClass (Components|GetOwner) "/Game/Custom/Components/AC_InventoryManager.AC_InventoryManager_C") (.ItemHardCodedName (Utilities|Struct|BreakS_ItemStaticData (.ItemStaticData (Utilities|Struct|BreakS_ItemDynamicData _array_element))))))
        (bind _structout (Utilities|Struct|SetmembersinS_ItemDynamicData _array_element _totalamountowned))
        (Utilities|Array|Add (LocalVariables|GetusableItemsLocal) _structout))))
  (return (LocalVariables|GetusableItemsLocal)))

(fn EndCharacterTurn
  (Utilities|Array|RemoveItem (Variables|BattleInProgress|TurnOrder|GetTurnOrder) (Variables|BattleInProgress|GetCurrentCharacter))
  (BattleInProgress|Widgets|HideActionWidget)
  (bind _characterbattleslotreference (Variables|/Game/Custom/Components/AC_CharacterBattleStats.AC_CharacterBattleStats_C|GetCharacterBattleSlotReference (Variables|/Game/Custom/BP_BaseRPGCharacter.BP_BaseRPGCharacter_C|GetAC_CharacterBattleStats (Variables|BattleInProgress|GetCurrentCharacter)))
    (:then
      (Default|UnHighlightSlot _characterbattleslotreference)
      (Variables|/Script/UMG.WidgetSwitcher|SetActiveWidgetIndex (Variables|/Game/Custom/Widgets/BattleWidgets/Widget_ActionsPanel.Widget_ActionsPanel_C|GetWidgetSwitcher_Actions (Variables|/Game/Custom/Widgets/BattleWidgets/Widget_BattleInterface.Widget_BattleInterface_C|GetWidget_ActionsPanel (Variables|Widgets|GetBattleInterfaceReference))) 0))
    (:else
      _))
  (if (== (Utilities|Array|Length (Variables|BattleInProgress|TurnOrder|GetTurnOrder)) 0)
    (BattleInProgress|Functionality|TurnStart|GetTurnOrder)
    (else
      (BattleInProgress|Functionality|TurnStart|GetNextCharacter))))

(fn GoBacktoWorldMap
  (bind _playercharacter (Variables|BattleInProgress|GetPlayerCharacter))
  (bind _ac_characterbattlestats (Variables|/Game/Custom/BP_BaseRPGCharacter.BP_BaseRPGCharacter_C|GetAC_CharacterBattleStats _playercharacter))
  (bind _characterhardcodedname (Variables|/Game/Custom/Components/AC_CharacterBattleStats.AC_CharacterBattleStats_C|GetCharacterHardcodedName _ac_characterbattlestats))
  ;[0.15 0.15 0.15 0.5] Save character status after battle
  (bind _structout (Utilities|Struct|SetmembersinS_Character (.Value (Utilities|Map|Find (Variables|/Game/Custom/GI_RPG.GI_RPG_C|GetCharacterCollection (Variables|Default|GetGameInstanceReference)) _characterhardcodedname)) (Variables|/Game/Custom/Components/AC_CharacterBattleStats.AC_CharacterBattleStats_C|GetCurrentHP _ac_characterbattlestats) (Variables|/Game/Custom/Components/AC_CharacterBattleStats.AC_CharacterBattleStats_C|GetCurrentMP _ac_characterbattlestats)))
  (Utilities|Map|Add (Variables|/Game/Custom/GI_RPG.GI_RPG_C|GetCharacterCollection (Variables|Default|GetGameInstanceReference)) _characterhardcodedname _structout)
  (Variables|/Game/Custom/GI_RPG.GI_RPG_C|SetSpawningAfterBattle (Variables|Default|GetGameInstanceReference) true))

(fn CreateBattleInterface
  (bind _returnvalue (UserInterface|CreateWidget "/Game/Custom/Widgets/BattleWidgets/Widget_BattleInterface.Widget_BattleInterface_C"))
  (bind _output_get (Variables|Widgets|SetBattleInterfaceReference _returnvalue))
  (UserInterface|Viewport|AddtoViewport _output_get 0)
  (for _array_element (Variables|/Game/Custom/Widgets/BattleWidgets/Widget_ActionsPanel.Widget_ActionsPanel_C|GetActionSlotReferences (Variables|/Game/Custom/Widgets/BattleWidgets/Widget_BattleInterface.Widget_BattleInterface_C|GetWidget_ActionsPanel (Variables|Widgets|GetBattleInterfaceReference)))
    (Variables|/Game/Custom/Widgets/BattleWidgets/Widget_ActionSlot.Widget_ActionSlot_C|SetBattleManagerReference _array_element self)))

(fn GetAllPasta
  (params (Pasta :type Array%20of%20S%20Pasta%20Structures))
  (for _array_element Pasta
    (if (.CanBeUsedInBattle (Utilities|Struct|BreakS_Pasta _array_element))
      (if (not (Utilities|Array|ContainsItem (LocalVariables|GetAlreadyAddedPasta) (.PastaHardCodedName (Utilities|Struct|BreakS_Pasta _array_element))))
        (Utilities|Array|Add (LocalVariables|GetAlreadyAddedPasta) (.PastaHardCodedName (Utilities|Struct|BreakS_Pasta _array_element)))
        (bind _totalamountowned (Default|CheckAmoutOfPastaType (Actor|GetComponentbyClass (Components|GetOwner) "/Game/Custom/Components/AC_InventoryManager.AC_InventoryManager_C") (.PastaHardCodedName (Utilities|Struct|BreakS_Pasta _array_element))))
        (bind _structout (Utilities|Struct|SetmembersinS_Pasta _array_element _totalamountowned))
        (Utilities|Array|Add (LocalVariables|GetUsablePasta) _structout))))
  (return (LocalVariables|GetUsablePasta)))