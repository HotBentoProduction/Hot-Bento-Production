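; Actor component that manages target selection for RPG battles, covering both character targeting and pan placement.
; It switches modes by toggling collision on all enemies and enemy spots, keeping only hidden-cell spots collidable during character targeting.
; Target pointers are shown by targeting type (self, single enemy, all enemies) and tracked for later hiding.
; Cancelling resets targeting flags, clears the Battle Manager tooltip and, mid-turn, has the Action Manager destroy the reference pan.
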(event EventBeginPlay
  (bind _asgi_rpg (Utilities|Casting|CastToGI_RPG (Game|GetGameInstance) :!label _label)
    (:then
      (Variables|Default|SetGameInstanceReference _asgi_rpg))
    (:CastFailed
      (Utilities|FlowControl|Delay 0.1)
      (goto _label))))

(fn EnableTargeting
  (params (CanTargetSelf :type Boolean) (TargetingType :type E_TargetingType%20Enum :default "NewEnumerator0"))
  (Variables|Targeting|SetCanTargetSelf CanTargetSelf)
  (Variables|Targeting|SetSelectedTargetingType TargetingType)
  (Variables|Targeting|SetIsTargetingEnabled true)
  (bind _outactors (Actor|GetAllActorsOfClass "/Game/Custom/Enemy/BP_BaseEnemy.BP_BaseEnemy_C"))
  (for _array_element _outactors
    (Collision|SetActorEnableCollision _array_element true))
  (bind _outactors_2 (Actor|GetAllActorsOfClass "/Game/Custom/BP_EnemySpot.BP_EnemySpot_C"))
  (for _array_element_2 _outactors_2
    (if (Variables|/Game/Custom/BP_EnemySpot.BP_EnemySpot_C|GetisCellHidden _array_element_2)
      (Collision|SetActorEnableCollision _array_element_2 true)
      (else
        (Collision|SetActorEnableCollision _array_element_2 false)))))

(fn DisableTargeting
  (Variables|Targeting|SetIsTargetingEnabled false)
  (CallFunction|CancelTargeting false))

(fn ShowTargets
  (params (IndicatedTarget :type BP%20Base%20Enemy%20Object%20Reference))
  (LocalVariables|SetIndicatedTargetLocal IndicatedTarget)
  (switch Utilities|FlowControl|Switch|SwitchonE_TargetingType (Variables|Targeting|GetSelectedTargetingType)
    (:NewEnumerator0
      (if (== (Variables|/Game/Custom/Components/AC_BattleManager.AC_BattleManager_C|GetCurrentCharacter (Variables|/Game/Custom/BP_BaseRPGCharacter.BP_BaseRPGCharacter_C|GetBattleManagerReferences (LocalVariables|GetIndicatedTargetLocal))) (LocalVariables|GetIndicatedTargetLocal))
        (Development|SetHiddeninGame (Variables|/Game/Custom/BP_BaseRPGCharacter.BP_BaseRPGCharacter_C|GetTargetPointer (LocalVariables|GetIndicatedTargetLocal)) false false)
        (Utilities|Array|Add (Variables|Targeting|GetTargetedCharacters) (LocalVariables|GetIndicatedTargetLocal))))
    (:NewEnumerator1
      (if (Variables|/Game/Custom/BP_BaseRPGCharacter.BP_BaseRPGCharacter_C|GetEnemy (LocalVariables|GetIndicatedTargetLocal))
        (Development|SetHiddeninGame (Variables|/Game/Custom/BP_BaseRPGCharacter.BP_BaseRPGCharacter_C|GetTargetPointer (LocalVariables|GetIndicatedTargetLocal)) false false)
        (Utilities|Array|Add (Variables|Targeting|GetTargetedCharacters) (LocalVariables|GetIndicatedTargetLocal))))
    (:NewEnumerator2
      (if (Variables|/Game/Custom/BP_BaseRPGCharacter.BP_BaseRPGCharacter_C|GetEnemy (LocalVariables|GetIndicatedTargetLocal))
        (for _array_element (Variables|/Game/Custom/Components/AC_BattleManager.AC_BattleManager_C|GetEnemies (Variables|/Game/Custom/BP_BaseRPGCharacter.BP_BaseRPGCharacter_C|GetBattleManagerReferences (LocalVariables|GetIndicatedTargetLocal)))
          (Development|SetHiddeninGame (Variables|/Game/Custom/BP_BaseRPGCharacter.BP_BaseRPGCharacter_C|GetTargetPointer _array_element) false false)
          (Utilities|Array|Add (Variables|Targeting|GetTargetedCharacters) _array_element))))))

(fn HideTargets
  (for _array_element (Variables|Targeting|GetTargetedCharacters)
    (Development|SetHiddeninGame (Variables|/Game/Custom/BP_BaseRPGCharacter.BP_BaseRPGCharacter_C|GetTargetPointer _array_element) true false))
  (Utilities|Array|Clear (Variables|Targeting|GetTargetedCharacters)))

(fn CancelTargeting
  (params (DuringTurn :type Boolean))
  (Default|ShowBattleToolTip (Actor|GetComponentbyClass (Components|GetOwner) "/Game/Custom/Components/AC_BattleManager.AC_BattleManager_C"))
  (Variables|Targeting|SetIsTargetingEnabled false)
  (Variables|TargetingPan|SetisPanTargetingEnable false)
  (Variables|TargetingPan|SetAbleToPickUpPans false)
  (Variables|TargetingPan|SetCanPanBePlacedDown false)
  (if DuringTurn
    (Default|DestroyReferencePan (Actor|GetComponentbyClass (Components|GetOwner) "/Game/Custom/Components/AC_ActionManager.AC_ActionManager_C"))))

(fn EnablePanTargeting
  (params (isSpecialPan :type Boolean) (SpecialPanPosition :type Array%20of%20Integers))
  (Variables|TargetingPan|SetisPanTargetingEnable true)
  (Variables|TargetingPan|SetSpecialPanPosition SpecialPanPosition)
  (bind _outactors (Actor|GetAllActorsOfClass "/Game/Custom/Enemy/BP_BaseEnemy.BP_BaseEnemy_C"))
  (for _array_element _outactors
    (Collision|SetActorEnableCollision _array_element false))
  (bind _outactors_2 (Actor|GetAllActorsOfClass "/Game/Custom/BP_EnemySpot.BP_EnemySpot_C"))
  (for _array_element_2 _outactors_2
    (Collision|SetActorEnableCollision _array_element_2 true)))

(fn EnablePanCollision
  (bind _outactors (Actor|GetAllActorsOfClass "/Game/Custom/Enemy/BP_BaseEnemy.BP_BaseEnemy_C"))
  (for _array_element _outactors
    (Collision|SetActorEnableCollision _array_element false))
  (bind _outactors_2 (Actor|GetAllActorsOfClass "/Game/Custom/BP_EnemySpot.BP_EnemySpot_C"))
  (for _array_element_2 _outactors_2
    (Collision|SetActorEnableCollision _array_element_2 true)))