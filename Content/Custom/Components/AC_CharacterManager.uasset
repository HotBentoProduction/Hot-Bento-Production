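; AC_CharacterManager is a component that manages the RPG's character collection stored in GI_RPG.
; On BeginPlay it caches the game instance, retrying the cast after a short delay until it succeeds.
; RestoreHP writes back clamped HP, and AddNewCharacterToCollection adds characters by hardcoded name while below the collection limit.
; The remaining functions, covering screens, stats, leveling, MP and actions, are empty stubs.
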(event EventBeginPlay
  (bind _asgi_rpg (Utilities|Casting|CastToGI_RPG (Game|GetGameInstance) :!label _label)
    (:then
      (Variables|Default|SetGameInstanceReference _asgi_rpg))
    (:CastFailed
      (Utilities|FlowControl|Delay 0.1)
      (goto _label))))

(fn CreateReferencetoCharacterOverviewScreen)

(fn CreateReferencetoCharacterSelectionScreen)

(fn CreateReferencetoActionsScreen)

(fn RefreshCharacterOverviewSlots)

(fn IncreaseCharacterStats)

(fn DecreaseCharacterStats)

(fn RestoreHP
  (params (CharacterHardcodedName :type Name) (HPAmount :type Float%20%28double-precision%29))
  (bind _gameinstancereference (Variables|Default|GetGameInstanceReference))
  (bind _charactercollection (Variables|/Game/Custom/GI_RPG.GI_RPG_C|GetCharacterCollection _gameinstancereference))
  (bind _value (Utilities|Map|Find _charactercollection CharacterHardcodedName))
  (bind (_characterhardcodedname _characterdisplayname _currentlevel _currentexperience _availableactionpoints _characteractorclass _charactericon _currenthp _currentmp _characterstats) (Utilities|Struct|BreakS_Character _value))
  (bind _structout (Utilities|Struct|SetmembersinS_Character _value (Math|Float|Clamp(Float) (+ _currenthp HPAmount) 0.0 (.Value (Utilities|Map|Find _characterstats "NewEnumerator1")))))
  (Utilities|Map|Add (Variables|/Game/Custom/GI_RPG.GI_RPG_C|GetCharacterCollection (Variables|Default|GetGameInstanceReference)) CharacterHardcodedName _structout))

(fn RestoreMP)

(fn AddNewCharactertoCollection
  (params (CharacterStruct :type S%20Character%20Structure))
  (LocalVariables|SetCharacterStructLocal CharacterStruct)
  (if (< (Utilities|Map|Length (Variables|/Game/Custom/GI_RPG.GI_RPG_C|GetCharacterCollection (Variables|Default|GetGameInstanceReference))) (Variables|Setup|GetMaxAmountInCollection))
    (Utilities|Map|Add (Variables|/Game/Custom/GI_RPG.GI_RPG_C|GetCharacterCollection (Variables|Default|GetGameInstanceReference)) (.CharacterHardCodedname (Utilities|Struct|BreakS_Character (LocalVariables|GetCharacterStructLocal))) (LocalVariables|GetCharacterStructLocal))))

(fn ShowStatsComparison)

(fn HideStatsComparison)

(fn RefreshSelectedCharacterData)

(fn LevelUpCharacter)

(fn AddExperiencetoCharacter)

(fn RefreshSelectedCharacterActionsData)

(fn GetProperActionSlot)

(fn RefreshSelectedActionData)

(fn RefreshCharactersSlotsinActionScreen)

(fn UpgradeAction)

(fn DegradeAction)

(fn ForgetAction)

(fn ReceiveActionPoints)

(fn DeductActionPoints)

(fn LearnNewAction)