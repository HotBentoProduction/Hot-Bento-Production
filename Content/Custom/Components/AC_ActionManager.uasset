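; Battle action component for a cooking-themed turn-based RPG that selects and executes attacks, defend, items, abilities, fleeing, pans and sauce jars.
; Selection drives the targeting and battle managers; activation applies results to targeted characters' battle stats.
; Attacks and sauce jars poll QTE widgets each tick, then derive damage from cook-panel or recipe ingredients via data tables.
; Ingredient effects are only tallied and printed; several potion, ability and DIY-recipe handlers are empty.
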(event EventBeginPlay
  (bind _asgi_rpg (Utilities|Casting|CastToGI_RPG (Game|GetGameInstance) :!label _label)
    (:then
      (Variables|Default|SetGameInstanceReference _asgi_rpg))
    (:CastFailed
      (Utilities|FlowControl|Delay 0.1)
      (goto _label))))

(event Custom|SelectAction
  (params (ActionType :type E_ActionType%20Enum :default "NewEnumerator0") (SecondaryActionName :type Name))
  (bind _currentcharacter (Utilities|GetCurrentCharacter))
  (bind _ac_characterbattlestats (Variables|/Game/Custom/BP_BaseRPGCharacter.BP_BaseRPGCharacter_C|GetAC_CharacterBattleStats _currentcharacter))
  (Variables|/Game/Custom/Components/AC_CharacterBattleStats.AC_CharacterBattleStats_C|SetSelectedActionType _ac_characterbattlestats ActionType)
  (Variables|/Game/Custom/Components/AC_CharacterBattleStats.AC_CharacterBattleStats_C|SetSelectedSecondaryAction _ac_characterbattlestats SecondaryActionName)
  (switch Utilities|FlowControl|Switch|SwitchonE_ActionType ActionType
    (:NewEnumerator1
      (Selection|SelectAttack :!label _label))
    (:NewEnumerator2
      (Selection|SelectDefend))
    (:NewEnumerator3
      (|SelectItem))
    (:NewEnumerator4
      (Selection|SelectFlee))
    (:NewEnumerator6
      (|SelectAbility))
    (:NewEnumerator9
      (Selection|SelectPan (Utilities|String|ToString(Name) SecondaryActionName)))
    (:NewEnumerator10
      (goto _label))))

(event Custom|ActivateActionEvent
  (params (SelectedAction :type E_ActionType%20Enum :default "NewEnumerator0") (SecondaryActionName :type Name))
  (bind _currentcharacter (Utilities|GetCurrentCharacter))
  (bind _ac_characterbattlestats (Variables|/Game/Custom/BP_BaseRPGCharacter.BP_BaseRPGCharacter_C|GetAC_CharacterBattleStats _currentcharacter))
  (Variables|/Game/Custom/Components/AC_CharacterBattleStats.AC_CharacterBattleStats_C|SetSelectedActionType _ac_characterbattlestats SelectedAction)
  (Variables|/Game/Custom/Components/AC_CharacterBattleStats.AC_CharacterBattleStats_C|SetSelectedSecondaryAction _ac_characterbattlestats SecondaryActionName)
  (switch Utilities|FlowControl|Switch|SwitchonE_ActionType SelectedAction
    (:NewEnumerator1
      ;[0.15 0.15 0.15 0.5] Check QTE event have succes or not
      (bind _foundwidgets (Widget|GetAllWidgetsOfClass "/Game/Custom/Widgets/BattleWidgets/Tap_Key_UI.Tap_Key_UI_C" false :!label _label))
      (if (Variables|/Game/Custom/Widgets/BattleWidgets/Tap_Key_UI.Tap_Key_UI_C|GetGo%20next%20frame (Utilities|Array|Get(acopy) _foundwidgets (Variables|Default|GetStart%20Check%20Index)))
        (if (not (Variables|/Game/Custom/Widgets/BattleWidgets/Tap_Key_UI.Tap_Key_UI_C|GetIsFail? (Utilities|Array|Get(acopy) _foundwidgets (Variables|Default|GetStart%20Check%20Index))))
          ;[0.15 0.15 0.15 0.5] Select Target and Calculate DMG
          (Activation|ActivateAttack))
        (else
          (Utilities|FlowControl|DelayUntilNextTick)
          (goto _label))))
    (:NewEnumerator2
      (Activation|ActivateDefend))
    (:NewEnumerator3
      (|ActivateItem))
    (:NewEnumerator4
      (Selection|SelectFlee))
    (:NewEnumerator6
      (|ActivateAbilityCopy))
    (:NewEnumerator8
      ;[0.15 0.15 0.15 0.5] Check QTE event have succes or not
      (bind _foundwidgets_2 (Widget|GetAllWidgetsOfClass "/Game/Custom/Widgets/BattleWidgets/Tap_Key_UI.Tap_Key_UI_C" false :!label _label_2))
      (if (Variables|/Game/Custom/Widgets/BattleWidgets/Tap_Key_UI.Tap_Key_UI_C|GetGo%20next%20frame (Utilities|Array|Get(acopy) _foundwidgets_2 (Variables|Default|GetStart%20Check%20Index)))
        (if (not (Variables|/Game/Custom/Widgets/BattleWidgets/Tap_Key_UI.Tap_Key_UI_C|GetIsFail? (Utilities|Array|Get(acopy) _foundwidgets_2 (Variables|Default|GetStart%20Check%20Index))))
          (|ActivatePastaGraph))
        (else
          (Utilities|FlowControl|DelayUntilNextTick)
          (goto _label_2))))
    (:NewEnumerator10
      (goto _label))))

(fn SelectItemMPPotion01)

(fn SelectItemMPPotion02)

(fn SelectItemHPPotion01
  (Default|ShowBattleToolTip (Utilities|GetBattleManager) "Select Target")
  (Default|EnableTargeting (Utilities|GetTargetingManager) false "NewEnumerator0"))

(fn SelectItemHPPotion02)

(fn SelectAbilityAOE
  (Default|ShowBattleToolTip (Utilities|GetBattleManager) "Select Target")
  (Default|EnableTargeting (Utilities|GetTargetingManager) false "NewEnumerator2"))

(fn SelectAbilityDOT)

(fn SelectAttack
  (Default|ShowBattleToolTip (Utilities|GetBattleManager) "Select Target")
  (Default|EnableTargeting (Utilities|GetTargetingManager) false "NewEnumerator1"))

(fn SelectDefend
  (Default|DisableTargetingandInput (Utilities|GetBattleManager))
  (Activation|ActivateDefend))

(fn SelectFlee
  (Activation|ActivateFlee))

(fn ActivateItemMPPotion01)

(fn ActivateItemMPPotion02)

(fn ActivateItemHPPotion01
  (for _array_element (Variables|/Game/Custom/Components/AC_CharacterBattleStats.AC_CharacterBattleStats_C|GetTargetedCharacters (Variables|/Game/Custom/BP_BaseRPGCharacter.BP_BaseRPGCharacter_C|GetAC_CharacterBattleStats (Utilities|GetCurrentCharacter)))
    (Default|RecoverHP (Variables|/Game/Custom/BP_BaseRPGCharacter.BP_BaseRPGCharacter_C|GetAC_CharacterBattleStats _array_element) 3e+01)))

(fn ActivateItemHPPotion02)

(fn ActivateAbilityAOE
  (bind _currentcharacter (Utilities|GetCurrentCharacter))
  (bind _ac_characterbattlestats (Variables|/Game/Custom/BP_BaseRPGCharacter.BP_BaseRPGCharacter_C|GetAC_CharacterBattleStats _currentcharacter))
  (bind _characterstats (Variables|/Game/Custom/Components/AC_CharacterBattleStats.AC_CharacterBattleStats_C|GetCharacterStats _ac_characterbattlestats))
  (for _array_element (Variables|/Game/Custom/Components/AC_CharacterBattleStats.AC_CharacterBattleStats_C|GetTargetedCharacters (Variables|/Game/Custom/BP_BaseRPGCharacter.BP_BaseRPGCharacter_C|GetAC_CharacterBattleStats (Utilities|GetCurrentCharacter)))
    (Default|ReceiveDamage (Variables|/Game/Custom/BP_BaseRPGCharacter.BP_BaseRPGCharacter_C|GetAC_CharacterBattleStats _array_element) (.Value (Utilities|Map|Find _characterstats "NewEnumerator3")) (.Value (Utilities|Map|Find _characterstats "NewEnumerator5")) (.Value (Utilities|Map|Find _characterstats "NewEnumerator6")))))

(fn ActivateAbilityDOT)

(fn ActivateAttack
  (Activation|ActivateNonRecipeIngredients)
  (Default|RecoverPasta (Variables|/Game/Custom/BP_BaseRPGCharacter.BP_BaseRPGCharacter_C|GetAC_CharacterBattleStats (Utilities|GetCurrentCharacter)) 2)
  (Default|ShowBattleToolTip (Utilities|GetBattleManager) "You recovered 2 pasta")
  (for _array_element (Variables|/Game/Custom/Components/AC_CharacterBattleStats.AC_CharacterBattleStats_C|GetTargetedCharacters (Variables|/Game/Custom/BP_BaseRPGCharacter.BP_BaseRPGCharacter_C|GetAC_CharacterBattleStats (Utilities|GetCurrentCharacter)))
    (bind _foundwidgets (Widget|GetAllWidgetsOfClass "/Game/Custom/Widgets/BattleWidgets/Widget_Cook_Panel.Widget_Cook_Panel_C" false))
    (for _array_element_2 _foundwidgets
      (bind _keys (Utilities|Map|Keys (Variables|/Game/Custom/Widgets/BattleWidgets/Widget_Cook_Panel.Widget_Cook_Panel_C|GetInUseIngridients _array_element_2)))
      (for _array_element_3 _keys
        (bind _returnvalue (Utilities|GetDataTableRow "/Game/Custom/DataTables/DT_Ingridients.DT_Ingridients" (Utilities|String|StringToName (Utilities|String|EnumtoString _array_element_3)))
          (:then
            (LocalVariables|SetlocalDamage (+ (LocalVariables|GetlocalDamage) (* (.Value (Utilities|Map|Find (Variables|/Game/Custom/Widgets/BattleWidgets/Widget_Cook_Panel.Widget_Cook_Panel_C|GetInUseIngridients _array_element_2) _array_element_3)) (.Dmg_Modifier (Utilities|Struct|BreakS_Ingridient _returnvalue)))))))))
    (Default|ReceiveDamage (Variables|/Game/Custom/BP_BaseRPGCharacter.BP_BaseRPGCharacter_C|GetAC_CharacterBattleStats _array_element) (+ -5.0 (LocalVariables|GetlocalDamage)) 0.0 0.0)))

(fn ActivateDefend
  (Default|ShowBattleToolTip (Utilities|GetBattleManager) (Utilities|Text|FormatText "{Character} is defending" (.Name (Utilities|GetCurrentCharacterName))))
  (Variables|/Game/Custom/Components/AC_CharacterBattleStats.AC_CharacterBattleStats_C|SetDefending (Variables|/Game/Custom/BP_BaseRPGCharacter.BP_BaseRPGCharacter_C|GetAC_CharacterBattleStats (Utilities|GetCurrentCharacter)) true)
  (Default|EndCharacterTurn (Utilities|GetBattleManager)))

(fn ActivateFlee
  (bind _asgi_rpg (Utilities|Casting|CastToGI_RPG (Game|GetGameInstance)))
  (Game|OpenLevel(byName) (Variables|/Game/Custom/GI_RPG.GI_RPG_C|GetMapName _asgi_rpg)))

(fn GetActionCost
  (params (ActionName :type Name))
  (bind _hardcodedname (Utilities|GetCurrentCharacterName))
  (bind _gameinstancereference (Variables|Default|GetGameInstanceReference))
  (bind _charactercollection (Variables|/Game/Custom/GI_RPG.GI_RPG_C|GetCharacterCollection _gameinstancereference))
  (bind _value (Utilities|Map|Find _charactercollection _hardcodedname))
  (bind _characteractions (Utilities|Struct|BreakS_Character _value))
  (bind _value_2 (Utilities|Map|Find _characteractions ActionName))
  (bind _returnvalue (Utilities|GetDataTableRow "/Game/Custom/DataTables/DT_Actions.DT_Actions" ActionName)
    (:then
      (return (+ (.BaseHPCost (Utilities|Struct|BreakS_Actions _returnvalue)) (* _value_2 (.PerLevelHPCost (Utilities|Struct|BreakS_Actions _returnvalue)))) (+ (.BaseMPCost (Utilities|Struct|BreakS_Actions _returnvalue)) (* _value_2 (.PerLevelMPCost (Utilities|Struct|BreakS_Actions _returnvalue))))))))

(fn SelectPasta
  (bind _battlemanager (Utilities|GetBattleManager))
  (bind _battleinterfacereference (Variables|/Game/Custom/Components/AC_BattleManager.AC_BattleManager_C|GetBattleInterfaceReference _battlemanager))
  (bind _widget_recipeselection (Variables|/Game/Custom/Widgets/BattleWidgets/Widget_BattleInterface.Widget_BattleInterface_C|GetWidget_RecipeSelection _battleinterfacereference))
  (Default|RefreshRecipes _widget_recipeselection)
  (Widget|SetVisibility _widget_recipeselection "Visible"))

(fn SelectPan
  (params (SelectedPan :type String))
  (CallFunction|DestroyReferencePan)
  (Variables|Default|SetSelectedPan (Utilities|String|StringToName SelectedPan))
  (bind _returnvalue (Utilities|GetDataTableRow "/Game/Custom/DataTables/DT_Pans.DT_Pans" (Utilities|String|StringToName SelectedPan))
    (:then
      (Default|EnablePanTargeting (Utilities|GetTargetingManager) false (.PanPosition (Utilities|Struct|BreakS_Pan _returnvalue)))
      (bind _returnvalue_2 (Game|SpawnActorfromClass (.Model (Utilities|Struct|BreakS_Pan _returnvalue)) (LocalVariables|GetZero) "Undefined" "MultiplyWithRoot" 0 0))
      (bind _asbasic_pan (Utilities|Casting|CastToBasicPan _returnvalue_2))
      (Utilities|Map|Add (Variables|Default|GetPanActorReference) (Variables|Default|GetSelectedPan) _asbasic_pan))))

(fn SelectRecipe
  (Default|ShowBattleToolTip (Utilities|GetBattleManager) "Select Target")
  (LocalVariables|SetisAoe false)
  (LocalVariables|SetisSelf false)
  (LocalVariables|SetisSingle false)
  (Default|EnableTargeting (Utilities|GetTargetingManager) false "NewEnumerator1"))

(fn ActivateRecipe
  (params (PastaName :type Name))
  (if (!= PastaName "DIY")
    (Activation|ActivateIngridientsEffect PastaName)
    (Activation|ActivatePasta PastaName "None")
    (else
      (Activation|ActivateDIYEffects)
      (Activation|ActivateDIYRecipe))))

(fn ActivateIngridientsEffect
  (params (PastaName :type Name))
  (LocalVariables|SetpushCounter 0)
  (LocalVariables|SettimeCounter 0)
  (LocalVariables|SetSleepCounter 0)
  (bind _returnvalue (Utilities|GetDataTableRow "/Game/Custom/DataTables/DT_recipes.DT_recipes" PastaName)
    (:then
      (bind _keys (Utilities|Map|Keys (.Ingridients (Utilities|Struct|BreakS_Recipes _returnvalue))))
      (for _array_element _keys
        (bind _returnvalue_2 (Utilities|GetDataTableRow "/Game/Custom/DataTables/DT_Ingridients.DT_Ingridients" (Utilities|String|StringToName (Utilities|String|EnumtoString _array_element)))
          (:then
            (switch Utilities|FlowControl|Switch|SwitchonE_IngridientEffect (.Effect (Utilities|Struct|BreakS_Ingridient _returnvalue_2))
              (:NewEnumerator2
                (LocalVariables|SetpushCounter (* (.Value (Utilities|Map|Find (.Ingridients (Utilities|Struct|BreakS_Recipes _returnvalue)) _array_element)) (+ (LocalVariables|GetpushCounter) 1))))
              (:NewEnumerator3
                (LocalVariables|SettimeCounter (* (.Value (Utilities|Map|Find (.Ingridients (Utilities|Struct|BreakS_Recipes _returnvalue)) _array_element)) (+ (LocalVariables|GettimeCounter) 1))))
              (:NewEnumerator4
                (LocalVariables|SetsleepCounter (* (.Value (Utilities|Map|Find (.Ingridients (Utilities|Struct|BreakS_Recipes _returnvalue)) _array_element)) (+ (LocalVariables|GetsleepCounter) 1))))))))
      (Development|PrintString (Utilities|String|Append "Push" ":" (Utilities|String|ToString(Integer) (LocalVariables|GetpushCounter)) "-" "Time Reduce" ":" (Utilities|String|ToString(Integer) (LocalVariables|GettimeCounter)) "-" "Sleep" ":" (Utilities|String|ToString(Integer) (LocalVariables|GetSleepCounter))) true true "(R=1.000000,G=0.327564,B=0.000000,A=1.000000)" 5.0))))

(fn ActivateDIYEffects
  (LocalVariables|SetpushCounter 0)
  (LocalVariables|SettimeCounter 0)
  (LocalVariables|SetsleepCounter 0)
  (bind _returnvalue (SaveGame|LoadGamefromSlot "Inventory"))
  (bind _asinventory (Utilities|Casting|CastToInventory _returnvalue))
  (bind _keys (Utilities|Map|Keys (.IngridientsMap (Utilities|Struct|BreakS_SauceJar (.Value (Utilities|Map|Find (Variables|/Game/Custom/SaveGame/Inventory.Inventory_C|GetSauceJars _asinventory) (Variables|Default|GetChosenSauceJar)))))))
  (for _array_element _keys
    (bind _returnvalue_2 (Utilities|GetDataTableRow "/Game/Custom/DataTables/DT_Ingridients.DT_Ingridients" (Utilities|String|StringToName (Utilities|String|EnumtoString _array_element)))
      (:then
        (switch Utilities|FlowControl|Switch|SwitchonE_IngridientEffect (.Effect (Utilities|Struct|BreakS_Ingridient _returnvalue_2))
          (:NewEnumerator2
            (LocalVariables|SetpushCounter (* (.Value (Utilities|Map|Find (.IngridientsMap (Utilities|Struct|BreakS_SauceJar (.Value (Utilities|Map|Find (Variables|/Game/Custom/SaveGame/Inventory.Inventory_C|GetSauceJars _asinventory) (Variables|Default|GetChosenSauceJar))))) _array_element)) (+ (LocalVariables|GetpushCounter) 1))))
          (:NewEnumerator3
            (LocalVariables|SettimeCounter (* (.Value (Utilities|Map|Find (.IngridientsMap (Utilities|Struct|BreakS_SauceJar (.Value (Utilities|Map|Find (Variables|/Game/Custom/SaveGame/Inventory.Inventory_C|GetSauceJars _asinventory) (Variables|Default|GetChosenSauceJar))))) _array_element)) (+ (LocalVariables|GettimeCounter) 1))))
          (:NewEnumerator4
            (LocalVariables|SetsleepCounter (* (.Value (Utilities|Map|Find (.IngridientsMap (Utilities|Struct|BreakS_SauceJar (.Value (Utilities|Map|Find (Variables|/Game/Custom/SaveGame/Inventory.Inventory_C|GetSauceJars _asinventory) (Variables|Default|GetChosenSauceJar))))) _array_element)) (+ (LocalVariables|GetsleepCounter) 1))))))))
  (Development|PrintString (Utilities|String|Append "Push" ":" (Utilities|String|ToString(Integer) (LocalVariables|GetpushCounter)) "-" "Time Reduce" ":" (Utilities|String|ToString(Integer) (LocalVariables|GettimeCounter)) "-" "Sleep" ":" (Utilities|String|ToString(Integer) (LocalVariables|GetsleepCounter))) true true "(R=1.000000,G=0.327564,B=0.000000,A=1.000000)" 5.0))

(fn ActivateDIYRecipe)

(fn ActivateNonRecipeIngredients
  (LocalVariables|SetpushCounter 0)
  (LocalVariables|SettimeCounter 0)
  (LocalVariables|SetsleepCounter 0)
  (bind _foundwidgets (Widget|GetAllWidgetsOfClass "/Game/Custom/Widgets/BattleWidgets/Widget_Cook_Panel.Widget_Cook_Panel_C" false))
  (for _array_element _foundwidgets
    (bind _keys (Utilities|Map|Keys (Variables|/Game/Custom/Widgets/BattleWidgets/Widget_Cook_Panel.Widget_Cook_Panel_C|GetInUseIngridients _array_element)))
    (for _array_element_2 _keys
      (bind _returnvalue (Utilities|GetDataTableRow "/Game/Custom/DataTables/DT_Ingridients.DT_Ingridients" (Utilities|String|StringToName (Utilities|String|EnumtoString _array_element_2)))
        (:then
          (switch Utilities|FlowControl|Switch|SwitchonE_IngridientEffect (.Effect (Utilities|Struct|BreakS_Ingridient _returnvalue))
            (:NewEnumerator2
              (LocalVariables|SetpushCounter (* (+ (LocalVariables|GetpushCounter) 1) (.Value (Utilities|Map|Find (Variables|/Game/Custom/Widgets/BattleWidgets/Widget_Cook_Panel.Widget_Cook_Panel_C|GetInUseIngridients _array_element) _array_element_2)))))
            (:NewEnumerator3
              (LocalVariables|SettimeCounter (* (.Value (Utilities|Map|Find (Variables|/Game/Custom/Widgets/BattleWidgets/Widget_Cook_Panel.Widget_Cook_Panel_C|GetInUseIngridients _array_element) _array_element_2)) (+ (LocalVariables|GettimeCounter) 1))))
            (:NewEnumerator4
              (LocalVariables|SetsleepCounter (* (.Value (Utilities|Map|Find (Variables|/Game/Custom/Widgets/BattleWidgets/Widget_Cook_Panel.Widget_Cook_Panel_C|GetInUseIngridients _array_element) _array_element_2)) (+ (LocalVariables|GetsleepCounter) 1))))))))
    (Development|PrintString (Utilities|String|Append "Push" ":" (Utilities|String|ToString(Integer) (LocalVariables|GetpushCounter)) "-" "Time Reduce" ":" (Utilities|String|ToString(Integer) (LocalVariables|GettimeCounter)) "-" "Sleep" ":" (Utilities|String|ToString(Integer) (LocalVariables|GetsleepCounter))) true true "(R=1.000000,G=0.327564,B=0.000000,A=1.000000)" 5.0)))

(fn ActivatePasta
  (params (PastaName :type Name) (RecipeName :type Name))
  (LocalVariables|SetRecipeNameLocal PastaName)
  (for _array_element (Variables|/Game/Custom/Components/AC_CharacterBattleStats.AC_CharacterBattleStats_C|GetTargetedCharacters (Variables|/Game/Custom/BP_BaseRPGCharacter.BP_BaseRPGCharacter_C|GetAC_CharacterBattleStats (Utilities|GetCurrentCharacter)))
    ;[0.15 0.15 0.15 0.5] Get Pasta row from Table via name
    (bind _returnvalue (Utilities|GetDataTableRow "/Game/Custom/DataTables/DT_recipes.DT_recipes" PastaName)
      (:then
        ;[0.15 0.15 0.15 0.5] Add Pasta Attack Stat to the Player Attack
        (bind _keys (Utilities|Map|Keys (.Ingridients (Utilities|Struct|BreakS_Recipes _returnvalue))))
        (for _array_element_2 _keys
          (bind _returnvalue_2 (Utilities|GetDataTableRow "/Game/Custom/DataTables/DT_Ingridients.DT_Ingridients" (Utilities|String|StringToName (Utilities|String|EnumtoString _array_element_2)))
            (:then
              (Default|ReceiveDamage (Variables|/Game/Custom/BP_BaseRPGCharacter.BP_BaseRPGCharacter_C|GetAC_CharacterBattleStats _array_element) (* (+ 0.0 (.Dmg_Modifier (Utilities|Struct|BreakS_Ingridient _returnvalue_2))) (.Value (Utilities|Map|Find (.Ingridients (Utilities|Struct|BreakS_Recipes _returnvalue)) _array_element_2))) 0.0 0.0)))))))
  (Default|RemoveRecipeAfterAttack (Utilities|GetBattleManager) (Variables|Default|GetChosenRecipe)))

(fn GetPastaCost
  (params (PastaName :type Name))
  (bind _returnvalue (Utilities|GetDataTableRow "/Game/Custom/DataTables/DT_Pastas.DT_Pastas" PastaName)
    (:then
      (return (.PastaConsumptionCost (Utilities|Struct|BreakS_Pasta _returnvalue))))))

(fn DestroyReferencePan
  (bind _panactorreference (Variables|Default|GetPanActorReference))
  (bind _selectedpan (Variables|Default|GetSelectedPan))
  (bind (_value _returnvalue) (Utilities|Map|Find _panactorreference _selectedpan))
  (if _returnvalue
    (Actor|DestroyActor _value)))

(fn SelectQTE
  (params (Index :type Integer))
  (bind _returnvalue (Game|GetPlayerController 0))
  (bind _array (Utilities|Array|MakeArray "W" "A" "S" "D"))
  (bind _outitem (Utilities|Array|Random _array))
  (bind _aspc_rpg_battle (Utilities|Casting|CastToPC_RPG_Battle _returnvalue))
  (if (> Index (Variables|Default|GetLoop%20Index)) :!label _label ; Loop to get QTE UI
    (Utilities|Array|SetArrayElem (Variables|Default|GetQTETarget%20Array) (Variables|Default|GetLoop%20Index) _outitem true)
    (Default|QTEEvent _aspc_rpg_battle _outitem (Class|KismetInputLibrary|KeyGetDisplayName _outitem false) true (Variables|Default|GetQTEDuration) _returnvalue (Variables|Default|GetLoop%20Index) (Variables|Default|GetX))
    (Math|Integer|IncrementInt (Variables|Default|GetLoop%20Index)
      (:%20%20
        (Variables|Default|SetX (- (Variables|Default|GetX) 2.5e+02))
        (goto _label)))
    (else
      (Variables|Default|SetLoop%20Index 0)
      (Variables|Default|SetX 1.2e+03)
      (return _aspc_rpg_battle))))

(fn NewFunction
  (params (self2 :type Tap%20Key%20UI%20Object%20Reference))
  (return (Variables|/Game/Custom/Widgets/BattleWidgets/Tap_Key_UI.Tap_Key_UI_C|GetIsPressed? self2)))