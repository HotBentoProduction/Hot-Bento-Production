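; Base enemy for a cooking-themed, turn-based RPG battle on a five-wide grid of spots tracked in the GameInstance.
; Forced movement shifts it between spots, letting soiled enemies enter pans to cook.
; On its turn, it resolves sleep or runs its selected action: move, attack an adjacent pan, or attack.
; Betray sauce redirects attacks onto the lowest-HP enemy; movement, regeneration and cook-countdown functions are empty or disconnected here.
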(event OnBeginCursorOver(CapsuleComponent)
  (params (TouchedComponent :type Primitive%20Component%20Object%20Reference))
  (bind _targetingmanagerreference (Variables|Default|GetTargetingManagerReference)
    (:then
      (if (Variables|/Game/Custom/Components/AC_TargetingManager.AC_TargetingManager_C|GetIsTargetingEnabled _targetingmanagerreference)
        (Default|ShowTargets _targetingmanagerreference self)))
    (:else)))

(event OnEndCursorOver(CapsuleComponent)
  (params (TouchedComponent :type Primitive%20Component%20Object%20Reference))
  (bind _targetingmanagerreference (Variables|Default|GetTargetingManagerReference)
    (:then
      (if (Variables|/Game/Custom/Components/AC_TargetingManager.AC_TargetingManager_C|GetIsTargetingEnabled _targetingmanagerreference)
        (Default|HideTargets _targetingmanagerreference)))
    (:else)))

(event OnClicked(CapsuleComponent)
  (params (TouchedComponent :type Primitive%20Component%20Object%20Reference) (ButtonPressed :type Key%20Structure))
  (bind _targetingmanagerreference (Variables|Default|GetTargetingManagerReference)
    (:then
      (if (Variables|/Game/Custom/Components/AC_TargetingManager.AC_TargetingManager_C|GetIsTargetingEnabled _targetingmanagerreference)
        (if (Utilities|Array|ContainsItem (Variables|/Game/Custom/Components/AC_TargetingManager.AC_TargetingManager_C|GetTargetedCharacters _targetingmanagerreference) self)
          (bind _battlemanagerreferences (Variables|Default|GetBattleManagerReferences)
            (:then
              (Default|RequestActionExecution _battlemanagerreferences (Variables|/Game/Custom/Components/AC_TargetingManager.AC_TargetingManager_C|GetTargetedCharacters _targetingmanagerreference)))
            (:else)))))
    (:else)))

(event Custom|UpdateCookTime)

(event Custom|ForcedMovement
  (params (KeyUsed :type Key%20Structure :default "None"))
  (bind _gameinstanceref (Variables|Default|GetGameInstanceRef))
  (bind _enemyspotmap (Variables|/Game/Custom/GI_RPG.GI_RPG_C|GetEnemySpotMap _gameinstanceref))
  (if (<= (Variables|Default|GetcurrentIndex) 5)
    (Variables|Default|SetWasAboutToGameOver? true)
    (else
      (Variables|Default|SetWasAboutToGameOver? false)))
  (Variables|/Game/Custom/BP_EnemySpot.BP_EnemySpot_C|SetisOccupied (.Value (Utilities|Map|Find (Variables|/Game/Custom/GI_RPG.GI_RPG_C|GetEnemySpotMap (Variables|Default|GetGameInstanceRef)) (Variables|Default|GetcurrentIndex))) false)
  (Default|StopShowing (.Value (Utilities|Map|Find (Variables|/Game/Custom/GI_RPG.GI_RPG_C|GetEnemySpotMap (Variables|Default|GetGameInstanceRef)) (Variables|Default|GetcurrentIndex))))
  (Variables|/Game/Custom/BP_EnemySpot.BP_EnemySpot_C|SetisEnemySoiled (.Value (Utilities|Map|Find (Variables|/Game/Custom/GI_RPG.GI_RPG_C|GetEnemySpotMap (Variables|Default|GetGameInstanceRef)) (Variables|Default|GetcurrentIndex))) false)
  (if (== KeyUsed "Up")
    (if (.ReturnValue (Utilities|Map|Find _enemyspotmap (+ (Variables|Default|GetcurrentIndex) 5)))
      (if (or (not (Variables|/Game/Custom/BP_EnemySpot.BP_EnemySpot_C|GetisOccupied (.Value (Utilities|Map|Find _enemyspotmap (+ (Variables|Default|GetcurrentIndex) 5))))) (and (Variables|/Game/Custom/BP_EnemySpot.BP_EnemySpot_C|GetisOccupiedByPan (.Value (Utilities|Map|Find _enemyspotmap (+ (Variables|Default|GetcurrentIndex) 5)))) (Variables|Default|GetisSoiled)))
        (Transformation|SetActorLocation (Math|Vector|MakeVector (.X (Math|Vector|BreakVector (.location (Transformation|GetActorTransform (.Value (Utilities|Map|Find _enemyspotmap (+ (Variables|Default|GetcurrentIndex) 5))))))) (.Y (Math|Vector|BreakVector (.location (Transformation|GetActorTransform (.Value (Utilities|Map|Find _enemyspotmap (+ (Variables|Default|GetcurrentIndex) 5))))))) (.z (Transformation|GetActorLocation))) false false)
        (Variables|/Game/Custom/BP_EnemySpot.BP_EnemySpot_C|SetisOccupied (.Value (Utilities|Map|Find _enemyspotmap (+ (Variables|Default|GetcurrentIndex) 5))) true)
        (Variables|/Game/Custom/BP_EnemySpot.BP_EnemySpot_C|SetisEnemySoiled (.Value (Utilities|Map|Find _enemyspotmap (+ (Variables|Default|GetcurrentIndex) 5))) (Variables|Default|GetisSoiled))
        (Default|StopShowing (.Value (Utilities|Map|Find _enemyspotmap (+ (Variables|Default|GetcurrentIndex) 5))))
        (if (and (Variables|/Game/Custom/BP_EnemySpot.BP_EnemySpot_C|GetisOccupiedByPan (.Value (Utilities|Map|Find _enemyspotmap (+ (Variables|Default|GetcurrentIndex) 5)))) (Variables|Default|GetisSoiled))
          (Variables|Default|SetisGettingCooked true)
          (else
            (Variables|Default|SetisGettingCooked false)))
        (if (Variables|Default|GetWasAboutToGameOver?)
          (Utilities|Array|SetArrayElem (Variables|/Game/Custom/GI_RPG.GI_RPG_C|GetgameOver? (Variables|Default|GetGameInstanceRef)) (Variables|Default|GetcurrentIndex) false))
        (Variables|Default|SetcurrentIndex (+ (Variables|Default|GetcurrentIndex) 5))
        (else
          (Variables|Default|SetFailedSteps (+ (Variables|Default|GetFailedSteps) 1) :!label _label)))
      (else
        (goto _label)))
    (elif (== KeyUsed "Down")
      (if (.ReturnValue (Utilities|Map|Find _enemyspotmap (- (Variables|Default|GetcurrentIndex) 5)))
        (if (or (not (Variables|/Game/Custom/BP_EnemySpot.BP_EnemySpot_C|GetisOccupied (.Value (Utilities|Map|Find _enemyspotmap (- (Variables|Default|GetcurrentIndex) 5))))) (and (Variables|/Game/Custom/BP_EnemySpot.BP_EnemySpot_C|GetisOccupiedByPan (.Value (Utilities|Map|Find _enemyspotmap (- (Variables|Default|GetcurrentIndex) 5)))) (Variables|Default|GetisSoiled)))
          (Transformation|SetActorLocation (Math|Vector|MakeVector (.X (Math|Vector|BreakVector (.location (Transformation|GetActorTransform (.Value (Utilities|Map|Find _enemyspotmap (- (Variables|Default|GetcurrentIndex) 5))))))) (.Y (Math|Vector|BreakVector (.location (Transformation|GetActorTransform (.Value (Utilities|Map|Find _enemyspotmap (- (Variables|Default|GetcurrentIndex) 5))))))) (.z (Transformation|GetActorLocation))) false false)
          (Variables|/Game/Custom/BP_EnemySpot.BP_EnemySpot_C|SetisOccupied (.Value (Utilities|Map|Find _enemyspotmap (- (Variables|Default|GetcurrentIndex) 5))) true)
          (Variables|/Game/Custom/BP_EnemySpot.BP_EnemySpot_C|SetisEnemySoiled (.Value (Utilities|Map|Find _enemyspotmap (- (Variables|Default|GetcurrentIndex) 5))) (Variables|Default|GetisSoiled))
          (Default|StopShowing (.Value (Utilities|Map|Find _enemyspotmap (- (Variables|Default|GetcurrentIndex) 5))))
          (if (and (Variables|/Game/Custom/BP_EnemySpot.BP_EnemySpot_C|GetisOccupiedByPan (.Value (Utilities|Map|Find _enemyspotmap (- (Variables|Default|GetcurrentIndex) 5)))) (Variables|Default|GetisSoiled))
            (Variables|Default|SetisGettingCooked true)
            (else
              (Variables|Default|SetisGettingCooked false)))
          (Variables|Default|SetcurrentIndex (+ (Variables|Default|GetcurrentIndex) -5))
          (else
            (Variables|Default|SetFailedSteps (+ (Variables|Default|GetFailedSteps) 1) :!label _label_2)
            (Variables|/Game/Custom/BP_EnemySpot.BP_EnemySpot_C|SetisOccupied (.Value (Utilities|Map|Find (Variables|/Game/Custom/GI_RPG.GI_RPG_C|GetEnemySpotMap (Variables|Default|GetGameInstanceRef)) (Variables|Default|GetcurrentIndex))) true)
            (Default|StopShowing (.Value (Utilities|Map|Find (Variables|/Game/Custom/GI_RPG.GI_RPG_C|GetEnemySpotMap (Variables|Default|GetGameInstanceRef)) (Variables|Default|GetcurrentIndex))))
            (Variables|/Game/Custom/BP_EnemySpot.BP_EnemySpot_C|SetisEnemySoiled (.Value (Utilities|Map|Find (Variables|/Game/Custom/GI_RPG.GI_RPG_C|GetEnemySpotMap (Variables|Default|GetGameInstanceRef)) (Variables|Default|GetcurrentIndex))) (Variables|Default|GetisSoiled))))
        (else
          (goto _label_2)))
      (elif (== KeyUsed "Right")
        (if (and (!= (Math|Integer|%(Integer) (Variables|Default|GetcurrentIndex) 5) 0) (or (not (Variables|/Game/Custom/BP_EnemySpot.BP_EnemySpot_C|GetisOccupied (.Value (Utilities|Map|Find _enemyspotmap (+ (Variables|Default|GetcurrentIndex) 1))))) (and (Variables|/Game/Custom/BP_EnemySpot.BP_EnemySpot_C|GetisOccupiedByPan (.Value (Utilities|Map|Find _enemyspotmap (+ (Variables|Default|GetcurrentIndex) 1)))) (Variables|Default|GetisSoiled))))
          (Transformation|SetActorLocation (Math|Vector|MakeVector (.X (Math|Vector|BreakVector (.location (Transformation|GetActorTransform (.Value (Utilities|Map|Find _enemyspotmap (+ (Variables|Default|GetcurrentIndex) 1))))))) (.Y (Math|Vector|BreakVector (.location (Transformation|GetActorTransform (.Value (Utilities|Map|Find _enemyspotmap (+ (Variables|Default|GetcurrentIndex) 1))))))) (.z (Transformation|GetActorLocation))) false false)
          (Variables|/Game/Custom/BP_EnemySpot.BP_EnemySpot_C|SetisOccupied (.Value (Utilities|Map|Find _enemyspotmap (+ (Variables|Default|GetcurrentIndex) 1))) true)
          (Variables|/Game/Custom/BP_EnemySpot.BP_EnemySpot_C|SetisEnemySoiled (.Value (Utilities|Map|Find _enemyspotmap (+ (Variables|Default|GetcurrentIndex) 1))) (Variables|Default|GetisSoiled))
          (Default|StopShowing (.Value (Utilities|Map|Find _enemyspotmap (+ (Variables|Default|GetcurrentIndex) 1))))
          (if (and (Variables|/Game/Custom/BP_EnemySpot.BP_EnemySpot_C|GetisOccupiedByPan (.Value (Utilities|Map|Find _enemyspotmap (+ (Variables|Default|GetcurrentIndex) 1)))) (Variables|Default|GetisSoiled))
            (Variables|Default|SetisGettingCooked true)
            (else
              (Variables|Default|SetisGettingCooked false)))
          (Variables|Default|SetcurrentIndex (+ (Variables|Default|GetcurrentIndex) 1))
          (else
            (Variables|Default|SetFailedSteps (+ (Variables|Default|GetFailedSteps) 1))
            (Variables|/Game/Custom/BP_EnemySpot.BP_EnemySpot_C|SetisOccupied (.Value (Utilities|Map|Find (Variables|/Game/Custom/GI_RPG.GI_RPG_C|GetEnemySpotMap (Variables|Default|GetGameInstanceRef)) (Variables|Default|GetcurrentIndex))) true :!label _label_3)
            (Default|StopShowing (.Value (Utilities|Map|Find (Variables|/Game/Custom/GI_RPG.GI_RPG_C|GetEnemySpotMap (Variables|Default|GetGameInstanceRef)) (Variables|Default|GetcurrentIndex))))
            (Variables|/Game/Custom/BP_EnemySpot.BP_EnemySpot_C|SetisEnemySoiled (.Value (Utilities|Map|Find (Variables|/Game/Custom/GI_RPG.GI_RPG_C|GetEnemySpotMap (Variables|Default|GetGameInstanceRef)) (Variables|Default|GetcurrentIndex))) (Variables|Default|GetisSoiled))))
        (elif (== KeyUsed "Left")
          (if (and (!= (Math|Integer|%(Integer) (Variables|Default|GetcurrentIndex) 5) 1) (or (not (Variables|/Game/Custom/BP_EnemySpot.BP_EnemySpot_C|GetisOccupied (.Value (Utilities|Map|Find _enemyspotmap (- (Variables|Default|GetcurrentIndex) 1))))) (and (Variables|/Game/Custom/BP_EnemySpot.BP_EnemySpot_C|GetisOccupiedByPan (.Value (Utilities|Map|Find _enemyspotmap (- (Variables|Default|GetcurrentIndex) 1)))) (Variables|Default|GetisSoiled))))
            (Transformation|SetActorLocation (Math|Vector|MakeVector (.X (Math|Vector|BreakVector (.location (Transformation|GetActorTransform (.Value (Utilities|Map|Find _enemyspotmap (- (Variables|Default|GetcurrentIndex) 1))))))) (.Y (Math|Vector|BreakVector (.location (Transformation|GetActorTransform (.Value (Utilities|Map|Find _enemyspotmap (- (Variables|Default|GetcurrentIndex) 1))))))) (.z (Transformation|GetActorLocation))) false false)
            (Variables|/Game/Custom/BP_EnemySpot.BP_EnemySpot_C|SetisOccupied (.Value (Utilities|Map|Find _enemyspotmap (- (Variables|Default|GetcurrentIndex) 1))) true)
            (Variables|/Game/Custom/BP_EnemySpot.BP_EnemySpot_C|SetisEnemySoiled (.Value (Utilities|Map|Find _enemyspotmap (- (Variables|Default|GetcurrentIndex) 1))) (Variables|Default|GetisSoiled))
            (Default|StopShowing (.Value (Utilities|Map|Find _enemyspotmap (- (Variables|Default|GetcurrentIndex) 1))))
            (if (and (Variables|/Game/Custom/BP_EnemySpot.BP_EnemySpot_C|GetisOccupiedByPan (.Value (Utilities|Map|Find _enemyspotmap (- (Variables|Default|GetcurrentIndex) 1)))) (Variables|Default|GetisSoiled))
              (Variables|Default|SetisGettingCooked true)
              (else
                (Variables|Default|SetisGettingCooked false)))
            (Variables|Default|SetcurrentIndex (+ (Variables|Default|GetcurrentIndex) -1))
            (else
              (Variables|Default|SetFailedSteps (+ (Variables|Default|GetFailedSteps) 1))
              (goto _label_3))))))))

(event Custom|ForceActionTrigger
  (bind _targetingmanagerreference (Variables|Default|GetTargetingManagerReference)
    (:then
      (if (Variables|/Game/Custom/Components/AC_TargetingManager.AC_TargetingManager_C|GetIsTargetingEnabled _targetingmanagerreference)
        (if (Utilities|Array|ContainsItem (Variables|/Game/Custom/Components/AC_TargetingManager.AC_TargetingManager_C|GetTargetedCharacters _targetingmanagerreference) self)
          (bind _battlemanagerreferences (Variables|Default|GetBattleManagerReferences)
            (:then
              (Default|RequestActionExecution _battlemanagerreferences (Variables|/Game/Custom/Components/AC_TargetingManager.AC_TargetingManager_C|GetTargetedCharacters _targetingmanagerreference)))
            (:else)))))
    (:else)))

(event Custom|OnHitByBetraySauce
  (params (Amount :type Integer))
  (Variables|Default|SetbetrayCount Amount)
  (Variables|Default|SetbetrayON? true))

(event EventBeginPlay
  (bind _asgi_rpg (Utilities|Casting|CastToGI_RPG (Game|GetGameInstance) :!label _label)
    (:then
      (Variables|Default|SetGameInstanceRef _asgi_rpg)
      (Variables|Default|SetBattleManagerRef (Actor|GetComponentbyClass (Game|GetPlayerController 0) "/Game/Custom/Components/AC_BattleManager.AC_BattleManager_C")))
    (:CastFailed
      (Utilities|FlowControl|DelayUntilNextTick)
      (goto _label))))

(event Collision|EventActorBeginOverlap
  (params (OtherActor :type Actor%20Object%20Reference)))

(event EventTick
  (params (DeltaSeconds :type Float%20%28single-precision%29)))

(event EventPerformActionbyAI
  (Variables|Default|SetwasAsleep? false)
  (if (Variables|Default|GetisGettingCooked)
    (bind _isdead (CallFunction|IsGettingCookedFunction))
    (if _isdead
      (Utilities|FlowControl|Delay 1.0)
      (Default|EndCharacterTurn (Variables|Default|GetBattleManagerReferences))
      (CallFunction|OnDeath)
      (else
        (if (== (Math|Random|RandomIntegerinRange 0 (Variables|Default|GetsleepCounter)) 0) :!label _label
          (Development|PrintString "Sleep was inefective")
          (else
            (Development|PrintString "Target is asleep")
            (Variables|Default|SetwasAsleep? true)))
        (Variables|Default|SetsleepCounter 0)
        (Utilities|FlowControl|Delay 1.0 :!label _label_2)
        (Variables|Default|SetbetrayCount 0)
        (Variables|Default|SetbetrayON? false)
        (Default|EndCharacterTurn (Variables|Default|GetBattleManagerReferences))))
    (else
      (CallFunction|StartRegeneration)
      (if (> (Variables|Default|GetsleepCounter) 0)
        (goto _label)
        (else
          (Development|PrintString (Utilities|GetDisplayName self) true true "(R=0.000000,G=0.660000,B=1.000000,A=1.000000)" 2e+01)
          (switch Utilities|FlowControl|Switch|SwitchonE_EnemyActions (Variables|Default|GetselectedAction)
            (:NewEnumerator0
              (CallFunction|MoveFunction)
              (goto _label_2))
            (:NewEnumerator1
              (CallFunction|AttackPanFunction)
              (goto _label_2))
            (:NewEnumerator2
              (CallFunction|AttackPlayerFunction)
              (goto _label_2))))))))

(event EventOnDamageReceived
  (params (Damage :type Float%20%28double-precision%29) (Critical :type Boolean) (IngredientsUsed :type Array%20of%20E_Ingridients%20Enums :default "NewEnumerator17"))
  (for _array_element IngredientsUsed
    (Development|PrintString (Utilities|String|Append "Was attacked by" ":" (Utilities|String|EnumtoString _array_element))))
  (Variables|Default|SetwasHitLastTurn true)
  (Variables|Default|SetStartRegen false))

(event EventOnDeath
  (bind _aspc_rpg_battle (Utilities|Casting|CastToPC_RPG_Battle (Game|GetPlayerController 0)))
  (Default|OnEnemyKilled (Variables|/Game/Custom/Controllers/PC_RPG_Battle.PC_RPG_Battle_C|GetAC_BattleManager _aspc_rpg_battle) self)
  (if (<= (Variables|Default|GetcurrentIndex) 5)
    (bind _asgi_rpg (Utilities|Casting|CastToGI_RPG (Game|GetGameInstance)))
    (Variables|/Game/Custom/BP_EnemySpot.BP_EnemySpot_C|SethasBeenCounted (.Value (Utilities|Map|Find (Variables|/Game/Custom/GI_RPG.GI_RPG_C|GetEnemySpotMap _asgi_rpg) (Variables|Default|GetcurrentIndex))) false)
    (Variables|/Game/Custom/GI_RPG.GI_RPG_C|SetEnemiesLeftBeforeGameOver _asgi_rpg (+ (Variables|/Game/Custom/GI_RPG.GI_RPG_C|GetEnemiesLeftBeforeGameOver _asgi_rpg) 1))))

(fn ConstructionScript
  (|CallParentFunction))

(fn TryBreakingPan
  (params (PointReference :type BP%20Enemy%20Spot%20Object%20Reference)))

(fn RecoverSauceBar)

(fn StartRegeneration)

(fn IsGettingCookedFunction)

(fn MoveFunction)

(fn GotoRightTurnArray
  (bind _self self)
  (bind _self_2 self)
  (bind _battlemanagerref (Variables|Default|GetBattleManagerRef))
  (bind _battlemanagerref_2 (Variables|Default|GetBattleManagerRef))
  (switch Utilities|FlowControl|Switch|SwitchonE_EnemyActions (Variables|Default|GetselectedAction)
    (:NewEnumerator0
      (Utilities|Array|RemoveItem (Variables|/Game/Custom/Components/AC_BattleManager.AC_BattleManager_C|GetMoveTurn _battlemanagerref) _self)
      (Utilities|Array|AddUnique (Variables|/Game/Custom/Components/AC_BattleManager.AC_BattleManager_C|GetAttackPanTurn _battlemanagerref) _self)
      (Variables|Default|SetselectedAction "NewEnumerator1"))
    (:NewEnumerator1
      (Utilities|Array|RemoveItem (Variables|/Game/Custom/Components/AC_BattleManager.AC_BattleManager_C|GetAttackPanTurn _battlemanagerref_2) _self_2)
      (Utilities|Array|AddUnique (Variables|/Game/Custom/Components/AC_BattleManager.AC_BattleManager_C|GetAttackPlayerTurn _battlemanagerref_2) _self_2)
      (Variables|Default|SetselectedAction "NewEnumerator2"))))

(fn AttackPanFunction
  ;[0.15 0.15 0.15 0.5] AttackPan
  (Variables|AttackPanFunction|SethasAttackedAPan false)
  (bind _asgi_rpg (Utilities|Casting|CastToGI_RPG (Game|GetGameInstance)))
  (bind _array_element (Utilities|Array|ForEachLoopwithBreak (Variables|AttackPanFunction|GetPossiblePanSpots) :!label _label)
    (:LoopBody
      (if (.ReturnValue (Utilities|Map|Find (Variables|/Game/Custom/GI_RPG.GI_RPG_C|GetEnemySpotMap _asgi_rpg) _array_element))
        (if (and (not (Variables|/Game/Custom/BP_EnemySpot.BP_EnemySpot_C|GetHasPanPartBeenBroken (.Value (Utilities|Map|Find (Variables|/Game/Custom/GI_RPG.GI_RPG_C|GetEnemySpotMap _asgi_rpg) _array_element)))) (Variables|/Game/Custom/BP_EnemySpot.BP_EnemySpot_C|GetisOccupiedByPan (.Value (Utilities|Map|Find (Variables|/Game/Custom/GI_RPG.GI_RPG_C|GetEnemySpotMap _asgi_rpg) _array_element))))
          (Default|PanPartAttacked (.Value (Utilities|Map|Find (Variables|/Game/Custom/GI_RPG.GI_RPG_C|GetEnemySpotMap _asgi_rpg) _array_element)))
          (Development|PrintString "PanAttacked")
          (Variables|AttackPanFunction|SethasAttackedAPan true)
          (goto _label Break))))
    (:Completed
      (if (Variables|AttackPanFunction|GethasAttackedAPan)
        _))))

(fn AttackPlayerFunction
  (if (Variables|Default|GetbetrayON?)
    (CallFunction|AttackEnemy)))

(fn GetRandomPoint
  (params (Array :type Array%20of%20Integers))
  (if (== (Utilities|Array|Length Array) 0)
    (return -99)
    (else
      (bind _array_element (Utilities|Array|ForEachLoopwithBreak Array :!label _label)
        (:LoopBody
          (if (Math|Random|RandomBool)
            (return _array_element)))
        (:Completed
          (if true
            (goto _label)))))))

(fn CreatePointArray)

(fn SelectActionfortheTurn
  (if (Variables|Default|GetbetrayON?)
    (Variables|Default|SetselectedAction "NewEnumerator2" :!label _label)
    (else
      (switch int (Math|Random|RandomIntegerinRange 0 2)
        (:0
          (Variables|Default|SetselectedAction "NewEnumerator0"))
        (:1
          (goto _label))
        (:2
          (goto _label))))))

(fn SimulateMove)

(fn SimulateAttackPan
  (bind _currentindex (Variables|Default|GetCurrentIndex))
  (bind _currentindex_2 (Variables|Default|GetCurrentIndex))
  (bind _currentindex_3 (Variables|Default|GetCurrentIndex))
  (bind _returnvalue (+ _currentindex_3 1))
  (bind _returnvalue_2 (+ _currentindex -1))
  ;[0.15 0.15 0.15 0.5] Search for a pan to attack
  (bind _output_get (Variables|AttackPanFunction|SetPossiblePanSpots (Utilities|Array|MakeArray (+ _currentindex_2 5) (+ _currentindex_2 -5))))
  (if (!= (Math|Integer|%(Integer) _returnvalue 5) 1)
    (Utilities|Array|Add _output_get _returnvalue))
  (if (!= (Math|Integer|%(Integer) _returnvalue_2 5) 0)
    (Utilities|Array|Add (Variables|AttackPanFunction|GetPossiblePanSpots) _returnvalue_2)
    (Utilities|Array|Shuffle (Variables|AttackPanFunction|GetPossiblePanSpots)))
  ;[0.15 0.15 0.15 0.5] AttackPan
  (Variables|AttackPanFunction|SethasAttackedAPan false)
  (bind _asgi_rpg (Utilities|Casting|CastToGI_RPG (Game|GetGameInstance)))
  (bind _array_element (Utilities|Array|ForEachLoopwithBreak (Variables|AttackPanFunction|GetPossiblePanSpots) :!label _label)
    (:LoopBody
      (if (.ReturnValue (Utilities|Map|Find (Variables|/Game/Custom/GI_RPG.GI_RPG_C|GetEnemySpotMap _asgi_rpg) _array_element))
        (if (and (not (Variables|/Game/Custom/BP_EnemySpot.BP_EnemySpot_C|GetHasPanPartBeenBroken (.Value (Utilities|Map|Find (Variables|/Game/Custom/GI_RPG.GI_RPG_C|GetEnemySpotMap _asgi_rpg) _array_element)))) (Variables|/Game/Custom/BP_EnemySpot.BP_EnemySpot_C|GetisOccupiedByPan (.Value (Utilities|Map|Find (Variables|/Game/Custom/GI_RPG.GI_RPG_C|GetEnemySpotMap _asgi_rpg) _array_element))))
          (Variables|AttackPanFunction|SethasAttackedAPan true)
          (goto _label Break))))
    (:Completed
      (if (not (Variables|AttackPanFunction|GethasAttackedAPan))
        (Development|PrintString (Utilities|String|Append (Utilities|GetDisplayName self) " " "Cannot attack pan"))
        (CallFunction|GotoRightTurnArray)))))

(fn AttackEnemy
  (for _index (range 1 (Variables|Default|GetbetrayCount))
    (LocalVariables|SetlowestHP 9999.0)
    (LocalVariables|SetlowestHPEnemy 0)
    (for _array_element (Variables|/Game/Custom/Components/AC_BattleManager.AC_BattleManager_C|GetEnemies (Variables|Default|GetBattleManagerRef))
      (if (< (Variables|/Game/Custom/Components/AC_CharacterBattleStats.AC_CharacterBattleStats_C|GetCurrentHP (Variables|/Game/Custom/BP_BaseRPGCharacter.BP_BaseRPGCharacter_C|GetAC_CharacterBattleStats _array_element)) (LocalVariables|GetlowestHP))
        (LocalVariables|SetlowestHP (Variables|/Game/Custom/Components/AC_CharacterBattleStats.AC_CharacterBattleStats_C|GetCurrentHP (Variables|/Game/Custom/BP_BaseRPGCharacter.BP_BaseRPGCharacter_C|GetAC_CharacterBattleStats _array_element)))
        (LocalVariables|SetlowestHPEnemy _array_element)))
    (bind _returnvalue (Utilities|GetDataTableRow "/Game/Custom/DataTables/DT_Enemies.DT_Enemies" (Variables|Default|GetWhatEnemyAmI))
      (:then
        (bind _returnvalue_2 (Utilities|GetDataTableRow "/Game/Custom/DataTables/DT_Ingridients.DT_Ingridients" (Utilities|String|StringToName (Utilities|String|EnumtoString (Utilities|Array|Get(acopy) (.Ingredients (Utilities|Struct|BreakS_Enemy _returnvalue)) (Math|Random|RandomIntegerinRange 0 (- (Utilities|Array|Length (.Ingredients (Utilities|Struct|BreakS_Enemy _returnvalue))) 1))))))
          (:then
            (Development|PrintString (Utilities|String|Append "Attacked:" (Utilities|GetDisplayName (LocalVariables|GetlowestHPEnemy)) " resulting in:" (Utilities|String|ToString(Float) (.Dmg_Modifier (Utilities|Struct|BreakS_Ingridient _returnvalue_2))) " dmg"))
            (Default|ReceiveDamage (Variables|/Game/Custom/BP_BaseRPGCharacter.BP_BaseRPGCharacter_C|GetAC_CharacterBattleStats (LocalVariables|GetlowestHPEnemy)) (.Dmg_Modifier (Utilities|Struct|BreakS_Ingridient _returnvalue_2)) 0.0 0.0 (Utilities|Array|MakeArray (Utilities|Array|Get(acopy) (.Ingredients (Utilities|Struct|BreakS_Enemy _returnvalue)) (Math|Random|RandomIntegerinRange 0 (- (Utilities|Array|Length (.Ingredients (Utilities|Struct|BreakS_Enemy _returnvalue))) 1)))))))))))