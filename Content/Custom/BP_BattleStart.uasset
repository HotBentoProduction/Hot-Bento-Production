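; BP_BattleStart is a trigger actor that starts an enemy encounter when the player walks into its box.
; BeginPlay caches the GI_RPG game instance; on box overlap by BP_ThirdPersonCharacter it calls EncounterEnemies on the ACBattleManager reached through the player controller.
; The encounter and battle map names come from the game instance's EnemyCounter and MapCounter, while random picks from PossibleEncounters and PossibleBattleMaps are left unconnected.
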(event OnComponentBeginOverlap(Box)
  (params (OverlappedComponent :type Primitive%20Component%20Object%20Reference) (OtherActor :type Actor%20Object%20Reference) (OtherComp :type Primitive%20Component%20Object%20Reference) (OtherBodyIndex :type Integer) (bFromSweep :type Boolean) (SweepResult :type Hit%20Result%20Structure%20%28by%20ref%29))
  (bind _as_gi_rpg (Variables|Default|GetAs%20GI%20RPG))
  (if (== (Utilities|GetClass OtherActor) "/Game/ThirdPerson/Blueprints/BP_ThirdPersonCharacter.BP_ThirdPersonCharacter_C")
    (bind _asbp_third_person_character (Utilities|Casting|CastToBP_ThirdPersonCharacter OtherActor))
    (Default|EncounterEnemies (Variables|/Game/Custom/Controllers/PC_RPG_World.PC_RPG_World_C|GetAC_BattleManager (Variables|/Game/ThirdPerson/Blueprints/BP_ThirdPersonCharacter.BP_ThirdPersonCharacter_C|GetPlayerController _asbp_third_person_character)) (Variables|/Game/Custom/GI_RPG.GI_RPG_C|GetEnemyCounter _as_gi_rpg) (Variables|/Game/Custom/GI_RPG.GI_RPG_C|GetMapCounter _as_gi_rpg))))

(event Collision|EventActorBeginOverlap
  (params (OtherActor :type Actor%20Object%20Reference)))

(event EventTick
  (params (DeltaSeconds :type Float%20%28single-precision%29)))

(event EventBeginPlay
  (bind _asgi_rpg (Utilities|Casting|CastToGI_RPG (Game|GetGameInstance)))
  (Variables|Default|SetAs%20GI%20RPG _asgi_rpg))

(fn ConstructionScript)