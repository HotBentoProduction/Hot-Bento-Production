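; World player controller that sets up starting inventory and manages overworld menus for recipes, events, shop, treasure and pot changing.
; BeginPlay loads the Inventory save, seeding ingredients, recipes and GI_RPG pans on first execution, then creates the widgets collapsed.
; It retries until it can link to the third-person character, then toggles the map on the main-menu level.
; Events switch widget visibility, input mode and cursor; a setter passes encounters and battle maps to GI_RPG.
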(event EventBeginPlay
  (bind _returnvalue (SaveGame|LoadGamefromSlot "Inventory"))
  (bind _asinventory (Utilities|Casting|CastToInventory _returnvalue))
  (if (Variables|/Game/Custom/SaveGame/Inventory.Inventory_C|GetFirstExecution _asinventory)
    (CallFunction|AddRecipe&Ingridients _asinventory)
    (CallFunction|AddPans))
  (bind _returnvalue_2 (UserInterface|CreateWidget "/Game/Custom/Widgets/Recipes/Create_recipes.Create_recipes_C"))
  (UserInterface|Viewport|AddtoViewport _returnvalue_2 0)
  (Widget|SetVisibility _returnvalue_2 "Collapsed")
  (Variables|Default|SetCreate%20Recipes%20Reference _returnvalue_2)
  (bind _returnvalue_3 (UserInterface|CreateWidget "/Game/Custom/Widgets/Event/Widget_Event.Widget_Event_C"))
  (UserInterface|Viewport|AddtoViewport _returnvalue_3 0)
  (Widget|SetVisibility _returnvalue_3 "Collapsed")
  (Variables|Default|SetWidget%20Event _returnvalue_3)
  (bind _returnvalue_4 (UserInterface|CreateWidget "/Game/Custom/Widgets/Shop/Widget_Shop.Widget_Shop_C"))
  (UserInterface|Viewport|AddtoViewport _returnvalue_4 0)
  (Widget|SetVisibility _returnvalue_4 "Collapsed")
  (Variables|Default|SetWidget%20Shop _returnvalue_4)
  (bind _returnvalue_5 (UserInterface|CreateWidget "/Game/Custom/Widgets/Treasure/Widget_Treasure.Widget_Treasure_C"))
  (UserInterface|Viewport|AddtoViewport _returnvalue_5 0)
  (Widget|SetVisibility _returnvalue_5 "Collapsed")
  (Variables|Default|SetWidget%20Treasure _returnvalue_5)
  (bind _returnvalue_6 (UserInterface|CreateWidget "/Game/Custom/Widgets/BattleWidgets/StartUpgratePot/Widget_ChangePots.Widget_ChangePots_C"))
  (UserInterface|Viewport|AddtoViewport _returnvalue_6 0)
  (Widget|SetVisibility _returnvalue_6 "Collapsed")
  (Variables|Default|SetWidgetTakePot _returnvalue_6)
  (Input|SetInputModeGameOnly self false)
  (bind _asbp_third_person_character (Utilities|Casting|CastToBP_ThirdPersonCharacter (Pawn|GetControlledPawn) :!label _label)
    (:then
      (Variables|/Game/ThirdPerson/Blueprints/BP_ThirdPersonCharacter.BP_ThirdPersonCharacter_C|SetPlayerController _asbp_third_person_character self)
      (bind _asgi_rpg (Utilities|Casting|CastToGI_RPG (Game|GetGameInstance)))
      (bind _returnvalue_7 (Game|GetCurrentLevelName true))
      (if (Utilities|Enum|Equal(Enum) (Variables|/Game/Custom/GI_RPG.GI_RPG_C|GetMainMenuMapName _asgi_rpg) _returnvalue_7)
        (Default|ShowHideMap _asgi_rpg)))
    (:CastFailed
      (Utilities|FlowControl|Delay 0.2)
      (goto _label))))

(event EventTreasureButton
  (bind _widget_treasure (Variables|Default|GetWidget%20Treasure))
  (Default|RandomTreasure _widget_treasure)
  (Widget|SetVisibility _widget_treasure "Visible")
  (Input|SetInputModeGameandUI self 0 "DoNotLock" true false)
  (Variables|Default|SetbShowMouseCursor true))

(event EventStartShowingRecipeWidget
  (Widget|SetVisibility (Variables|Default|GetCreate%20Recipes%20Reference) "Visible")
  (Input|SetInputModeGameandUI self 0 "DoNotLock" true false)
  (Variables|Default|SetbShowMouseCursor true))

(event EventStopShowingRecipeWidget
  (Widget|SetVisibility (Variables|Default|GetCreate%20Recipes%20Reference) "Collapsed")
  (Input|SetInputModeGameOnly self false)
  (Variables|Default|SetbShowMouseCursor false))

(event EventChangePot
  (bind _widgettakepot (Variables|Default|GetWidgetTakePot))
  (Widget|SetVisibility _widgettakepot "Visible")
  (Default|GetApfromGameInstance _widgettakepot)
  (Input|SetInputModeGameandUI self _widgettakepot "DoNotLock" true false)
  (Variables|Default|SetbShowMouseCursor true))

(event EventShopButton
  (Widget|SetVisibility (Variables|Default|GetWidget%20Shop) "Visible")
  (Input|SetInputModeGameandUI self 0 "DoNotLock" true false)
  (Variables|Default|SetbShowMouseCursor true))

(event EventEventButton
  (Widget|SetVisibility (Variables|Default|GetWidget%20Event) "Visible")
  (Input|SetInputModeGameandUI self 0 "DoNotLock" true false)
  (Variables|Default|SetbShowMouseCursor true))

(fn ConstructionScript)

(fn SetPossibleEncountersandBattleMaps
  (params (PossibleEncounters :type Array%20of%20Names) (PossibleBattleMaps :type Array%20of%20Names))
  (Utilities|FlowControl|Sequence
    (:then_0
      (if (> (Utilities|Array|Length PossibleEncounters) 0)
        (bind _asgi_rpg (Utilities|Casting|CastToGI_RPG (Game|GetGameInstance)))
        (Variables|/Game/Custom/GI_RPG.GI_RPG_C|SetPossibleEncounters _asgi_rpg PossibleEncounters)))
    (:then_1
      (if (> (Utilities|Array|Length PossibleBattleMaps) 0)
        (bind _asgi_rpg_2 (Utilities|Casting|CastToGI_RPG (Game|GetGameInstance)))
        (Variables|/Game/Custom/GI_RPG.GI_RPG_C|SetPossibleBattleMaps _asgi_rpg_2 PossibleBattleMaps)))))

(fn AddRecipe&Ingridients
  (params (Inventory :type Inventory%20Object%20Reference))
  ;[0.15 0.15 0.15 0.5] Change Deafult Value of Ingredient and Sauce
  (CallFunction|AddIngredients Inventory)
  (CallFunction|AddRecipes Inventory)
  (SaveGame|SaveGametoSlot Inventory "Inventory")
  (bind _ac_inventorymanager (Variables|Default|GetAC_InventoryManager)
    (:then
      (bind _outrownames (DataTable|GetDataTableRowNames "/Game/Custom/DataTables/DT_Pastas.DT_Pastas"))
      (for _array_element _outrownames
        ;[0.15 0.15 0.15 0.5 24] Check Pasta Amount to show in Menu
        (bind _returnvalue (Utilities|GetDataTableRow "/Game/Custom/DataTables/DT_Pastas.DT_Pastas" _array_element)
          (:then
            ;;[0.15 0.15 0.15 0.5] Case - Pasta found in Table: check pasta amount for corresponding Pasta Name
            (Default|AddPastatoPastaMenu _ac_inventorymanager (.PastaHardCodedName (Utilities|Struct|BreakS_Pasta _returnvalue)) (.PastaStackAmount (Utilities|Struct|BreakS_Pasta _returnvalue))))
          (:RowNotFound
            ;;[0.15 0.15 0.15 0.5] Case - Pasta not found in Table
            (Development|PrintString "Errore in PC_RPG_BATTLE  in get data tabel row Pasta")))))
    (:else)))

(fn AddIngredients
  (params (Inventory :type Inventory%20Object%20Reference))
  (bind _outrownames (DataTable|GetDataTableRowNames "/Game/Custom/DataTables/DT_Ingridients.DT_Ingridients"))
  (for _array_element _outrownames
    (bind _returnvalue (Utilities|GetDataTableRow "/Game/Custom/DataTables/DT_Ingridients.DT_Ingridients" _array_element)
      (:then
        (Utilities|Map|Add (Variables|/Game/Custom/SaveGame/Inventory.Inventory_C|GetIngridients Inventory) (.Name (Utilities|Struct|BreakS_Ingridient _returnvalue)) 50)))))

(fn AddRecipes
  (params (Inventory :type Inventory%20Object%20Reference))
  (bind _outrownames (DataTable|GetDataTableRowNames "/Game/Custom/DataTables/DT_recipes.DT_recipes"))
  (for _array_element _outrownames
    (bind _returnvalue (Utilities|GetDataTableRow "/Game/Custom/DataTables/DT_recipes.DT_recipes" _array_element)
      (:then
        (Utilities|Map|Add (Variables|/Game/Custom/SaveGame/Inventory.Inventory_C|GetRecipes Inventory) (Utilities|String|ToString(Name) (.Name (Utilities|Struct|BreakS_Recipes _returnvalue))) 0)))))

(fn AddPans
  (bind _asgi_rpg (Utilities|Casting|CastToGI_RPG (Game|GetGameInstance)))
  (Utilities|Map|Clear (Variables|/Game/Custom/GI_RPG.GI_RPG_C|GetEquipedPans _asgi_rpg))
  (for _index (range 1 3)
    (bind _returnvalue (Utilities|GetDataTableRow "/Game/Custom/DataTables/DT_Pans.DT_Pans" "1x1")
      (:then
        (Utilities|Map|Add (Variables|/Game/Custom/GI_RPG.GI_RPG_C|GetEquipedPans _asgi_rpg) (Utilities|String|StringToName (Utilities|String|Append (Utilities|String|ToString(Name) (.PanHardCodedName (Utilities|Struct|BreakS_Pan _returnvalue))) "_" (Utilities|String|ToString(Integer) _index))) _returnvalue)))))

(fn GetActionManager
  (return 0))

(fn GetCreateRecipeWidget
  (return (Variables|Default|GetCreate%20Recipes%20Reference)))