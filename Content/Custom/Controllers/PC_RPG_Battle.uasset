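; Player controller for RPG battles that sets up the fight and displays tap-key quick-time prompts.
; BeginPlay ensures the main character exists in the game instance collection, then has ACBattleManager create the interface, spawn combatants and get turn order.
; It pre-spawns collapsed Tap_Key_UI widgets, which QTEEvent reveals by index, positions and assigns a key, retrying each tick until found.
; The countdown-bar timeline logic is present but unconnected.
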(event Custom|QTEEvent
  (params (TargetKey :type Key%20Structure :default "None") (Key%28as%20Text%29 :type Text) (Timer :type Boolean) (Duration :type Float%20%28double-precision%29) (CalledFrom :type Actor%20Object%20Reference) (Index :type Integer) (X :type Float%20%28double-precision%29))
  ;[0.15 0.15 0.15 0.5] Creating Tap key Event
  (bind _output_get (Variables|Default|SetIndexAdd Index))
  (Variables|Default|SetTapKeyActorReference CalledFrom)
  (Utilities|Array|SetArrayElem (Variables|Default|GetKeyArray) (+ _output_get 1) TargetKey true)
  (bind _foundwidgets (Widget|GetAllWidgetsOfClass "/Game/Custom/Widgets/BattleWidgets/Tap_Key_UI.Tap_Key_UI_C" false :!label _label))
  (Utilities|IsValid (Utilities|Array|Get(acopy) _foundwidgets (+ _output_get 1))
    (:Is%20Valid
      (Widget|SetIsEnabled (Variables|/Game/Custom/Widgets/BattleWidgets/Tap_Key_UI.Tap_Key_UI_C|GetCanvas (Utilities|Array|Get(acopy) _foundwidgets (+ _output_get 1))) true)
      (Widget|SetVisibility (Variables|/Game/Custom/Widgets/BattleWidgets/Tap_Key_UI.Tap_Key_UI_C|GetCanvas (Utilities|Array|Get(acopy) _foundwidgets (+ _output_get 1))) "Visible")
      (Utilities|Array|SetArrayElem (Variables|Default|GetTapUIFocused) (+ _output_get 1) (Utilities|Array|Get(acopy) _foundwidgets (+ _output_get 1)) true)
      (UserInterface|Viewport|AddtoViewport (Utilities|Array|Get(acopy) _foundwidgets (+ _output_get 1)) 0)
      (Class|UserWidget|SetPositioninViewport (Utilities|Array|Get(acopy) _foundwidgets (+ _output_get 1)) (Math|Vector2D|MakeVector2D X 354.0) false)
      (Variables|Default|SetCurrentTapKeyReference (Utilities|Array|Get(acopy) _foundwidgets (+ _output_get 1)))
      (Variables|/Game/Custom/Widgets/BattleWidgets/Tap_Key_UI.Tap_Key_UI_C|SetKey (Variables|Default|GetCurrentTapKeyReference) TargetKey)
      (Variables|Default|SetInTapKeyProgress? true)
      (Default|SetText (Variables|Default|GetCurrentTapKeyReference) Key%28as%20Text%29))
    (:Is%20Not%20Valid
      (Utilities|FlowControl|DelayUntilNextTick)
      (Development|PrintString "Not Found")
      (goto _label))))

(event EventBeginPlay
  (bind _ac_battlemanager (Variables|Default|GetAC_BattleManager))
  (bind _asgi_rpg (Utilities|Casting|CastToGI_RPG (Game|GetGameInstance)))
  (if (== (Utilities|Map|Length (Variables|/Game/Custom/GI_RPG.GI_RPG_C|GetPastaNameDictionary _asgi_rpg)) 0)
    _
    (else
      _))
  (bind _asgi_rpg_2 (Utilities|Casting|CastToGI_RPG (Game|GetGameInstance)))
  (if (.ReturnValue (Utilities|Map|Find (Variables|/Game/Custom/GI_RPG.GI_RPG_C|GetCharacterCollection _asgi_rpg_2) (Utilities|Struct|BreakS_CharacterSlot (Variables|/Game/Custom/GI_RPG.GI_RPG_C|GetMainCharacter _asgi_rpg_2))))
    _
    (else
      (CallFunction|CreateNewMainCharacter)))
  (Input|SetInputModeGameandUI self 0 "DoNotLock" true false)
  (Variables|Default|SetbShowMouseCursor true)
  (Utilities|FlowControl|Delay 0.2)
  (Utilities|FlowControl|Sequence
    (:then_0
      (Utilities|FlowControl|Sequence
        (:then_0
          (Default|CreateBattleInterface (Variables|Default|GetAC_BattleManager)))
        (:then_1
          (Default|SpawnPlayerCharacter _ac_battlemanager))
        (:then_2
          (Default|SpawnEnemies _ac_battlemanager))
        (:then_3
          (Default|GetTurnOrder (Variables|Default|GetAC_BattleManager)))
        (:then_4
          (if (> (Variables|Default|GetTapKeyUIPrespawn) (Variables|Default|GetLoopSpawnForTapKeyUI)) :!label _label
            (bind _returnvalue (UserInterface|CreateWidget "/Game/Custom/Widgets/BattleWidgets/Tap_Key_UI.Tap_Key_UI_C" :!label _label_2))
            (Utilities|IsValid _returnvalue
              (:Is%20Valid
                (UserInterface|Viewport|AddtoViewport _returnvalue 0)
                (Variables|/Script/UMG.Widget|SetVisibility (Variables|/Game/Custom/Widgets/BattleWidgets/Tap_Key_UI.Tap_Key_UI_C|GetCanvas _returnvalue) "Collapsed")
                (bind _result (Math|Integer|IncrementInt (Variables|Default|GetLoopSpawnForTapKeyUI))
                  (:%20%20
                    (Variables|Default|SetLoopSpawnForTapKeyUI _result)
                    (goto _label))))
              (:Is%20Not%20Valid
                (Utilities|FlowControl|DelayUntilNextTick)
                (goto _label_2)))))))))

(event Input|MouseEvents|RightMouseButton
  (params (Key :type Key%20Structure :default "None")))

(fn ConstructionScript)

(fn CreateNewMainCharacter
  (bind _returnvalue (Utilities|GetDataTableRow "/Game/Custom/DataTables/DT_MainCharacter.DT_MainCharacter" "TBA")
    (:then
      (Default|AddNewCharactertoCollection (Variables|Default|GetAC_CharacterManager) _returnvalue))))