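; Enemy grid slot where the player places a pan during battle targeting, previewing its footprint on hover.
; Hover derives neighboring slots from pan dimensions on a three-wide grid, or highlights a special pan's position mask, via GameInstance's EnemySpotMap.
; Material swaps show slot state, while occupied or missing slots can invalidate placement through the targeting manager.
; Clicking a valid slot removes the pan, blocks covered slots, ends the character's turn and disables targeting.
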(event OnBeginCursorOver(Cube)
  (params (TouchedComponent :type Primitive%20Component%20Object%20Reference))
  (bind _targetingmanagerreference (Variables|Default|GetTargetingManagerReference))
  (bind _targetingmanagerreference_2 (Variables|Default|GetTargetingManagerReference))
  (Variables|Default|SetisMainTarget true)
  (Variables|/Game/Custom/Components/AC_TargetingManager.AC_TargetingManager_C|SetCanPanBePlacedDown (Variables|Default|GetTargetingManagerReference) true)
  (if (and (Variables|/Game/Custom/Components/AC_TargetingManager.AC_TargetingManager_C|GetisPanTargetingEnable (Variables|Default|GetTargetingManagerReference)) true)
    (bind _nearbyspots (CallFunction|SearchNearSpots))
    (bind _output_get (Variables|Default|SetNearbySpots _nearbyspots))
    (CallFunction|ActivateNearbySpots _output_get)
    (if (and (Variables|Default|GetisOccupied) (Variables|Default|GetisOccupiedByPan))
      (if (Variables|/Game/Custom/Components/AC_TargetingManager.AC_TargetingManager_C|GetisSpecialPan _targetingmanagerreference_2) :!label _label
        (if (!= (Utilities|Array|Get(acopy) (Variables|/Game/Custom/Components/AC_TargetingManager.AC_TargetingManager_C|GetSpecialPanPosition _targetingmanagerreference_2) (Variables|Default|GetSlotIndex)) 0)
          (Rendering|Material|SetMaterial (Variables|Default|GetCube) 0 "/Engine/VREditor/BasicMeshes/MI_Cube_02.MI_Cube_02" :!label _label_2))
        (else
          (goto _label_2)))
      (elif (Variables|Default|GetisOccupied)
        (if (Variables|/Game/Custom/Components/AC_TargetingManager.AC_TargetingManager_C|GetisSpecialPan _targetingmanagerreference)
          (if (!= (Utilities|Array|Get(acopy) (Variables|/Game/Custom/Components/AC_TargetingManager.AC_TargetingManager_C|GetSpecialPanPosition _targetingmanagerreference) (Variables|Default|GetSlotIndex)) 0)
            (Rendering|Material|SetMaterial (Variables|Default|GetCube) 0 "/Engine/VREditor/BasicMeshes/MI_Cube_03.MI_Cube_03" :!label _label_3)
            (Variables|/Game/Custom/Components/AC_TargetingManager.AC_TargetingManager_C|SetCanPanBePlacedDown (Variables|Default|GetTargetingManagerReference) false))
          (else
            (goto _label_3)))
        (else
          (goto _label))))))

(event OnEndCursorOver(Cube)
  (params (TouchedComponent :type Primitive%20Component%20Object%20Reference))
  (if (not (Variables|Default|GetisOccupiedByPan))
    (CallFunction|DeactivateNearbySpots (Variables|Default|GetNearbySpots))
    (Rendering|Material|SetMaterial (Variables|Default|GetCube) 0 "/Engine/EditorMeshes/Camera/MI_CraneRig.MI_CraneRig")))

(event OnClicked(Cube)
  (params (TouchedComponent :type Primitive%20Component%20Object%20Reference) (ButtonPressed :type Key%20Structure))
  (if (Variables|/Game/Custom/Components/AC_TargetingManager.AC_TargetingManager_C|GetCanPanBePlacedDown (Variables|Default|GetTargetingManagerReference))
    (Default|RemovePan (Variables|Default|GetGameInstanceReference))
    (CallFunction|BlockedOFF)
    (CallFunction|BlockNearbySpots)
    (Utilities|Array|Clear (Variables|Default|GetNearbySpots))
    (Default|EndCharacterTurn (Actor|GetComponentbyClass (Components|GetOwner (Variables|Default|GetTargetingManagerReference)) "/Game/Custom/Components/AC_BattleManager.AC_BattleManager_C"))
    (Default|DisableTargeting (Variables|Default|GetTargetingManagerReference))))

(event Custom|StartShowing
  (bind _targetingmanagerreference (Variables|Default|GetTargetingManagerReference))
  (bind _targetingmanagerreference_2 (Variables|Default|GetTargetingManagerReference))
  (if (and (Variables|Default|GetisOccupied) (Variables|Default|GetisOccupiedByPan))
    (if (Variables|/Game/Custom/Components/AC_TargetingManager.AC_TargetingManager_C|GetisSpecialPan _targetingmanagerreference_2) :!label _label
      (if (!= (Utilities|Array|Get(acopy) (Variables|/Game/Custom/Components/AC_TargetingManager.AC_TargetingManager_C|GetSpecialPanPosition _targetingmanagerreference_2) (Variables|Default|GetSlotIndex)) 0)
        (Rendering|Material|SetMaterial (Variables|Default|GetCube) 0 "/Engine/VREditor/BasicMeshes/MI_Cube_02.MI_Cube_02" :!label _label_2))
      (else
        (goto _label_2)))
    (elif (Variables|Default|GetisOccupied)
      (if (Variables|/Game/Custom/Components/AC_TargetingManager.AC_TargetingManager_C|GetisSpecialPan _targetingmanagerreference)
        (if (!= (Utilities|Array|Get(acopy) (Variables|/Game/Custom/Components/AC_TargetingManager.AC_TargetingManager_C|GetSpecialPanPosition _targetingmanagerreference) (Variables|Default|GetSlotIndex)) 0)
          (Rendering|Material|SetMaterial (Variables|Default|GetCube) 0 "/Engine/VREditor/BasicMeshes/MI_Cube_03.MI_Cube_03" :!label _label_3)
          (Variables|/Game/Custom/Components/AC_TargetingManager.AC_TargetingManager_C|SetCanPanBePlacedDown (Variables|Default|GetTargetingManagerReference) false))
        (else
          (goto _label_3)))
      (else
        (goto _label)))))

(event Custom|StopShowing
  (Rendering|Material|SetMaterial (Variables|Default|GetCube) 0 "/Engine/EditorMeshes/Camera/MI_CraneRig.MI_CraneRig"))

(fn ConstructionScript)

(fn SearchNearSpots
  (bind _targetingmanagerreference (Variables|Default|GetTargetingManagerReference))
  (bind _targetingmanagerreference_2 (Variables|Default|GetTargetingManagerReference))
  (bind _pandimensions (Variables|/Game/Custom/Components/AC_TargetingManager.AC_TargetingManager_C|GetPanDimensions _targetingmanagerreference_2))
  (if (Variables|/Game/Custom/Components/AC_TargetingManager.AC_TargetingManager_C|GetisSpecialPan _targetingmanagerreference)
    (for (_array_element _array_index) (Variables|/Game/Custom/Components/AC_TargetingManager.AC_TargetingManager_C|GetSpecialPanPosition _targetingmanagerreference)
      (if (!= _array_element 0)
        (CallFunction|StartShowing (.Value (Utilities|Map|Find (Variables|/Game/Custom/GI_RPG.GI_RPG_C|GetEnemySpotMap (Variables|Default|GetGameInstanceReference)) _array_index)))))
    (CallFunction|StartShowing)
    (else
      (bind _keys (Utilities|Map|Keys _pandimensions))
      (for _array_element_2 _keys
        (for _index (range 1 (- _array_element_2 1))
          (if (and (!= (+ (Variables|Default|GetSlotIndex) _index) 4) (!= (+ (Variables|Default|GetSlotIndex) _index) 7))
            (Utilities|Array|Add (LocalVariables|GetNearbySpotForPan) (+ (Variables|Default|GetSlotIndex) _index)))))
      (bind _values (Utilities|Map|Values _pandimensions))
      (for _array_element_3 _values
        (for _index_2 (range 1 (- _array_element_3 1))
          (Utilities|Array|Add (LocalVariables|GetNearbySpotForPan) (+ (Variables|Default|GetSlotIndex) (* _index_2 3)))))
      (return (LocalVariables|GetNearbySpotForPan)))))

(fn ActivateNearbySpots
  (params (NearbySpots :type Array%20of%20Integers))
  (if (!= (Utilities|Array|Length NearbySpots) 0)
    (for _array_element NearbySpots
      (if (.ReturnValue (Utilities|Map|Find (Variables|/Game/Custom/GI_RPG.GI_RPG_C|GetEnemySpotMap (Variables|Default|GetGameInstanceReference)) _array_element))
        (CallFunction|StartShowing (.Value (Utilities|Map|Find (Variables|/Game/Custom/GI_RPG.GI_RPG_C|GetEnemySpotMap (Variables|Default|GetGameInstanceReference)) _array_element)))
        (else
          (Variables|/Game/Custom/Components/AC_TargetingManager.AC_TargetingManager_C|SetCanPanBePlacedDown (Variables|Default|GetTargetingManagerReference) false))))
    (else
      (Variables|/Game/Custom/Components/AC_TargetingManager.AC_TargetingManager_C|SetCanPanBePlacedDown (Variables|Default|GetTargetingManagerReference) false))))

(fn DeactivateNearbySpots
  (params (NearbySpots :type Array%20of%20Integers))
  (bind _targetingmanagerreference (Variables|Default|GetTargetingManagerReference))
  (if (Variables|/Game/Custom/Components/AC_TargetingManager.AC_TargetingManager_C|GetisSpecialPan _targetingmanagerreference)
    (for (_array_element _array_index) (Variables|/Game/Custom/Components/AC_TargetingManager.AC_TargetingManager_C|GetSpecialPanPosition _targetingmanagerreference)
      (if (!= _array_element 0)
        (CallFunction|StopShowing (.Value (Utilities|Map|Find (Variables|/Game/Custom/GI_RPG.GI_RPG_C|GetEnemySpotMap (Variables|Default|GetGameInstanceReference)) _array_index)))))
    (CallFunction|StopShowing)
    (else
      (for _array_element_2 NearbySpots
        (if (.ReturnValue (Utilities|Map|Find (Variables|/Game/Custom/GI_RPG.GI_RPG_C|GetEnemySpotMap (Variables|Default|GetGameInstanceReference)) _array_element_2))
          (CallFunction|StopShowing (.Value (Utilities|Map|Find (Variables|/Game/Custom/GI_RPG.GI_RPG_C|GetEnemySpotMap (Variables|Default|GetGameInstanceReference)) _array_element_2))))))))

(fn BlockedOFF
  (Variables|Default|SetisOccupied true)
  (Variables|Default|SetisOccupiedByPan true)
  (Rendering|Material|SetMaterial (Variables|Default|GetCube) 0 "/Engine/VREditor/BasicMeshes/MI_Pyramid_01.MI_Pyramid_01")
  (Utilities|Array|Add (Variables|/Game/Custom/GI_RPG.GI_RPG_C|GetPanPosition (Variables|Default|GetGameInstanceReference)) (Variables|Default|GetSlotIndex)))

(fn BlockNearbySpots
  (for _array_element (Variables|Default|GetNearbySpots)
    (if (.ReturnValue (Utilities|Map|Find (Variables|/Game/Custom/GI_RPG.GI_RPG_C|GetEnemySpotMap (Variables|Default|GetGameInstanceReference)) _array_element))
      (CallFunction|BlockedOFF (.Value (Utilities|Map|Find (Variables|/Game/Custom/GI_RPG.GI_RPG_C|GetEnemySpotMap (Variables|Default|GetGameInstanceReference)) _array_element))))))