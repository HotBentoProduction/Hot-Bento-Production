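; BP_MainCharacter is the player character in an RPG battle system, handling its death and the costs of its battle actions.
; On death it clears defending, marks itself dead and notifies the battle manager.
; Abilities look up costs in the player controller's action manager and deduct HP and MP through the battle stats component.
; Pasta actions subtract each item's consumption cost from its stack in the GI_RPG game instance dictionary.
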(event EventBeginPlay)

(event EventTick
  (params (DeltaSeconds :type Float%20%28single-precision%29)))

(event EventOnDeath
  (Variables|/Game/Custom/Components/AC_CharacterBattleStats.AC_CharacterBattleStats_C|SetDefending (Variables|Default|GetAC_CharacterBattleStats) false)
  (Variables|Default|SetDead true)
  (bind _battlemanagerreferences (Variables|Default|GetBattleManagerReferences)
    (:then
      (Default|OnPlayerKilled _battlemanagerreferences))
    (:else)))

(event EventExecuteActionAbilities
  (params (SecondaryActionName :type Name :default "None"))
  (bind (_costhp _costmp) (Default|GetActionCost (Actor|GetComponentbyClass (Game|GetPlayerController 0) "/Game/Custom/Components/AC_ActionManager.AC_ActionManager_C") SecondaryActionName))
  (Default|ReduceHP (Variables|Default|GetAC_CharacterBattleStats) _costhp)
  (Default|ReduceMP (Variables|Default|GetAC_CharacterBattleStats) _costmp))

(event EventExecuteActionPasta
  (params (PastaName :type Name :default "None"))
  ;[0.15 0.15 0.15 0.5] Get the Pasta Cost for Use
  (Default|GetPastaCost (Actor|GetComponentbyClass (Game|GetPlayerController 0) "/Game/Custom/Components/AC_ActionManager.AC_ActionManager_C") PastaName)
  (bind _asgi_rpg (Utilities|Casting|CastToGI_RPG (Game|GetGameInstance)))
  ;[0.15 0.15 0.15 0.5] Update Pasta Current Amount after Use
  (bind _structout (Utilities|Struct|SetmembersinS_Pasta (.Value (Utilities|Map|Find (Variables|/Game/Custom/GI_RPG.GI_RPG_C|GetPastaNameDictionary _asgi_rpg) PastaName)) (- (.PastaStackAmount (Utilities|Struct|BreakS_Pasta (.Value (Utilities|Map|Find (Variables|/Game/Custom/GI_RPG.GI_RPG_C|GetPastaNameDictionary _asgi_rpg) PastaName)))) (.PastaConsumptionCost (Utilities|Struct|BreakS_Pasta (.Value (Utilities|Map|Find (Variables|/Game/Custom/GI_RPG.GI_RPG_C|GetPastaNameDictionary _asgi_rpg) PastaName)))))))
  (Utilities|Map|Add (Variables|/Game/Custom/GI_RPG.GI_RPG_C|GetPastaNameDictionary _asgi_rpg) (.PastaHardCodedName (Utilities|Struct|BreakS_Pasta (.Value (Utilities|Map|Find (Variables|/Game/Custom/GI_RPG.GI_RPG_C|GetPastaNameDictionary _asgi_rpg) PastaName)))) _structout))

(event Collision|EventActorBeginOverlap
  (params (OtherActor :type Actor%20Object%20Reference)))

(fn ConstructionScript
  (|CallParentFunction))