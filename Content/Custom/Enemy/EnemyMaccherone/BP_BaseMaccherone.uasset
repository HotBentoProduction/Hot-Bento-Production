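; Base Maccherone enemy for turn-based cooking battles, overriding parent actions with stats from DT_Enemies.
; Movement claims spots in the GameInstance map, stepping one or occasionally two rows by index offsets of five.
; Attacks queue random ingredients through the battle manager, or target enemies when betrayed.
; Cooking counts CookTime down to death; regeneration restores it, then, once enabled, lowers CurrentHP (the sauce bar) and clears soiling at full cook time.
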(event EventBeginPlay
  (|CallParentFunction)
  (bind _returnvalue (Utilities|GetDataTableRow "/Game/Custom/DataTables/DT_Enemies.DT_Enemies" "BaseMaccherone")
    (:then
      (Variables|Default|SetcookTimeRegen (.CookingTimeRegen (Utilities|Struct|BreakS_Enemy _returnvalue)))
      (Variables|Default|SetcookTime (.CookingTime (Utilities|Struct|BreakS_Enemy _returnvalue)))
      (Variables|Default|SetWhatEnemyAmI (.EnemyHardcodedName (Utilities|Struct|BreakS_Enemy _returnvalue))))))

(event Collision|EventActorBeginOverlap
  (params (OtherActor :type Actor%20Object%20Reference))
  (|CallParentFunction OtherActor) ; This node is disabled and will not be called.\nDrag off pins to build functionality.
)

(event EventTick
  (params (DeltaSeconds :type Float%20%28single-precision%29))
  (|CallParentFunction DeltaSeconds) ; This node is disabled and will not be called.\nDrag off pins to build functionality.
)

(event EventOnSoiled
  (Variables|Default|SetisSoiled true)
  (bind _asgi_rpg (Utilities|Casting|CastToGI_RPG (Game|GetGameInstance)))
  (Variables|/Game/Custom/BP_EnemySpot.BP_EnemySpot_C|SetisEnemySoiled (.Value (Utilities|Map|Find (Variables|/Game/Custom/GI_RPG.GI_RPG_C|GetEnemySpotMap _asgi_rpg) (Variables|Default|GetcurrentIndex))) true))

(fn ConstructionScript
  (|CallParentFunction))

(fn TryBreakingPan
  (params (PointReference :type BP%20Enemy%20Spot%20Object%20Reference))
  (|CallParentFunction PointReference)
  (if (Math|Random|RandomBool)
    (return true)
    (else
      (return false))))

(fn RecoverSauceBar
  (bind _ac_characterbattlestats (Variables|Default|GetAC_CharacterBattleStats))
  (bind _returnvalue (Utilities|GetDataTableRow "/Game/Custom/DataTables/DT_Enemies.DT_Enemies" "BaseMaccherone")
    (:then
      (Variables|/Game/Custom/Components/AC_CharacterBattleStats.AC_CharacterBattleStats_C|SetCurrentHP _ac_characterbattlestats (Math|Float|Clamp(Float) (- (Variables|/Game/Custom/Components/AC_CharacterBattleStats.AC_CharacterBattleStats_C|GetCurrentHP _ac_characterbattlestats) (.SauceBarRegen (Utilities|Struct|BreakS_Enemy _returnvalue))) 0.0 (.Value (Utilities|Map|Find (Variables|/Game/Custom/Components/AC_CharacterBattleStats.AC_CharacterBattleStats_C|GetCharacterStats (Variables|Default|GetAC_CharacterBattleStats)) "NewEnumerator1"))))
      (Default|RefreshHP _ac_characterbattlestats))))

(fn StartRegeneration
  (bind _returnvalue (Utilities|GetDataTableRow "/Game/Custom/DataTables/DT_Enemies.DT_Enemies" "BaseMaccherone")
    (:then
      (Variables|Default|SetcookTime (Math|Integer|Clamp(Integer) (+ (Variables|Default|GetcookTime) (Variables|Default|GetcookTimeRegen)) 0 (.CookingTime (Utilities|Struct|BreakS_Enemy _returnvalue))))
      (CallFunction|UpdateCookTime)
      (if (Variables|Default|GetStartRegen)
        (if (== (Variables|Default|GetcookTime) (.CookingTime (Utilities|Struct|BreakS_Enemy _returnvalue)))
          (CallFunction|RecoverSauceBar)
          (if (Variables|Default|GetisSoiled)
            (Variables|Default|SetisSoiled false)
            (bind _asgi_rpg (Utilities|Casting|CastToGI_RPG (Game|GetGameInstance)))
            (Variables|/Game/Custom/BP_EnemySpot.BP_EnemySpot_C|SetisEnemySoiled (.Value (Utilities|Map|Find (Variables|/Game/Custom/GI_RPG.GI_RPG_C|GetEnemySpotMap _asgi_rpg) (Variables|Default|GetcurrentIndex))) false)))
        (elif (Variables|Default|GetwasHitLastTurn)
          (Variables|Default|SetwasHitLastTurn false)
          (else
            (Variables|Default|SetStartRegen true)))))))

(fn IsGettingCookedFunction
  (bind _output_get (Variables|Default|SetcookTime (- (Variables|Default|GetcookTime) 1)))
  (Development|PrintString (Utilities|String|Append "Turn before death for" (Utilities|GetDisplayName self) ": " (Utilities|String|ToString(Integer) _output_get)))
  (CallFunction|UpdateCookTime)
  (if (<= _output_get 0)
    (return true)
    (else
      (return false))))

(fn MoveFunction
  (bind _chosenspottomove (Variables|MoveFunction|GetchosenSpotToMove))
  (bind _returnvalue (Transformation|GetActorTransform _chosenspottomove))
  (bind (_x _y) (Math|Vector|BreakVector (.location _returnvalue)))
  (Utilities|IsValid _chosenspottomove
    (:Is%20Valid
      (Transformation|SetActorLocation (Math|Vector|MakeVector _x _y (.z (Transformation|GetActorLocation))) false true))
    (:Is%20Not%20Valid
      (Development|PrintString ""))))

(fn CreatePointArray
  (bind _currentindex (Variables|Default|GetCurrentIndex))
  (switch int (Math|Random|RandomInteger 3)
    (:0
      (Variables|MoveFunction|SetMovePointArray (Utilities|Array|MakeArray (+ (Variables|Default|GetCurrentIndex) -5)) :!label _label))
    (:1
      (goto _label))
    (:2
      (if (<= (Variables|Default|GetCurrentIndex) 10)
        (goto _label)
        (else
          (Variables|MoveFunction|SetMovePointArray (Utilities|Array|MakeArray (+ _currentindex -5) (+ _currentindex -10))))))))

(fn AttackPlayerFunction
  (bind _ac_characterbattlestats (Variables|Default|GetAC_CharacterBattleStats))
  (bind _battlemanagerreference (Variables|/Game/Custom/Components/AC_CharacterBattleStats.AC_CharacterBattleStats_C|GetBattleManagerReference _ac_characterbattlestats))
  (if (Variables|Default|GetbetrayON?)
    (CallFunction|AttackEnemy)
    (else
      (LocalVariables|SetAttackValue (.Value (Utilities|Map|Find (Variables|/Game/Custom/Components/AC_CharacterBattleStats.AC_CharacterBattleStats_C|GetCharacterStats _ac_characterbattlestats) "NewEnumerator3")))
      (if (not (>= (Variables|/Game/Custom/Components/AC_CharacterBattleStats.AC_CharacterBattleStats_C|GetCurrentHP (Variables|/Game/Custom/BP_BaseRPGCharacter.BP_BaseRPGCharacter_C|GetAC_CharacterBattleStats (Variables|/Game/Custom/Components/AC_BattleManager.AC_BattleManager_C|GetPlayerCharacter _battlemanagerreference))) 1e+02))
        (bind _returnvalue (Utilities|GetDataTableRow "/Game/Custom/DataTables/DT_Enemies.DT_Enemies" (Variables|Default|GetWhatEnemyAmI))
          (:then
            (Default|AddEnemyAttack _battlemanagerreference (LocalVariables|GetAttackValue) (Utilities|Array|Get(acopy) (.Ingredients (Utilities|Struct|BreakS_Enemy _returnvalue)) (Math|Random|RandomIntegerinRange 0 (- (Utilities|Array|Length (.Ingredients (Utilities|Struct|BreakS_Enemy _returnvalue))) 1))) self)))))))

(fn SelectActionfortheTurn
  (|CallParentFunction))

(fn SimulateMove
  (Variables|MoveFunction|SetchosenSpotToMove 0)
  (if (<= (Variables|Default|GetcurrentIndex) 5)
    (CallFunction|GotoRightTurnArray)
    (else
      (CallFunction|CreatePointArray)
      (bind _array_element (Utilities|Array|ForEachLoopwithBreak (Variables|MoveFunction|GetMovePointArray) :!label _label)
        (:LoopBody
          (if (Variables|/Game/Custom/BP_EnemySpot.BP_EnemySpot_C|GetisOccupied (.Value (Utilities|Map|Find (Variables|/Game/Custom/GI_RPG.GI_RPG_C|GetEnemySpotMap (Variables|Default|GetGameInstanceRef)) _array_element)))
            (if (Utilities|IsValid (Variables|MoveFunction|GetchosenSpotToMove))
              (goto _label Break)
              (else
                (CallFunction|GotoRightTurnArray)
                (goto _label Break)))
            (else
              (bind _output_get (Variables|MoveFunction|SetchosenSpotToMove (.Value (Utilities|Map|Find (Variables|/Game/Custom/GI_RPG.GI_RPG_C|GetEnemySpotMap (Variables|Default|GetGameInstanceRef)) _array_element))))
              (Utilities|IsValid _output_get
                (:Is%20Valid
                  (Variables|/Game/Custom/BP_EnemySpot.BP_EnemySpot_C|SetenemyReference _output_get self)
                  (Variables|/Game/Custom/BP_EnemySpot.BP_EnemySpot_C|SetisOccupied _output_get true)
                  (Variables|/Game/Custom/BP_EnemySpot.BP_EnemySpot_C|SetisEnemySoiled _output_get (Variables|Default|GetisSoiled))
                  (Default|StopShowing _output_get)
                  (Variables|/Game/Custom/BP_EnemySpot.BP_EnemySpot_C|SetenemyReference (.Value (Utilities|Map|Find (Variables|/Game/Custom/GI_RPG.GI_RPG_C|GetEnemySpotMap (Variables|Default|GetGameInstanceRef)) (Variables|Default|GetcurrentIndex))) 0)
                  (Variables|/Game/Custom/BP_EnemySpot.BP_EnemySpot_C|SetisOccupied (.Value (Utilities|Map|Find (Variables|/Game/Custom/GI_RPG.GI_RPG_C|GetEnemySpotMap (Variables|Default|GetGameInstanceRef)) (Variables|Default|GetcurrentIndex))) false)
                  (Variables|/Game/Custom/BP_EnemySpot.BP_EnemySpot_C|SetisEnemySoiled (.Value (Utilities|Map|Find (Variables|/Game/Custom/GI_RPG.GI_RPG_C|GetEnemySpotMap (Variables|Default|GetGameInstanceRef)) (Variables|Default|GetcurrentIndex))) false)
                  (Variables|Default|SetcurrentIndex _array_element))
                (:Is%20Not%20Valid
                  (CallFunction|GotoRightTurnArray))))))))))