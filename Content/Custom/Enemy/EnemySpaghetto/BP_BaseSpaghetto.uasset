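; BP_BaseSpaghetto is a turn-based battle enemy on an indexed spot grid, configured from its DT_Enemies row.
; It picks random actions weighted by half-HP, with sleep and betrayal forcing one choice.
; Movement claims a random free diagonal spot toward lower indices, carrying soiled state through GameInstance's spot map.
; Attacks queue damage with a random ingredient on the battle manager, or hit enemies when betrayed; old StateTree turn logic is disconnected.
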(event EventBeginPlay
  (|CallParentFunction)
  (bind _returnvalue (Utilities|GetDataTableRow "/Game/Custom/DataTables/DT_Enemies.DT_Enemies" "BaseSpaghetto")
    (:then
      (Variables|Default|SetsauceBarRegen (.CookingTimeRegen (Utilities|Struct|BreakS_Enemy _returnvalue)))
      (Variables|Default|SetWhatEnemyAmI (.EnemyHardcodedName (Utilities|Struct|BreakS_Enemy _returnvalue))))))

(event Collision|EventActorBeginOverlap
  (params (OtherActor :type Actor%20Object%20Reference))
  (|CallParentFunction OtherActor) ; This node is disabled and will not be called.\nDrag off pins to build functionality.
)

(event EventTick
  (params (DeltaSeconds :type Float%20%28single-precision%29))
  (|CallParentFunction DeltaSeconds) ; This node is disabled and will not be called.\nDrag off pins to build functionality.
)

(event EventOnSoiled
  (Variables|Default|SetisSoiled true)
  (bind _asgi_rpg (Utilities|Casting|CastToGI_RPG (Game|GetGameInstance)))
  (Variables|/Game/Custom/BP_EnemySpot.BP_EnemySpot_C|SetisEnemySoiled (.Value (Utilities|Map|Find (Variables|/Game/Custom/GI_RPG.GI_RPG_C|GetEnemySpotMap _asgi_rpg) (Variables|Default|GetcurrentIndex))) true))

(fn ConstructionScript
  (|CallParentFunction))

(fn TryBreakingPan
  (params (PointReference :type BP%20Enemy%20Spot%20Object%20Reference))
  (return true))

(fn RecoverSauceBar
  (bind _ac_characterbattlestats (Variables|Default|GetAC_CharacterBattleStats))
  (bind _returnvalue (Utilities|GetDataTableRow "/Game/Custom/DataTables/DT_Enemies.DT_Enemies" "BaseSpaghetto")
    (:then
      (Variables|/Game/Custom/Components/AC_CharacterBattleStats.AC_CharacterBattleStats_C|SetCurrentHP _ac_characterbattlestats (Math|Float|Clamp(Float) (- (Variables|/Game/Custom/Components/AC_CharacterBattleStats.AC_CharacterBattleStats_C|GetCurrentHP _ac_characterbattlestats) (.SauceBarRegen (Utilities|Struct|BreakS_Enemy _returnvalue))) 0.0 (.Value (Utilities|Map|Find (Variables|/Game/Custom/Components/AC_CharacterBattleStats.AC_CharacterBattleStats_C|GetCharacterStats (Variables|Default|GetAC_CharacterBattleStats)) "NewEnumerator1"))))
      (Default|RefreshHP _ac_characterbattlestats))))

(fn StartRegeneration
  (|CallParentFunction))

(fn IsGettingCookedFunction
  (bind _output_get (Variables|Default|SetpoisonStack (- (Variables|Default|GetpoisonStack) 1)))
  (Development|PrintString (Utilities|String|Append "Turn before death for" (Utilities|GetDisplayName self) ": " (Utilities|String|ToString(Integer) _output_get)))
  (CallFunction|UpdateCookTime)
  (if (<= _output_get 0)
    (return true)
    (else
      (return false))))

(fn MoveFunction
  (bind _gameinstanceref (Variables|Default|GetGameInstanceRef))
  (bind _currentindex (Variables|Default|GetcurrentIndex))
  (bind _enemyspotmap (Variables|/Game/Custom/GI_RPG.GI_RPG_C|GetEnemySpotMap _gameinstanceref))
  (bind _value (Utilities|Map|Find _enemyspotmap _currentindex))
  (bind _returnvalue (Transformation|GetActorTransform _value))
  (bind (_x _y) (Math|Vector|BreakVector (.location _returnvalue)))
  (Utilities|IsValid _value
    (:Is%20Valid
      (Transformation|SetActorLocation (Math|Vector|MakeVector _x _y (.z (Transformation|GetActorLocation))) false true))
    (:Is%20Not%20Valid
      (Development|PrintString ""))))

(fn CreatePointArray
  (bind _currentindex (Variables|Default|GetCurrentIndex))
  (bind _currentindex_2 (Variables|Default|GetCurrentIndex))
  (bind _currentindex_3 (Variables|Default|GetCurrentIndex))
  (if (<= (Variables|Default|GetcurrentIndex) 5)
    (CallFunction|GotoRightTurnArray)
    (else
      (switch int (Math|Integer|%(Integer) (Variables|Default|GetCurrentIndex) 5)
        (:0
          (Variables|MoveFunction|SetMovePointArray (Utilities|Array|MakeArray (+ (Variables|Default|GetCurrentIndex) -6))))
        (:1
          (Variables|MoveFunction|SetMovePointArray (Utilities|Array|MakeArray (+ (Variables|Default|GetCurrentIndex) -4))))
        (:2
          (Variables|MoveFunction|SetMovePointArray (Utilities|Array|MakeArray (+ _currentindex_3 -6) (+ _currentindex_3 -4))))
        (:3
          (Variables|MoveFunction|SetMovePointArray (Utilities|Array|MakeArray (+ _currentindex_2 -6) (+ _currentindex_2 -4))))
        (:4
          (Variables|MoveFunction|SetMovePointArray (Utilities|Array|MakeArray (+ _currentindex -6) (+ _currentindex -4))))))))

(fn AttackPlayerFunction
  (bind _ac_characterbattlestats (Variables|Default|GetAC_CharacterBattleStats))
  (bind _battlemanagerreference (Variables|/Game/Custom/Components/AC_CharacterBattleStats.AC_CharacterBattleStats_C|GetBattleManagerReference _ac_characterbattlestats))
  (if (Variables|Default|GetbetrayON?)
    (CallFunction|AttackEnemy)
    (else
      (LocalVariables|SetAttackValue (.Value (Utilities|Map|Find (Variables|/Game/Custom/Components/AC_CharacterBattleStats.AC_CharacterBattleStats_C|GetCharacterStats _ac_characterbattlestats) "NewEnumerator3")))
      (if (not (>= (Variables|/Game/Custom/Components/AC_CharacterBattleStats.AC_CharacterBattleStats_C|GetCurrentHP (Variables|/Game/Custom/BP_BaseRPGCharacter.BP_BaseRPGCharacter_C|GetAC_CharacterBattleStats (Variables|/Game/Custom/Components/AC_BattleManager.AC_BattleManager_C|GetPlayerCharacter _battlemanagerreference))) 1e+02))
        (bind _returnvalue (Utilities|GetDataTableRow "/Game/Custom/DataTables/DT_Enemies.DT_Enemies" (Variables|Default|GetWhatEnemyAmI))
          (:then
            (Default|AddEnemyAttack _battlemanagerreference (LocalVariables|GetAttackValue) (Utilities|Array|Get(acopy) (.Ingredients (Utilities|Struct|BreakS_Enemy _returnvalue)) (Math|Random|RandomIntegerinRange 0 (- (Utilities|Array|Length (.Ingredients (Utilities|Struct|BreakS_Enemy _returnvalue))) 1))) self)))))))

(fn SelectActionfortheTurn
  (bind _ac_characterbattlestats (Variables|Default|GetAC_CharacterBattleStats))
  (if (or (Variables|Default|GetisSleeping) (Variables|Default|GetbetrayON?))
    (Variables|Default|SetselectedAction "NewEnumerator2")
    (elif (> (Variables|/Game/Custom/Components/AC_CharacterBattleStats.AC_CharacterBattleStats_C|GetCurrentHP _ac_characterbattlestats) (* (.Value (Utilities|Map|Find (Variables|/Game/Custom/Components/AC_CharacterBattleStats.AC_CharacterBattleStats_C|GetCharacterStats _ac_characterbattlestats) "NewEnumerator1")) 0.5))
      (switch int (Math|Random|RandomIntegerinRange 0 2)
        (:0
          (Variables|Default|SetselectedAction "NewEnumerator0"))
        (:1
          (Variables|Default|SetselectedAction "NewEnumerator2" :!label _label))
        (:2
          (goto _label)))
      (else
        (switch int (Math|Random|RandomIntegerinRange 0 5)
          (:0
            (Variables|Default|SetselectedAction "NewEnumerator0"))
          (:1
            (Variables|Default|SetselectedAction "NewEnumerator2" :!label _label_2))
          (:2
            (goto _label_2))
          (:3
            (goto _label_2))
          (:4
            (goto _label_2))
          (:5
            (goto _label_2)))))))

(fn SimulateMove
  (bind _movepointarray (Variables|MoveFunction|GetMovePointArray))
  (bind _returnvalue (Utilities|Array|Length _movepointarray))
  (if (<= (Variables|Default|GetcurrentIndex) 5)
    (CallFunction|GotoRightTurnArray)
    (else
      (CallFunction|CreatePointArray)
      (if (!= _returnvalue 0) :!label _label
        (bind _returnvalue_2 (Math|Random|RandomInteger _returnvalue))
        (if (Variables|/Game/Custom/BP_EnemySpot.BP_EnemySpot_C|GetisOccupied (.Value (Utilities|Map|Find (Variables|/Game/Custom/GI_RPG.GI_RPG_C|GetEnemySpotMap (Variables|Default|GetGameInstanceRef)) (Utilities|Array|Get(acopy) _movepointarray _returnvalue_2))))
          (Utilities|Array|RemoveIndex (Variables|MoveFunction|GetMovePointArray) _returnvalue_2)
          (goto _label)
          (else
            (bind _output_get (Variables|MoveFunction|SetchosenSpotToMove (.Value (Utilities|Map|Find (Variables|/Game/Custom/GI_RPG.GI_RPG_C|GetEnemySpotMap (Variables|Default|GetGameInstanceRef)) (Utilities|Array|Get(acopy) _movepointarray _returnvalue_2)))))
            (Utilities|IsValid _output_get
              (:Is%20Valid
                (Variables|/Game/Custom/BP_EnemySpot.BP_EnemySpot_C|SetisOccupied _output_get true)
                (Variables|/Game/Custom/BP_EnemySpot.BP_EnemySpot_C|SetisEnemySoiled _output_get (Variables|Default|GetisSoiled))
                (Variables|/Game/Custom/BP_EnemySpot.BP_EnemySpot_C|SetenemyReference _output_get self)
                (Variables|/Game/Custom/BP_EnemySpot.BP_EnemySpot_C|SetisOccupied (.Value (Utilities|Map|Find (Variables|/Game/Custom/GI_RPG.GI_RPG_C|GetEnemySpotMap (Variables|Default|GetGameInstanceRef)) (Variables|Default|GetcurrentIndex))) false)
                (Variables|/Game/Custom/BP_EnemySpot.BP_EnemySpot_C|SetenemyReference (.Value (Utilities|Map|Find (Variables|/Game/Custom/GI_RPG.GI_RPG_C|GetEnemySpotMap (Variables|Default|GetGameInstanceRef)) (Variables|Default|GetcurrentIndex))) 0)
                (Variables|/Game/Custom/BP_EnemySpot.BP_EnemySpot_C|SetisEnemySoiled (.Value (Utilities|Map|Find (Variables|/Game/Custom/GI_RPG.GI_RPG_C|GetEnemySpotMap (Variables|Default|GetGameInstanceRef)) (Variables|Default|GetcurrentIndex))) false)
                (Variables|Default|SetcurrentIndex (Variables|/Game/Custom/BP_EnemySpot.BP_EnemySpot_C|GetSlotIndex (Variables|MoveFunction|GetchosenSpotToMove)))
                (Default|StopShowing (Variables|MoveFunction|GetchosenSpotToMove)))
              (:Is%20Not%20Valid
                (CallFunction|GotoRightTurnArray)))))
        (else
          (CallFunction|GotoRightTurnArray))))))