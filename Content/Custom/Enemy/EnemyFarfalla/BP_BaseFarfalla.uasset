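; Farfalla enemy for the turn-based cooking battle, loading cook stats from DT_Enemies and choosing its action from betray and sleep state.
; Cook time drops while cooked and regenerates otherwise, eventually restoring the sauce bar and clearing soiled state.
; Movement uses knight-style jumps on a five-wide grid, randomly claiming a free spot in GI_RPG's EnemySpotMap before teleporting there.
; Attacks queue a random ingredient with the battle manager, or target enemies when betrayed.
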(event EventBeginPlay
  (|CallParentFunction)
  (bind _returnvalue (Utilities|GetDataTableRow "/Game/Custom/DataTables/DT_Enemies.DT_Enemies" "BaseFarfalla")
    (:then
      (Variables|Default|SetcookTimeRegen (.CookingTimeRegen (Utilities|Struct|BreakS_Enemy _returnvalue)))
      (Variables|Default|SetcookTime (.CookingTime (Utilities|Struct|BreakS_Enemy _returnvalue)))
      (Variables|Default|SetWhatEnemyAmI (.EnemyHardcodedName (Utilities|Struct|BreakS_Enemy _returnvalue))))))

(event Collision|EventActorBeginOverlap
  (params (OtherActor :type Actor%20Object%20Reference))
  (|CallParentFunction OtherActor) ; This node is disabled and will not be called.\nDrag off pins to build functionality.
)

(event EventTick
  (params (DeltaSeconds :type Float%20%28single-precision%29))
  (|CallParentFunction DeltaSeconds) ; This node is disabled and will not be called.\nDrag off pins to build functionality.
)

(event EventOnSoiled
  (Variables|Default|SetisSoiled true)
  (bind _asgi_rpg (Utilities|Casting|CastToGI_RPG (Game|GetGameInstance)))
  (Variables|/Game/Custom/BP_EnemySpot.BP_EnemySpot_C|SetisEnemySoiled (.Value (Utilities|Map|Find (Variables|/Game/Custom/GI_RPG.GI_RPG_C|GetEnemySpotMap _asgi_rpg) (Variables|Default|GetcurrentIndex))) true))

(fn ConstructionScript
  (|CallParentFunction))

(fn TryBreakingPan
  (params (PointReference :type BP%20Enemy%20Spot%20Object%20Reference))
  (return true))

(fn RecoverSauceBar
  (bind _ac_characterbattlestats (Variables|Default|GetAC_CharacterBattleStats))
  (bind _returnvalue (Utilities|GetDataTableRow "/Game/Custom/DataTables/DT_Enemies.DT_Enemies" "BaseFarfalla")
    (:then
      (Variables|/Game/Custom/Components/AC_CharacterBattleStats.AC_CharacterBattleStats_C|SetCurrentHP _ac_characterbattlestats (Math|Float|Clamp(Float) (- (Variables|/Game/Custom/Components/AC_CharacterBattleStats.AC_CharacterBattleStats_C|GetCurrentHP _ac_characterbattlestats) (.SauceBarRegen (Utilities|Struct|BreakS_Enemy _returnvalue))) 0.0 (.Value (Utilities|Map|Find (Variables|/Game/Custom/Components/AC_CharacterBattleStats.AC_CharacterBattleStats_C|GetCharacterStats (Variables|Default|GetAC_CharacterBattleStats)) "NewEnumerator1"))))
      (Default|RefreshHP _ac_characterbattlestats))))

(fn StartRegeneration
  (bind _returnvalue (Utilities|GetDataTableRow "/Game/Custom/DataTables/DT_Enemies.DT_Enemies" "BaseFarfalla")
    (:then
      (Variables|Default|SetcookTime (Math|Integer|Clamp(Integer) (+ (Variables|Default|GetcookTime) (Variables|Default|GetcookTimeRegen)) 0 (.CookingTime (Utilities|Struct|BreakS_Enemy _returnvalue))))
      (CallFunction|UpdateCookTime)
      (if (Variables|Default|GetStartRegen)
        (if (== (Variables|Default|GetcookTime) (.CookingTime (Utilities|Struct|BreakS_Enemy _returnvalue)))
          (CallFunction|RecoverSauceBar)
          (if (Variables|Default|GetisSoiled)
            (Variables|Default|SetisSoiled false)
            (bind _asgi_rpg (Utilities|Casting|CastToGI_RPG (Game|GetGameInstance)))
            (Variables|/Game/Custom/BP_EnemySpot.BP_EnemySpot_C|SetisEnemySoiled (.Value (Utilities|Map|Find (Variables|/Game/Custom/GI_RPG.GI_RPG_C|GetEnemySpotMap _asgi_rpg) (Variables|Default|GetcurrentIndex))) false)))
        (elif (Variables|Default|GetwasHitLastTurn)
          (Variables|Default|SetwasHitLastTurn false)
          (else
            (Variables|Default|SetStartRegen true)))))))

(fn IsGettingCookedFunction
  (bind _output_get (Variables|Default|SetcookTime (- (Variables|Default|GetcookTime) 1)))
  (Development|PrintString (Utilities|String|Append "Turn before death for" (Utilities|GetDisplayName self) ": " (Utilities|String|ToString(Integer) _output_get)))
  (CallFunction|UpdateCookTime)
  (if (<= _output_get 0)
    (return true)
    (else
      (return false))))

(fn AttackPlayerFunction
  (bind _ac_characterbattlestats (Variables|Default|GetAC_CharacterBattleStats))
  (bind _battlemanagerreference (Variables|/Game/Custom/Components/AC_CharacterBattleStats.AC_CharacterBattleStats_C|GetBattleManagerReference _ac_characterbattlestats))
  (if (Variables|Default|GetbetrayON?)
    (CallFunction|AttackEnemy)
    (else
      (LocalVariables|SetAttackValue (.Value (Utilities|Map|Find (Variables|/Game/Custom/Components/AC_CharacterBattleStats.AC_CharacterBattleStats_C|GetCharacterStats _ac_characterbattlestats) "NewEnumerator3")))
      (if (not (>= (Variables|/Game/Custom/Components/AC_CharacterBattleStats.AC_CharacterBattleStats_C|GetCurrentHP (Variables|/Game/Custom/BP_BaseRPGCharacter.BP_BaseRPGCharacter_C|GetAC_CharacterBattleStats (Variables|/Game/Custom/Components/AC_BattleManager.AC_BattleManager_C|GetPlayerCharacter _battlemanagerreference))) 1e+02))
        (bind _returnvalue (Utilities|GetDataTableRow "/Game/Custom/DataTables/DT_Enemies.DT_Enemies" (Variables|Default|GetWhatEnemyAmI))
          (:then
            (Default|AddEnemyAttack _battlemanagerreference (LocalVariables|GetAttackValue) (Utilities|Array|Get(acopy) (.Ingredients (Utilities|Struct|BreakS_Enemy _returnvalue)) (Math|Random|RandomIntegerinRange 0 (- (Utilities|Array|Length (.Ingredients (Utilities|Struct|BreakS_Enemy _returnvalue))) 1))) self)))))))

(fn CreatePointArray
  (if (<= (Variables|Default|GetcurrentIndex) 5)
    (CallFunction|GotoRightTurnArray)
    (else
      (switch int (Math|Integer|%(Integer) (Variables|Default|GetcurrentIndex) 5)
        (:0
          (Variables|MoveFunction|SetMoveArray (Utilities|Array|MakeArray (- (Variables|Default|GetcurrentIndex) 7) (- (Variables|Default|GetcurrentIndex) 11))))
        (:1
          (Variables|MoveFunction|SetMoveArray (Utilities|Array|MakeArray (- (Variables|Default|GetcurrentIndex) 9) (- (Variables|Default|GetcurrentIndex) 3))))
        (:2
          (Variables|MoveFunction|SetMoveArray (Utilities|Array|MakeArray (- (Variables|Default|GetcurrentIndex) 3) (- (Variables|Default|GetcurrentIndex) 9) (- (Variables|Default|GetcurrentIndex) 11))))
        (:3
          (Variables|MoveFunction|SetMoveArray (Utilities|Array|MakeArray (- (Variables|Default|GetcurrentIndex) 3) (- (Variables|Default|GetcurrentIndex) 7) (- (Variables|Default|GetcurrentIndex) 9) (- (Variables|Default|GetcurrentIndex) 11))))
        (:4
          (Variables|MoveFunction|SetMoveArray (Utilities|Array|MakeArray (- (Variables|Default|GetcurrentIndex) 7) (- (Variables|Default|GetcurrentIndex) 9) (- (Variables|Default|GetcurrentIndex) 11))))))))

(fn SelectActionfortheTurn
  (if (or (Variables|Default|GetbetrayON?) (> (Variables|Default|GetsleepCounter) 0))
    (Variables|Default|SetselectedAction "NewEnumerator2")
    (else
      (Variables|Default|SetselectedAction "NewEnumerator0"))))

(fn SimulateMove
  (CallFunction|CreatePointArray)
  (bind _fail_ (CallFunction|SimulateMoveFunction))
  (if _fail_
    (CallFunction|GotoRightTurnArray)))

(fn SimulateMoveFunction
  (bind _movearray (Variables|MoveFunction|GetMoveArray))
  (bind _returnvalue (Utilities|Array|Length _movearray))
  (if (== _returnvalue 0) :!label _label
    (return true)
    (else
      (bind _returnvalue_2 (Math|Random|RandomInteger _returnvalue))
      (if (< (Utilities|Array|Get(acopy) (Variables|MoveFunction|GetMoveArray) _returnvalue_2) 0)
        _
        (elif (Variables|/Game/Custom/BP_EnemySpot.BP_EnemySpot_C|GetisOccupied (.Value (Utilities|Map|Find (Variables|/Game/Custom/GI_RPG.GI_RPG_C|GetEnemySpotMap (Variables|Default|GetGameInstanceRef)) (Utilities|Array|Get(acopy) (Variables|MoveFunction|GetMoveArray) _returnvalue_2))))
          _
          (else
            (bind _output_get (Variables|MoveFunction|SetselectSpot (.Value (Utilities|Map|Find (Variables|/Game/Custom/GI_RPG.GI_RPG_C|GetEnemySpotMap (Variables|Default|GetGameInstanceRef)) (Utilities|Array|Get(acopy) (Variables|MoveFunction|GetMoveArray) _returnvalue_2)))))
            (Utilities|IsValid _output_get
              (:Is%20Valid
                (Variables|/Game/Custom/BP_EnemySpot.BP_EnemySpot_C|SetisOccupied _output_get true)
                (Variables|/Game/Custom/BP_EnemySpot.BP_EnemySpot_C|SetisEnemySoiled _output_get (Variables|Default|GetisSoiled))
                (Variables|/Game/Custom/BP_EnemySpot.BP_EnemySpot_C|SetenemyReference _output_get self)
                (Variables|/Game/Custom/BP_EnemySpot.BP_EnemySpot_C|SetisOccupied (.Value (Utilities|Map|Find (Variables|/Game/Custom/GI_RPG.GI_RPG_C|GetEnemySpotMap (Variables|Default|GetGameInstanceRef)) (Variables|Default|GetcurrentIndex))) false)
                (Variables|/Game/Custom/BP_EnemySpot.BP_EnemySpot_C|SetenemyReference (.Value (Utilities|Map|Find (Variables|/Game/Custom/GI_RPG.GI_RPG_C|GetEnemySpotMap (Variables|Default|GetGameInstanceRef)) (Variables|Default|GetcurrentIndex))) 0)
                (Variables|/Game/Custom/BP_EnemySpot.BP_EnemySpot_C|SetisEnemySoiled (.Value (Utilities|Map|Find (Variables|/Game/Custom/GI_RPG.GI_RPG_C|GetEnemySpotMap (Variables|Default|GetGameInstanceRef)) (Variables|Default|GetcurrentIndex))) false)
                (Variables|Default|SetcurrentIndex (Variables|/Game/Custom/BP_EnemySpot.BP_EnemySpot_C|GetSlotIndex (Variables|MoveFunction|GetselectSpot)))
                (Default|StopShowing (Variables|MoveFunction|GetselectSpot))
                (return false))
              (:Is%20Not%20Valid
                (return true))))))
      (Utilities|Array|RemoveIndex (Variables|MoveFunction|GetMoveArray) _returnvalue_2)
      (goto _label))))

(fn MoveFunction
  (CallFunction|MovefromPosition))

(fn MovefromPosition
  (bind _gameinstanceref (Variables|Default|GetGameInstanceRef))
  (bind _currentindex (Variables|Default|GetcurrentIndex))
  (bind _enemyspotmap (Variables|/Game/Custom/GI_RPG.GI_RPG_C|GetEnemySpotMap _gameinstanceref))
  (bind _value (Utilities|Map|Find _enemyspotmap _currentindex))
  (bind _returnvalue (Transformation|GetActorTransform _value))
  (bind (_x _y) (Math|Vector|BreakVector (.location _returnvalue)))
  (Utilities|IsValid _value
    (:Is%20Valid
      (Transformation|SetActorLocation (Math|Vector|MakeVector _x _y (.z (Transformation|GetActorLocation))) false true))
    (:Is%20Not%20Valid
      (Development|PrintString ""))))